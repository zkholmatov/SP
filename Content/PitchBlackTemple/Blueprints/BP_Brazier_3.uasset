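; BP_Brazier_3 is a hanging caged brazier with a point light and embers, suspended on a procedurally built chain.
; The construction script lowers the cage, light and embers by DropDownLength, then adds scaled, rotated Chain mesh components downward to fill the drop.
; Link count derives from the mesh bounds plus ChainLinkOffset, while link spacing uses the bounds alone.
; The event graph has no active logic.
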(event EventBeginPlay)

(event Collision|EventActorBeginOverlap
  (params (OtherActor :type Actor%20Object%20Reference)))

(event EventTick
  (params (DeltaSeconds :type Float%20%28single-precision%29)))

(fn ConstructionScript
  (bind _dropdownlength (Variables|Default|GetDropDownLength))
  (bind _chain (Variables|Default|GetChain))
  (bind _returnvalue (StaticMesh|GetBoundingBox _chain))
  (bind _returnvalue_2 (- 0.0 _dropdownlength))
  (bind _returnvalue_3 (/ (.x (.max _returnvalue)) 3.0))
  (Transformation|AddLocalOffset (Variables|Default|GetSM_CagedBrazier_01) (Math|Vector|MakeVector 0.0 0.0 _returnvalue_2) false false)
  (Transformation|AddLocalOffset (Variables|Default|GetPointLight) (Math|Vector|MakeVector 0.0 0.0 _returnvalue_2) false false)
  (Transformation|AddLocalOffset (Variables|Default|GetSM_Embers_03) (Math|Vector|MakeVector 0.0 0.0 _returnvalue_2) false false)
  (for _index (range 0 (Math|Float|Truncate (/ (Variables|Default|GetDropDownLength) (+ _returnvalue_3 (Variables|Default|GetChainLink_Offset)))))
    (bind _returnvalue_4 (AddComponent|AddStaticMeshComponent false (Math|Transform|MakeTransform (Math|Vector|MakeVector 0.0 0.0 (- 0.0 (* _index _returnvalue_3))) "-90.000000,0.000000,0.000000" "0.330000,0.330000,0.330000")))
    (Components|StaticMesh|SetStaticMesh _returnvalue_4 _chain)))