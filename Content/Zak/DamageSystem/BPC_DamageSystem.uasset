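; Actor component that tracks health, death and damage for its owner, with functions to heal and set max health.
; TakeDamage uses a CanBeDamaged macro to ignore hits when dead or invincible, block parryable hits while parrying, or subtract health.
; It fires event dispatchers for parry, death and damage response, the latter only when interruptable or forced by the DamageInfo struct.
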(event EventBeginPlay)

(event EventTick
  (params (DeltaSeconds :type Float%20%28single-precision%29)))

(fn HealFunction
  (params (Amount :type Float%20%28double-precision%29))
  (if (not (Variables|Default|GetDead?))
    (bind _output_get (Variables|Default|SetHealth (Math|Float|Clamp(Float) (+ Amount (Variables|Default|GetHealth)) 0.0 (Variables|Default|GetMaxHealth))))
    (return _output_get)))

(fn TakeDamage
  (params (DamageInfo :type S%20Damage%20Info%20Structure))
  (bind (_amount _damagetype _damageresponse _canbeparried_ _shouldforceinterrupt_ _damagedirection _damagecauser) (Utilities|Struct|BreakS_DamageInfo DamageInfo))
  (Utilities|CanbeDamaged _canbeparried_
    (:NoDamage
      (return false 0.0 false (stale _output_get)))
    (:BlockDamage
      (Default|CallOnParried _canbeparried_ _damagecauser _damagedirection)
      (return false 0.0 true (stale _output_get)))
    (:DoDamage
      (bind _output_get (Variables|Default|SetHealth (- (Variables|Default|GetHealth) _amount)))
      (if (<= _output_get 0.0)
        (Variables|Default|SetDead? true)
        (Default|CallOnDeath)
        (return true _amount false _output_get)
        (elif (or (Variables|Default|GetInterruptable?) _shouldforceinterrupt_)
          (Default|CallOnDamageResponse _damageresponse _damagedirection _damagecauser)
          (return true _amount false _output_get))))))

(fn SetMaxHealth
  (params (MaxHealth :type Float%20%28double-precision%29))
  (bind _output_get (Variables|Default|SetMaxHealth MaxHealth))
  (Variables|Default|SetHealth _output_get))