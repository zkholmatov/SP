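; Actor component that gives a BP_Enemy physics-driven hit reactions.
; On BeginPlay it adds a physical animation component to the owner and caches the enemy's mesh.
; HitReaction applies a profile below the pelvis, simulates bodies below spine_01 and adds an impulse along the trace at the hit bone, falling back to spine_02.
; Tick decays a timer driving physics blend weight, then stops simulation from spine_02 down and disables itself.
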(event Custom|HitReaction
  (params (Hit :type Hit%20Result%20Structure))
  (bind (_bblockinghit _binitialoverlap _time _distance _location _impactpoint _normal _impactnormal _physmat _hitactor _hitcomponent _hitbonename _bonename _hititem _elementindex _faceindex _tracestart _traceend) (Collision|BreakHitResult Hit))
  (bind _returnvalue (Utilities|Name|MakeLiteralName "spine_02"))
  (bind _returnvalue_2 (== _hitbonename "spine_01"))
  (bind _returnvalue_3 (== _hitbonename ""))
  (bind _returnvalue_4 (or _returnvalue_2 _returnvalue_3))
  (bind _returnvalue_5 (select _returnvalue_4 _returnvalue _hitbonename))
  (Components|Tick|SetComponentTickEnabled true)
  (Variables|Default|SetHitReactionTimeRemaining (+ (Variables|Default|GetHitReactionTimeRemaining) 1.0))
  (Class|PhysicalAnimationComponent|ApplyPhysicalAnimationProfileBelow (Variables|Default|GetPhysicalAnimationComponent) "pelvis" "HitReactionProfile" false false)
  (Class|SkeletalMeshComponent|SetAllBodiesBelowSimulatePhysics (Variables|Default|GetMesh) (Utilities|Name|MakeLiteralName "spine_01") true false)
  (Development|PrintString (Utilities|String|ToString(Name) _returnvalue_5))
  (Physics|AddImpulse (Variables|Default|GetMesh) (* (Math|Vector|Normalize (- _traceend _tracestart)) 5e+03) _returnvalue_5 true))

(event EventBeginPlay
  (bind _returnvalue (Game|AddComponentbyClass (Components|GetOwner) "/Script/Engine.PhysicalAnimationComponent"))
  (bind _output_get (Variables|Default|SetPhysicalAnimationComponent _returnvalue))
  (Class|PhysicalAnimationComponent|SetSkeletalMeshComponent _output_get)
  (bind _asbp_enemy (Utilities|Casting|CastToBP_Enemy (Components|GetOwner)))
  (bind _output_get_2 (Variables|Default|SetAs%20BP%20Enemy _asbp_enemy))
  (Variables|Default|SetMesh (Variables|/Script/Engine.Character|GetMesh _output_get_2)))

(event EventTick
  (params (DeltaSeconds :type Float%20%28single-precision%29))
  (bind _mesh (Variables|Default|GetMesh))
  (Variables|Default|SetHitReactionTimeRemaining (- (Math|Interpolation|FInterpTo (Variables|Default|GetHitReactionTimeRemaining) 0.0 0.0 1.0) (* DeltaSeconds 2.0)))
  (if (<= (Variables|Default|GetHitReactionTimeRemaining) 0.0)
    (Variables|Default|SetHitReactionTimeRemaining 0.0)
    (Utilities|IsValid _mesh
      (:Is%20Valid
        (Class|SkeletalMeshComponent|SetAllBodiesBelowSimulatePhysics _mesh (Utilities|Name|MakeLiteralName "spine_02") false true)
        (Components|Tick|SetComponentTickEnabled false)))
    (else
      (Class|SkeletalMeshComponent|SetAllBodiesBelowPhysicsBlendWeight (Variables|Default|GetMesh) (Utilities|Name|MakeLiteralName "spine_01") (Math|Float|Min(Float) (Variables|Default|GetHitReactionTimeRemaining) 1.0) false true))))