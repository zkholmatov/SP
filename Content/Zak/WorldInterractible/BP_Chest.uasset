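; BP_Chest is an interactable chest that opens once when the player overlaps its trigger box.
; The construction script hides the ChildActor component.
; A cast to BP_Player and a DoOnce gate start a timeline that rotates the Top lid on roll.
; The timeline update also feeds a short delay that then makes the child actor component visible.
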(event OnComponentBeginOverlap(Box)
  (params (OverlappedComponent :type Primitive%20Component%20Object%20Reference) (OtherActor :type Actor%20Object%20Reference) (OtherComp :type Primitive%20Component%20Object%20Reference) (OtherBodyIndex :type Integer) (bFromSweep :type Boolean) (SweepResult :type Hit%20Result%20Structure%20%28by%20ref%29))
  (Utilities|Casting|CastToBP_Player OtherActor)
  (Utilities|FlowControl|DoOnce false
    (:Completed
      (bind _newtrack_0 (Timeline|Timeline PlayFromStart)
        (:Update
          (Transformation|SetRelativeRotation (Variables|Default|GetTop) (Math|Rotator|MakeRotator _newtrack_0 0.0 0.0) false false)
          (Utilities|FlowControl|Delay 0.5)
          (Rendering|SetVisibility (Variables|Default|GetChildActor) true false))))))

(event EventBeginPlay)

(event Collision|EventActorBeginOverlap
  (params (OtherActor :type Actor%20Object%20Reference)))

(event EventTick
  (params (DeltaSeconds :type Float%20%28single-precision%29)))

(fn ConstructionScript
  (Rendering|SetVisibility (Variables|Default|GetChildActor) false false))