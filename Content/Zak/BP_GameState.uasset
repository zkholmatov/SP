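; Game state that tracks boss deaths and level reveal, persisting them through the game instance's save and load requests.
; InitiateBinds hooks enemy, boss and dialogue dispatchers, reapplies the reveal, and passes boss flags to lifts and teleportals via interface.
; RevealLevel switches World Partition data layers at runtime, then requests a save.
; Player death, purge and boss death events only run delays, and boss-death flags are set through nested checks.
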(event Custom|PlayerDeath
  (if true
    (Utilities|FlowControl|Delay 2.5)))

(event Custom|Purge
  (if (not (Variables|Default|GetPurge?))
    (Variables|Default|SetPurge? true)
    (Utilities|FlowControl|Delay 4.0)))

(event Custom|FirstBossDeath
  (if (not (Variables|Default|GetFirstBossDeath?))
    (Variables|Default|SetFirstBossDeath? true)
    (Utilities|FlowControl|Delay 4.0)))

(event Custom|SecondBossDeath
  (if (not (Variables|Default|GetSecondBossDeath?))
    (Variables|Default|SetSecondBossDeath? true)
    (Utilities|FlowControl|Delay 4.0)))

(event Custom|InitiateBinds
  ;[1 1 1] Event dispatcher bindings
  (Utilities|FlowControl|Sequence
    (:then_0
      (bind _outactors (Actor|GetAllActorsOfClass "/Game/Mason/AI_SystemTwo/BP_EnemyOne.BP_EnemyOne_C"))
      (for _array_element _outactors
        (EventDispatchers|BindEventtoOnEnemyDeath _array_element (EventDispatchers|CreateEvent :!event Custom|Purge))))
    (:then_1
      (bind _outactors_2 (Actor|GetAllActorsOfClass "/Game/Mason/AI_SystemTwo/Enemy4/BP_EnemyFour.BP_EnemyFour_C"))
      (for _array_element_2 _outactors_2
        (EventDispatchers|BindEventtoOnBossDeath _array_element_2 (EventDispatchers|CreateEvent :!event Custom|FirstBossDeath))))
    (:then_2
      (bind _outactors_3 (Actor|GetAllActorsOfClass "/Game/Zak/AbyssalWarden/BP_AbyssalWarden.BP_AbyssalWarden_C"))
      (for _array_element_3 _outactors_3
        (EventDispatchers|BindEventtoOnBossDeath _array_element_3 (EventDispatchers|CreateEvent :!event Custom|SecondBossDeath))))
    (:then_3
      (bind _outactors_4 (Actor|GetAllActorsOfClass "/Game/Zak/BP_Dialogue.BP_Dialogue_C"))
      (for _array_element_4 _outactors_4
        (EventDispatchers|AssignOnDialogueStarted _array_element_4 (EventDispatchers|CreateEvent :!event Custom|RevealLevel))))
    (:then_4
      (if (Variables|Default|GetLevelRevealed?)
        (CallFunction|RevealLevel)))
    (:then_5
      (bind _outactors_5 (Actor|GetAllActorsOfClass "/Game/Mason/BP_Lift.BP_Lift_C"))
      (for _array_element_5 _outactors_5
        (Class|BPIBossIsDead|BPIBossIsDead(Message) _array_element_5 (Variables|Default|GetMyre%20Dead) (Variables|Default|GetWarden%20Dead) (Variables|Default|GetFinal%20Boss%20Dead)))
      (bind _outactors_6 (Actor|GetAllActorsOfClass "/Game/IntroMap/Blueprints/BP_Teleportal.BP_Teleportal_C"))
      (for _array_element_6 _outactors_6
        (Class|BPIBossIsDead|BPIBossIsDead(Message) _array_element_6 (Variables|Default|GetMyre%20Dead) (Variables|Default|GetWarden%20Dead) (Variables|Default|GetFinal%20Boss%20Dead))))
    (:then_6
      (if (not (Variables|Default|GetFirstBossDeath?))
        (bind _returnvalue (Actor|GetActorOfClass "/Game/Zak/Interractible/BP_BossArena.BP_BossArena_C"))
        (Default|BossDefeated _returnvalue)))))

(event Custom|RevealLevel
  (Variables|Default|SetLevelRevealed? true)
  (bind _returnvalue (WorldPartition|GetDataLayerManager)) ; get data layer manager for world level partition as reference to set data layer in runtime
  (DataLayers|SetDataLayerRuntimeState _returnvalue (Variables|Default|GetOutDataLayerAsset) "Loaded" false :!class /Script/Engine.DataLayerManager) ; Function to toggle data layers
  (bind _returnvalue_2 (WorldPartition|GetDataLayerManager)) ; get data layer manager for world level partition as reference to set data layer in runtime
  (DataLayers|SetDataLayerRuntimeState _returnvalue_2 (Variables|Default|GetInDataLayerAsset) "Activated" false :!class /Script/Engine.DataLayerManager) ; Function to toggle data layers
  (Default|RequestSave (Variables|Default|GetAs%20BP%20Game%20Instance) true))

(event EventBeginPlay
  (bind _asbp_player (Utilities|Casting|CastToBP_Player (Game|GetPlayerCharacter 0))
    (:then
      (EventDispatchers|BindEventtoOnPlayerDeath _asbp_player (EventDispatchers|CreateEvent :!event Custom|PlayerDeath)))
    (:CastFailed
      _))
  (bind _asbp_game_instance (Utilities|Casting|CastToBP_GameInstance (Game|GetGameInstance)))
  (bind _output_get (Variables|Default|SetAs%20BP%20Game%20Instance _asbp_game_instance))
  (Default|RequestLoad _output_get self))

(event EventLoadData
  (params (SaveGameRef :type BP%20Save%20Game%20Object%20Reference))
  (Variables|Default|SetLevelRevealed? (Variables|/Game/Zak/SaveGame/BP_SaveGame.BP_SaveGame_C|GetLevelRevealed? SaveGameRef))
  (Variables|Default|SetMyre%20Dead (Variables|/Game/Zak/SaveGame/BP_SaveGame.BP_SaveGame_C|GetMyreDead SaveGameRef))
  (Variables|Default|SetWarden%20Dead (Variables|/Game/Zak/SaveGame/BP_SaveGame.BP_SaveGame_C|GetWardenDead SaveGameRef))
  (Variables|Default|SetFinal%20Boss%20Dead (Variables|/Game/Zak/SaveGame/BP_SaveGame.BP_SaveGame_C|GetFinalBossDead SaveGameRef)))

(event EventSaveData
  (params (SaveGameRef :type BP%20Save%20Game%20Object%20Reference))
  (Variables|/Game/Zak/SaveGame/BP_SaveGame.BP_SaveGame_C|SetLevelRevealed? SaveGameRef (Variables|Default|GetLevelRevealed?))
  (Variables|/Game/Zak/SaveGame/BP_SaveGame.BP_SaveGame_C|SetMyreDead SaveGameRef (Variables|Default|GetMyre%20Dead))
  (Variables|/Game/Zak/SaveGame/BP_SaveGame.BP_SaveGame_C|SetWardenDead SaveGameRef (Variables|Default|GetWarden%20Dead))
  (Variables|/Game/Zak/SaveGame/BP_SaveGame.BP_SaveGame_C|SetFinalBossDead SaveGameRef (Variables|Default|GetFinal%20Boss%20Dead)))

(event EventBPIBossIsDead
  (params (myre :type Boolean) (warden :type Boolean) (finalBoss :type Boolean))
  ;[0.08523 1 0.08627] interface call from bosses
  (if myre
    (Variables|Default|SetMyre%20Dead myre)
    (if warden
      (Variables|Default|SetWarden%20Dead warden)
      (if finalBoss
        (Variables|Default|SetFinal%20Boss%20Dead finalBoss)))))

(fn ConstructionScript)