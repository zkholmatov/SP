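; BP_Dialogue is a placeable trigger that plays a spatialized dialogue sound once, when the player first enters its sphere.
; It fires dialogue started and finished calls around a delay of the dialogue's duration, then requests a save through BP_GameInstance.
; Heard lines persist by adding the actor's display name to the save, which is matched on load to block replays.
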(event OnComponentBeginOverlap(Sphere)
  (params (OverlappedComponent :type Primitive%20Component%20Object%20Reference) (OtherActor :type Actor%20Object%20Reference) (OtherComp :type Primitive%20Component%20Object%20Reference) (OtherBodyIndex :type Integer) (bFromSweep :type Boolean) (SweepResult :type Hit%20Result%20Structure%20%28by%20ref%29))
  (Utilities|Casting|CastToBP_Player OtherActor)
  (if (not (Variables|Default|GetHeardDialogue?))
    (Variables|Default|SetHeardDialogue? true)
    (Variables|Default|SetInteracted? true)
    (Audio|PlaySoundatLocation (Variables|Default|GetSound) (Transformation|GetActorLocation) "0, 0, 0" 0.5 1.0 0.0 "/Game/Zak/NPC/Dialogue.Dialogue" 0 0 0)
    (Default|CallOnDialogueStarted)
    (Utilities|FlowControl|Delay (Variables|Default|GetDialogueDuration))
    (Default|CallOnDialogueFinished)
    (Default|RequestSave (Variables|Default|GetAs%20BP%20Game%20Instance) true)))

(event EventBeginPlay
  (bind _asbp_game_instance (Utilities|Casting|CastToBP_GameInstance (Game|GetGameInstance)))
  (bind _output_get (Variables|Default|SetAs%20BP%20Game%20Instance _asbp_game_instance))
  (Default|RequestLoad _output_get self))

(event EventSaveData
  (params (SaveGameRef :type BP%20Save%20Game%20Object%20Reference))
  (if (Variables|Default|GetInteracted?)
    (Utilities|Array|AddUnique (.dialoguename (Variables|/Game/Zak/SaveGame/BP_SaveGame.BP_SaveGame_C|GetDialogueSave SaveGameRef)) (Utilities|GetDisplayName self))))

(event EventLoadData
  (params (SaveGameRef :type BP%20Save%20Game%20Object%20Reference))
  (for _array_element (.dialoguename (Variables|/Game/Zak/SaveGame/BP_SaveGame.BP_SaveGame_C|GetDialogueSave SaveGameRef))
    (if (Utilities|Enum|Equal(Enum) _array_element (Utilities|GetDisplayName self))
      (Variables|Default|SetHeardDialogue? true))))

(fn ConstructionScript)