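; Weapon Blueprint that configures its combat stats and type-specific attack setup from an item data table.
; On BeginPlay it reads its DT_Items row, then uses the weapon type (great sword, sword or dagger) to pick animation set, socket name and combo montages.
; EnableTrail spawns an attached particle trail centered, oriented and sized from the mesh's VFXStart and VFXEnd sockets.
; The construction script binds to OnEnableTrail.
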(event Custom|EnableTrail
  (bind _weapon (Variables|Default|GetWeapon))
  (bind _returnvalue (Transformation|GetSocketLocation _weapon "VFXStart"))
  (bind _returnvalue_2 (Transformation|GetSocketLocation _weapon "VFXEnd"))
  (bind _returnvalue_3 (- _returnvalue _returnvalue_2))
  (bind _returnvalue_4 (Niagara|SpawnSystemAttached (Variables|Default|GetParticleSystem) _weapon "None" (/ (+ _returnvalue _returnvalue_2) 2.0) (Math|Rotator|MakeRotfromZ _returnvalue_3) "KeepWorldPosition" true))
  (Effects|Components|ParticleSystem|SetFloatParameter _returnvalue_4 "TrailWidth" (Math|Vector|VectorLength _returnvalue_3)))

(event EventBeginPlay
  (bind _returnvalue (Utilities|GetDataTableRow "/Game/Omar/Inventory/DataTables/DT_Items.DT_Items" (Variables|Default|GetDataTableRowName))
    (:then
      (Variables|Default|SetAttack (.Attack (Utilities|Struct|BreakS_Item _returnvalue)))
      (Variables|Default|SetCritChance (.CritChance (Utilities|Struct|BreakS_Item _returnvalue)))
      (Variables|Default|SetCritDamage (.CritDamage (Utilities|Struct|BreakS_Item _returnvalue)))
      (bind _output_get (Variables|Default|SetWeaponType (.WeaponType (Utilities|Struct|BreakS_Item _returnvalue))))
      (switch Utilities|FlowControl|Switch|SwitchonE_WeaponTypes _output_get
        (:NewEnumerator0
          (Variables|Default|SetAnimationSet 0)
          (Variables|Default|SetSocketName "GreatswordSocket")
          ;[1 1 1] GreatCombo1
          (Variables|Default|SetAttackCombo (Utilities|Array|MakeArray "/Game/Zak/Player/AnimGreatsword/AttackCombo1/AS_Combo_Attack_01_01_Seq_Montage.AS_Combo_Attack_01_01_Seq_Montage" "/Game/Zak/Player/AnimGreatsword/AttackCombo1/AS_Combo_Attack_01_02_Seq_Montage.AS_Combo_Attack_01_02_Seq_Montage" "/Game/Zak/Player/AnimGreatsword/AttackCombo1/AS_Combo_Attack_01_03_Seq_Montage.AS_Combo_Attack_01_03_Seq_Montage" "/Game/Zak/Player/AnimGreatsword/AttackCombo1/AS_Combo_Attack_01_04_Seq_Montage.AS_Combo_Attack_01_04_Seq_Montage")))
        (:NewEnumerator1
          (Variables|Default|SetAnimationSet 1)
          (Variables|Default|SetSocketName "SwordSocket")
          ;[1 1 1] SwordCombo4
          (Variables|Default|SetAttackCombo (Utilities|Array|MakeArray "/Game/Zak/Player/AnimSword/AttackCombo4/Combo_Attack_04_01_Seq1_Montage.Combo_Attack_04_01_Seq1_Montage" "/Game/Zak/Player/AnimSword/AttackCombo4/Combo_Attack_04_02_Seq1_Montage.Combo_Attack_04_02_Seq1_Montage" "/Game/Zak/Player/AnimSword/AttackCombo4/Combo_Attack_04_03_Seq_Montage.Combo_Attack_04_03_Seq_Montage" "/Game/Zak/Player/AnimSword/AttackCombo4/Combo_Attack_04_04_Seq_Montage.Combo_Attack_04_04_Seq_Montage")))
        (:NewEnumerator2
          (Variables|Default|SetAnimationSet 2)
          (Variables|Default|SetSocketName "DaggerSocket_R")
          ;[1 1 1] DaggerCombo1
          (Variables|Default|SetAttackCombo (Utilities|Array|MakeArray "/Game/Zak/Player/AnimDagger/AttackCombo1/AS_Combo_Attack_01_01_Seq_Montage.AS_Combo_Attack_01_01_Seq_Montage" "/Game/Zak/Player/AnimDagger/AttackCombo1/AS_Combo_Attack_01_02_Seq_Montage.AS_Combo_Attack_01_02_Seq_Montage" "/Game/Zak/Player/AnimDagger/AttackCombo1/AS_Combo_Attack_01_03_Seq_Montage.AS_Combo_Attack_01_03_Seq_Montage" "/Game/Zak/Player/AnimDagger/AttackCombo1/AS_Combo_Attack_01_04_Seq_Montage.AS_Combo_Attack_01_04_Seq_Montage")))))))

(fn ConstructionScript
  (EventDispatchers|BindEventtoOnEnableTrail (EventDispatchers|CreateEvent :!event Custom|EnableTrail)))