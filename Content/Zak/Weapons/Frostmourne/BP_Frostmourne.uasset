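; Frostmourne weapon Blueprint, configuring its parent weapon class with a trace radius, Niagara trail, data table row and four-montage attack combo.
; On BeginPlay it creates a dynamic weapon material and binds events to the player's light, heavy, charged, jump and sprint attack dispatchers.
; StartGlow pulses the material's color parameter by chaining the Glow timeline into GlowReverse.
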(event Custom|StartGlow
  (bind _amount (Timeline|Glow PlayFromStart)
    (:Update
      (Rendering|Material|SetVectorParameterValue (Variables|Default|GetMaterial) "color" (Utilities|Struct|MakeLinearColor 0.0 0.0 _amount 1.0) :!class /Script/Engine.MaterialInstanceDynamic))
    (:Finished
      (bind _amount_2 (Timeline|GlowReverse PlayFromStart)
        (:Update
          (Rendering|Material|SetVectorParameterValue (Variables|Default|GetMaterial) "color" (Utilities|Struct|MakeLinearColor 0.0 0.0 _amount_2 1.0) :!class /Script/Engine.MaterialInstanceDynamic))))))

(event EventBeginPlay
  (Variables|Default|SetTraceRadius 2e+01)
  (bind _returnvalue (Rendering|Material|CreateDynamicMaterialInstance (Variables|Default|GetWeapon) 0 "/Game/Zak/Weapons/Frostmourne/frostmourne1_Inst.frostmourne1_Inst" "None" :!class /Script/Engine.PrimitiveComponent))
  (Variables|Default|SetMaterial _returnvalue)
  (Variables|Default|SetParticleSystem "/Game/Zak/VFX/Niagara/WeaponFX/NS_FrostmourneTrail.NS_FrostmourneTrail")
  (Variables|Default|SetDataTableRowName "Frostmourne")
  (bind _asbp_player (Utilities|Casting|CastToBP_Player (Game|GetPlayerCharacter 0)))
  (Variables|Default|SetAs%20BP%20Player _asbp_player)
  (EventDispatchers|BindEventtoOnLightAttack (Variables|Default|GetAs%20BP%20Player) (EventDispatchers|CreateEvent :!event Custom|StartGlow))
  (EventDispatchers|BindEventtoOnHeavyAttack (Variables|Default|GetAs%20BP%20Player) (EventDispatchers|CreateEvent :!event Custom|StartGlow))
  (EventDispatchers|BindEventtoOnChargedAttack (Variables|Default|GetAs%20BP%20Player) (EventDispatchers|CreateEvent :!event Custom|StartGlow))
  (EventDispatchers|BindEventtoOnJumpAttack (Variables|Default|GetAs%20BP%20Player) (EventDispatchers|CreateEvent :!event Custom|StartGlow))
  (EventDispatchers|BindEventtoOnSprintAttack (Variables|Default|GetAs%20BP%20Player) (EventDispatchers|CreateEvent :!event Custom|StartGlow))
  (|CallParentFunction)
  ;[1 1 1] GreatCombo3
  (Variables|Default|SetAttackCombo (Utilities|Array|MakeArray "/Game/Zak/Player/AnimGreatsword/AttackCombo3/AS_Combo_Attack_03_01_Seq_Montage.AS_Combo_Attack_03_01_Seq_Montage" "/Game/Zak/Player/AnimGreatsword/AttackCombo3/AS_Combo_Attack_03_02_Seq_Montage.AS_Combo_Attack_03_02_Seq_Montage" "/Game/Zak/Player/AnimGreatsword/AttackCombo3/AS_Combo_Attack_03_03_Seq_Montage.AS_Combo_Attack_03_03_Seq_Montage" "/Game/Zak/Player/AnimGreatsword/AttackCombo3/AS_Combo_Attack_03_04_Seq_Montage.AS_Combo_Attack_03_04_Seq_Montage")))

(fn ConstructionScript
  (|CallParentFunction))