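; Abyssal Blade weapon Blueprint that configures its parent weapon class with the blade's trail effect, data table row and combo attacks.
; On BeginPlay it sets those values, calling the parent logic before filling in a four-montage attack combo.
; It also attaches a Niagara effect midway between the weapon's VFXStart and VFXEnd sockets, oriented along that line with trail width matched to their distance.
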(event EventBeginPlay
  (bind _weapon (Variables|Default|GetWeapon))
  (bind _returnvalue (Transformation|GetSocketLocation _weapon "VFXStart"))
  (bind _returnvalue_2 (Transformation|GetSocketLocation _weapon "VFXEnd"))
  (bind _returnvalue_3 (- _returnvalue _returnvalue_2))
  (Variables|Default|SetParticleSystem "/Game/Zak/VFX/Niagara/WeaponFX/NS_AbyssalBladeTrail.NS_AbyssalBladeTrail")
  (Variables|Default|SetDataTableRowName "AbyssalBlade")
  (|CallParentFunction)
  (bind _returnvalue_4 (Niagara|SpawnSystemAttached "/Game/Zak/VFX/Niagara/WeaponFX/NS_AbyssalBlade.NS_AbyssalBlade" _weapon "None" (/ (+ _returnvalue _returnvalue_2) 2.0) (Math|Rotator|MakeRotfromZ _returnvalue_3) "KeepWorldPosition" true))
  (Effects|Components|ParticleSystem|SetFloatParameter _returnvalue_4 "TrailWidth" (Math|Vector|VectorLength _returnvalue_3))
  ;[1 1 1] GreatCombo2
  (Variables|Default|SetAttackCombo (Utilities|Array|MakeArray "/Game/Zak/Player/AnimGreatsword/AttackCombo2/AS_Combo_Attack_02_01_Seq_Montage.AS_Combo_Attack_02_01_Seq_Montage" "/Game/Zak/Player/AnimGreatsword/AttackCombo2/AS_Combo_Attack_02_02_Seq_Montage.AS_Combo_Attack_02_02_Seq_Montage" "/Game/Zak/Player/AnimGreatsword/AttackCombo2/AS_Combo_Attack_02_03_Seq_Montage.AS_Combo_Attack_02_03_Seq_Montage" "/Game/Zak/Player/AnimGreatsword/AttackCombo2/AS_Combo_Attack_02_04_Seq_Montage.AS_Combo_Attack_02_04_Seq_Montage")))

(fn ConstructionScript
  (|CallParentFunction))