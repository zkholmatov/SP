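; BP_TwinBlades is a twin-blade weapon child Blueprint that configures its parent weapon logic for the TwilightRequiem data table row.
; Its construction script enables and assigns a second mesh, while BeginPlay sets the row name and trace radius before calling the parent.
; The trail enable and disable events are empty, and an unconnected chain holds unused Niagara code for a void dagger trail sized between two weapon sockets.
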(event Custom|DisableTrail_1)

(event EventBeginPlay
  (Variables|Default|SetDataTableRowName "TwilightRequiem")
  (Variables|Default|SetTraceRadius 1e+01)
  (|CallParentFunction))

(event EventEnableTrail)

(fn ConstructionScript
  (Variables|Default|SetSecondMesh "/Game/Zak/Weapons/TwinBlade/Black.Black")
  (Variables|Default|SetHasSecondMesh? true)
  (|CallParentFunction))