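; BP_Sword is a sword Blueprint that caches a reference to the player's BP_Player on BeginPlay.
; Its glow logic is disconnected: Tick is empty, and neither the dynamic red-material setup nor the color update runs.
; That unused logic would set the material color's blue channel high while attacking, ramp it by timeline while charging, and reverse the timeline otherwise.
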(event EventBeginPlay
  (bind _asbp_player (Utilities|Casting|CastToBP_Player (Game|GetPlayerCharacter 0)))
  (Variables|Default|SetAs%20BP%20Player _asbp_player))

(event EventTick
  (params (DeltaSeconds :type Float%20%28single-precision%29)))

(fn ConstructionScript)