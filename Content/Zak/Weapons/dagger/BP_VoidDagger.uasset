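; BP_VoidDagger is the Void Dagger weapon, a child Blueprint that mostly relies on its parent class.
; BeginPlay sets the data table row name to VoidDagger before calling the parent BeginPlay.
; EnableTrail and DisableTrail_1 are empty overrides.
; Disconnected leftover nodes would spawn an attached NS_VoidDagger Niagara trail between the weapon's VFX sockets and size its width from their distance, but they never run.
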(event Custom|DisableTrail_1)

(event EventBeginPlay
  (Variables|Default|SetDataTableRowName "VoidDagger")
  (|CallParentFunction))

(event EventEnableTrail)

(fn ConstructionScript
  (|CallParentFunction))