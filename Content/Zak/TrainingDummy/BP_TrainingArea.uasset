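; BP_TrainingArea is a trigger volume that shows extra content in the player HUD's controls list while the player is inside it.
; On BeginPlay it caches the first player controller's HUD as BPC_PlayerHUD.
; Box overlaps with BP_Player add the Content widget to the Controls vertical box on entry and remove it on exit.
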(event OnComponentBeginOverlap(Box)
  (params (OverlappedComponent :type Primitive%20Component%20Object%20Reference) (OtherActor :type Actor%20Object%20Reference) (OtherComp :type Primitive%20Component%20Object%20Reference) (OtherBodyIndex :type Integer) (bFromSweep :type Boolean) (SweepResult :type Hit%20Result%20Structure%20%28by%20ref%29))
  (Utilities|Casting|CastToBP_Player OtherActor)
  (Class|VerticalBox|AddChildtoVerticalBox (Variables|/Game/Zak/UI/W_PlayerHUD.W_PlayerHUD_C|GetControls (Variables|/Game/Zak/UI/BPC_PlayerHUD.BPC_PlayerHUD_C|GetPlayerHUD (Variables|Default|GetAs%20BPC%20Player%20HUD))) (Variables|Default|GetContent)))

(event OnComponentEndOverlap(Box)
  (params (OverlappedComponent :type Primitive%20Component%20Object%20Reference) (OtherActor :type Actor%20Object%20Reference) (OtherComp :type Primitive%20Component%20Object%20Reference) (OtherBodyIndex :type Integer))
  (Utilities|Casting|CastToBP_Player OtherActor)
  (Class|PanelWidget|RemoveChild (Variables|/Game/Zak/UI/W_PlayerHUD.W_PlayerHUD_C|GetControls (Variables|/Game/Zak/UI/BPC_PlayerHUD.BPC_PlayerHUD_C|GetPlayerHUD (Variables|Default|GetAs%20BPC%20Player%20HUD))) (Variables|Default|GetContent)))

(event EventBeginPlay
  (bind _asbpc_player_hud (Utilities|Casting|CastToBPC_PlayerHUD (HUD|GetHUD (Game|GetPlayerController 0))))
  (Variables|Default|SetAs%20BPC%20Player%20HUD _asbpc_player_hud))

(fn ConstructionScript)