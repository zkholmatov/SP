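; Tutorial enemy dummy that shows the player a controls task list, then arms itself and fights back once the tasks are complete.
; A looping timer drives montage attacks in range, with notifies toggling timer-based sword sphere traces that deal parryable damage.
; BPCDamageSystem drives directional hit reactions, while health refills after a delay or death; low health allows executions that shatter the dummy.
; One-time block, heal and execute hints pause the game and save progress.
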(event OnComponentBeginOverlap(CombatRadius)
  (params (OverlappedComponent :type Primitive%20Component%20Object%20Reference) (OtherActor :type Actor%20Object%20Reference) (OtherComp :type Primitive%20Component%20Object%20Reference) (OtherBodyIndex :type Integer) (bFromSweep :type Boolean) (SweepResult :type Hit%20Result%20Structure%20%28by%20ref%29))
  ;[1 1 1] Within Radius Overlap
  (Utilities|Casting|CastToBP_Player OtherActor)
  (Rendering|SetVisibility (Variables|Default|GetHealthWidget) true false)
  (if (not (Variables|Default|GetTutorialComplete?))
    (Class|VerticalBox|AddChildtoVerticalBox (Variables|/Game/Zak/UI/W_PlayerHUD.W_PlayerHUD_C|GetControls (Variables|/Game/Zak/UI/BPC_PlayerHUD.BPC_PlayerHUD_C|GetPlayerHUD (Variables|Default|GetAs%20BPC%20Player%20HUD))) (Variables|Default|GetControls))))

(event OnComponentEndOverlap(CombatRadius)
  (params (OverlappedComponent :type Primitive%20Component%20Object%20Reference) (OtherActor :type Actor%20Object%20Reference) (OtherComp :type Primitive%20Component%20Object%20Reference) (OtherBodyIndex :type Integer))
  ;[1 1 1] Within Radius Overlap
  (Utilities|Casting|CastToBP_Player OtherActor)
  (Rendering|SetVisibility (Variables|Default|GetHealthWidget) false false))

(event OnComponentBeginOverlap(AttackRadius)
  (params (OverlappedComponent :type Primitive%20Component%20Object%20Reference) (OtherActor :type Actor%20Object%20Reference) (OtherComp :type Primitive%20Component%20Object%20Reference) (OtherBodyIndex :type Integer) (bFromSweep :type Boolean) (SweepResult :type Hit%20Result%20Structure%20%28by%20ref%29))
  ;[1 1 1] Within Radius Overlap
  (Utilities|Casting|CastToBP_Player OtherActor)
  (Variables|Default|SetWithinRange? true))

(event OnComponentEndOverlap(AttackRadius)
  (params (OverlappedComponent :type Primitive%20Component%20Object%20Reference) (OtherActor :type Actor%20Object%20Reference) (OtherComp :type Primitive%20Component%20Object%20Reference) (OtherBodyIndex :type Integer))
  ;[1 1 1] Within Radius Overlap
  (Utilities|Casting|CastToBP_Player OtherActor)
  (Variables|Default|SetWithinRange? false))

(event Custom|HealHint
  (if (not (Variables|Default|GetHealExplained?))
    (Class|VerticalBox|AddChildtoVerticalBox (Variables|/Game/Zak/UI/W_PlayerHUD.W_PlayerHUD_C|GetHints (Variables|/Game/Zak/UI/BPC_PlayerHUD.BPC_PlayerHUD_C|GetPlayerHUD (Variables|Default|GetAs%20BPC%20Player%20HUD))) (Variables|Default|GetHintHeal))
    (Variables|Default|SetHealExplained? true)
    (Default|RequestSave (Variables|Default|GetAs%20BP%20Game%20Instance%202) true)
    (Audio|PlaySound2D "/Engine/VREditor/Sounds/UI/Camera_Shutter.Camera_Shutter" 1.0 1.0 0.0 0 0)
    (Game|SetGamePaused true)))

(event Custom|StopAttack
  ;[1 1 1] Attack
  (Utilities|Time|ClearandInvalidateTimerbyHandle (stale Custom|Attack _returnvalue)))

(event Custom|StopSwordTrace
  ;[1 0.3137 0.3137 1 30] Trace
  (Utilities|Time|ClearandInvalidateTimerbyHandle (Variables|Default|GetNewVar)))

(event Custom|DamageResponse
  (params (DamageResponse :type E_DamageResponse%20Enum :default "NewEnumerator0") (DamageDirection :type E_DamageDirection%20Enum :default "NewEnumerator0") (DamageCauser :type Actor%20Object%20Reference))
  ;[1 1 1] Hit Reaction
  (CallFunction|StartRegen)
  (CallFunction|StopSwordTrace)
  (Variables|Default|SetStunned? true)
  (bind _newparam (CallFunction|SetHitReactionMontage DamageDirection))
  (Animation|Montage|PlayMontage (Variables|Character|GetMesh) _newparam
    (:OnCompleted
      (Variables|Default|SetStunned? false))))

(event Custom|Death
  (bind _bpc_damagesystem (Variables|Default|GetBPC_DamageSystem))
  ;[1 1 1] Death
  (Variables|/Game/Zak/DamageSystem/BPC_DamageSystem.BPC_DamageSystem_C|SetDead? _bpc_damagesystem false)
  (Default|SetMaxHealth _bpc_damagesystem (Variables|Default|GetHealth)))

(event Custom|RegenLoop
  ;[1 1 1] Regen
  (bind _output_get (Variables|Default|SetTemp (+ (Variables|Default|GetTemp) 0.1)))
  (if (>= _output_get 5.0)
    (Default|SetMaxHealth (Variables|Default|GetBPC_DamageSystem) (Variables|Default|GetHealth))
    (Variables|Default|SetTemp 0.0)
    (Utilities|Time|ClearandInvalidateTimerbyHandle (stale Custom|StartRegen _returnvalue))))

(event Custom|AllTasksComplete
  (Default|SetMaxHealth (Variables|Default|GetBPC_DamageSystem) (Variables|Default|GetHealth))
  (Variables|Default|SetTutorialComplete? true)
  (Variables|Default|SetStunned? false)
  (Class|PanelWidget|RemoveChild (Variables|/Game/Zak/UI/W_PlayerHUD.W_PlayerHUD_C|GetControls (Variables|/Game/Zak/UI/BPC_PlayerHUD.BPC_PlayerHUD_C|GetPlayerHUD (Variables|Default|GetAs%20BPC%20Player%20HUD))) (Variables|Default|GetControls))
  (bind _notifyname (Animation|Montage|PlayMontage (Variables|Character|GetMesh) "/Game/Zak/TrainingDummy/Anims/Idle_To_Idle_Combat_Seq_Montage.Idle_To_Idle_Combat_Seq_Montage")
    (:OnCompleted
      (Variables|Type|SetAttacker? true :!label _label))
    (:OnInterrupted
      (goto _label))
    (:OnNotifyBegin
      (switch name _notifyname
        (:Attack
          (goto _label))
        (:Wield
          (bind _returnvalue (Game|SpawnActorfromClass "/Game/Zak/Weapons/RedSword/BP_RedSword.BP_RedSword_C" (Transformation|GetActorTransform) "Undefined" "MultiplyWithRoot" 0 0))
          (bind _output_get (Variables|Default|SetAs%20BP%20Weapon _returnvalue))
          (Transformation|AttachComponentToComponent _output_get (Variables|Character|GetMesh) "WeaponSocket" "SnapToTarget" "SnapToTarget" "SnapToTarget" true))))))

(event Custom|StartSwordTrace
  ;[1 0.3137 0.3137 1 30] Trace
  (Default|EnableTrail (Variables|Default|GetAs%20BP%20Weapon))
  (bind _returnvalue (Utilities|Time|SetTimerbyEvent (delegate Custom|SwordTraceLoop) 0.01 true))
  (Variables|Default|SetNewVar _returnvalue))

(event Custom|SwordTraceLoop
  (bind _as_bp_weapon (Variables|Default|GetAs%20BP%20Weapon))
  (bind _weapon (Variables|/Game/Zak/Weapons/BP_Weapon.BP_Weapon_C|GetWeapon _as_bp_weapon))
  ;[1 0.3137 0.3137 1 30] Trace
  (bind (_outhit _returnvalue) (Collision|SphereTraceForObjects (Transformation|GetSocketLocation _weapon "TrailStart") (Transformation|GetSocketLocation _weapon "TrailEnd") 1e+01 (Utilities|Array|MakeArray "ObjectTypeQuery3") false 0 "None" true "(R=1.000000,G=0.000000,B=0.000000,A=1.000000)" "(R=0.000000,G=1.000000,B=0.000000,A=1.000000)" 2.0))
  (if _returnvalue
    (CallFunction|StopSwordTrace)
    (bind _wasdamaged_ (Class|BPIDamageable|TakeDamage(Message) (.HitActor (Collision|BreakHitResult _outhit)) (Utilities|Struct|MakeS_DamageInfo 5e+01 "NewEnumerator1" "NewEnumerator3" true false (CallFunction|CalculateDamageDirection (Variables|Default|GetAs%20BP%20Weapon) (.HitActor (Collision|BreakHitResult _outhit))) self)))
    (if _wasdamaged_
      (Niagara|SpawnSystematLocation "/Game/Zak/VFX/Niagara/NS_Hit.NS_Hit" (.ImpactPoint (Collision|BreakHitResult _outhit))))))

(event Custom|SavingCompleted
  (params (SaveGameRef :type BP%20Save%20Game%20Object%20Reference))
  ;[1 1 1] Attack
  (Audio|PlaySound2D "/Engine/VREditor/Sounds/UI/Camera_Shutter.Camera_Shutter" 1.0 1.0 0.0 0 0))

(event Custom|LockLoop
  (bind _mesh (Variables|Character|GetMesh))
  ;[1 1 1] Target Lock
  (Utilities|IsValid _mesh
    (:Is%20Valid
      (Transformation|SetWorldLocation (Variables|/Game/Zak/UI/BP_TargetLock.BP_TargetLock_C|GetTargetLockWidget (Variables|Default|GetTargetLockWidget)) (Transformation|GetSocketLocation _mesh "spine_05") false false))))

(event Custom|AttackLoop
  (bind _as_bp_game_instance_2 (Variables|Default|GetAs%20BP%20Game%20Instance%202))
  ;[1 1 1] Attack
  (if (Math|Boolean|ANDBoolean (not (Variables|Default|GetAttacking?)) (not (Variables|Default|GetStunned?)) (not (Variables|Default|GetExecuted?)) (Variables|Default|GetWithinRange?) (Variables|Type|GetAttacker?))
    (Variables|Default|SetAttacking? true)
    (bind _notifyname (Animation|Montage|PlayMontage (Variables|Character|GetMesh) "/Game/Zak/TrainingDummy/Anims/Combo_Attack_04_01_Seq_Montage.Combo_Attack_04_01_Seq_Montage")
      (:OnCompleted
        (Variables|Default|SetAttacking? false :!label _label)
        (if (Variables|Default|GetWithinRange?)
          _))
      (:OnInterrupted
        (goto _label))
      (:OnNotifyBegin
        (switch name _notifyname
          (:Hint
            (if (not (Variables|Default|GetBlockExplained?))
              (Class|VerticalBox|AddChildtoVerticalBox (Variables|/Game/Zak/UI/W_PlayerHUD.W_PlayerHUD_C|GetHints (Variables|/Game/Zak/UI/BPC_PlayerHUD.BPC_PlayerHUD_C|GetPlayerHUD (Variables|Default|GetAs%20BPC%20Player%20HUD))) (Variables|Default|GetHintBlock))
              (Variables|Default|SetBlockExplained? true)
              (Game|SetGamePaused true)
              (EventDispatchers|BindEventtoOnGameSaved _as_bp_game_instance_2 (delegate Custom|SavingCompleted))
              (Default|RequestSave _as_bp_game_instance_2 true)))
          (:TraceStart
            (CallFunction|StartSwordTrace))
          (:TraceEnd
            (CallFunction|StopSwordTrace)))))))

(event Custom|StartRegen
  ;[1 1 1] Regen
  (Variables|Default|SetTemp 0.0)
  (bind _returnvalue (Utilities|Time|SetTimerbyEvent (delegate Custom|RegenLoop) 0.1 true)))

(event Custom|Attack
  ;[1 1 1] Attack
  (bind _returnvalue (Utilities|Time|SetTimerbyEvent (delegate Custom|AttackLoop) 2.0 true false -1.0)))

(event EventBeginPlay
  ;[1 1 1] Setup
  (bind _asbp_game_instance (Utilities|Casting|CastToBP_GameInstance (Game|GetGameInstance)))
  (Variables|Default|SetAs%20BP%20Game%20Instance%202 _asbp_game_instance)
  (Class|BPIPersistence|RequestLoad(Message) (Game|GetGameInstance) self)
  (Variables|/Game/Zak/DamageSystem/BPC_DamageSystem.BPC_DamageSystem_C|SetInvincible? (Variables|Default|GetBPC_DamageSystem) false)
  (bind _asbpc_player_hud (Utilities|Casting|CastToBPC_PlayerHUD (HUD|GetHUD (Game|GetPlayerController 0))))
  (Variables|Default|SetAs%20BPC%20Player%20HUD _asbpc_player_hud)
  (Utilities|FlowControl|Sequence
    (:then_0
      (bind _asbp_player (Utilities|Casting|CastToBP_Player (Game|GetPlayerCharacter 0)))
      (bind _output_get (Variables|Default|SetAs%20BP%20Player _asbp_player))
      (EventDispatchers|BindEventtoOnDamageTaken _output_get (EventDispatchers|CreateEvent :!event Custom|HealHint))
      (if (Variables|Default|GetTutorialComplete?)
        (Variables|Type|SetAttacker? true)
        (bind _returnvalue (Game|SpawnActorfromClass "/Game/Zak/Weapons/FalseGod/BP_FalseGod.BP_FalseGod_C" (Transformation|GetActorTransform) "Undefined" "MultiplyWithRoot" 0 0))
        (bind _output_get_2 (Variables|Default|SetAs%20BP%20Weapon _returnvalue))
        (Transformation|AttachComponentToComponent _output_get_2 (Variables|Character|GetMesh) "WeaponSocket" "SnapToTarget" "SnapToTarget" "SnapToTarget" true)))
    (:then_1
      (bind _returnvalue_2 (Game|SpawnActorfromClass "/Game/Zak/UI/BP_TargetLock.BP_TargetLock_C" (Math|Transform|MakeTransform (Transformation|GetSocketLocation (Variables|Character|GetMesh) "spine_05") "0, 0, 0" "1.000000,1.000000,1.000000") "Undefined" "MultiplyWithRoot" 0 0))
      (Variables|Default|SetTargetLockWidget _returnvalue_2)
      (Default|SetMaxHealth (Variables|Default|GetBPC_DamageSystem) (Variables|Default|GetHealth))
      (bind _returnvalue_3 (UserInterface|CreateWidget "/Game/Omar/UI/WidgetBlueprints/WB_HealthBar.WB_HealthBar_C" 0 self))
      (UserInterface|SetWidget (Variables|Default|GetHealthWidget) _returnvalue_3)
      (bind _returnvalue_4 (UserInterface|CreateWidget "/Game/Zak/UI/W_Execution.W_Execution_C"))
      (UserInterface|SetWidget (Variables|Default|GetExecuteWidget) _returnvalue_4)
      (CallFunction|Attack))))

(event EventUnlock
  ;[1 1 1] Target Lock
  (Rendering|SetVisibility (Variables|/Game/Zak/UI/BP_TargetLock.BP_TargetLock_C|GetTargetLockWidget (Variables|Default|GetTargetLockWidget)) false false)
  (Utilities|Time|ClearandInvalidateTimerbyHandle (stale EventLock _returnvalue)))

(event EventLock
  ;[1 1 1] Target Lock
  (Rendering|SetVisibility (Variables|/Game/Zak/UI/BP_TargetLock.BP_TargetLock_C|GetTargetLockWidget (Variables|Default|GetTargetLockWidget)) true false)
  (bind _returnvalue (Utilities|Time|SetTimerbyEvent (delegate Custom|LockLoop) 0.01 true)))

(event EventExecution
  (params (ExecutionSequence :type Integer))
  ;[1 1 1 1 30] Execution
  (switch int ExecutionSequence
    (:0
      (Variables|Default|SetExecutionSequence 0))
    (:1
      (Variables|Default|SetExecutionSequence 1))
    (:2
      (Variables|Default|SetExecutionSequence 2)))
  (Transformation|SetActorRotation (Math|Rotator|MakeRotator 0.0 0.0 (.yaw (Math|Rotator|FindLookatRotation (Transformation|GetActorLocation) (Transformation|GetActorLocation (Game|Player|GetPlayerPawn 0))))))
  (Variables|Default|SetExecuted? true)
  (Variables|/Game/Zak/DamageSystem/BPC_DamageSystem.BPC_DamageSystem_C|SetInvincible? (Variables|Default|GetBPC_DamageSystem) true)
  (Transformation|DetachFromComponent (Variables|Default|GetStaticMesh) "KeepWorld" "KeepWorld" "KeepWorld" true)
  (bind _notifyname (Animation|Montage|PlayMontage (Variables|Character|GetMesh) (Utilities|Select :Index (Variables|Default|GetExecutionSequence) :Option%200 "/Game/Great_Sword/Animations/Sequence2/02_Attack/15_Execution/02_Target/AS_Execution_Target_03_Seq_Montage.AS_Execution_Target_03_Seq_Montage" :Option%201 "/Game/Zak/TrainingDummy/Anims/Execution_Target_02_RM_Seq_Montage.Execution_Target_02_RM_Seq_Montage" :Option%202 "/Game/Dual_Sword/Animations/Sequence2/02_Attack/16_Exeution/02_Target/AS_Exeution_Target_02_Seq_Montage.AS_Exeution_Target_02_Seq_Montage") 0.7)
    (:OnNotifyBegin
      (switch name _notifyname
        (:Fracture
          (Utilities|FlowControl|Sequence
            (:then_0
              (Components|DestroyComponent (Variables|Character|GetMesh))
              (bind _as_bp_weapon (Variables|Default|GetAs%20BP%20Weapon)
                (:then
                  (Components|DestroyComponent (Variables|/Script/Engine.Actor|GetRootComponent _as_bp_weapon)))
                (:else
                  _))
              (Game|SpawnActorfromClass "/Game/Zak/Fracture/BP_FractureDummy.BP_FractureDummy_C" (Transformation|GetActorTransform) "Undefined" "OverrideRootScale" 0 0)
              (Game|SpawnActorfromClass "/Game/Zak/WorldInterractible/FS_Impact.FS_Impact_C" (Transformation|GetActorTransform) "AlwaysSpawn" "MultiplyWithRoot" 0 0)
              (CallFunction|Death)
              (Actor|DestroyActor))
            (:then_1
              (bind _as_bp_weapon_2 (Variables|Default|GetAs%20BP%20Weapon)
                (:then
                  (Transformation|DetachFromActor _as_bp_weapon_2 "KeepWorld" "KeepWorld" "KeepWorld")
                  (Collision|SetCollisionEnabled (Variables|/Game/Zak/Weapons/BP_Weapon.BP_Weapon_C|GetWeapon _as_bp_weapon_2) "QueryAndPhysics")
                  (Physics|SetSimulatePhysics (Variables|/Game/Zak/Weapons/BP_Weapon.BP_Weapon_C|GetWeapon _as_bp_weapon_2) true))
                (:else)))))))))

(event EventLoadData
  (params (SaveGameRef :type BP%20Save%20Game%20Object%20Reference))
  (bind _tutorialsave (Variables|/Game/Zak/SaveGame/BP_SaveGame.BP_SaveGame_C|GetTutorialSave SaveGameRef))
  (Variables|Default|SetTutorialComplete? (.controlsexplained? _tutorialsave))
  (Variables|Default|SetBlockExplained? (.blockexplained? _tutorialsave))
  (Variables|Default|SetHealExplained? (.healexplained? _tutorialsave))
  (Variables|Default|SetExecutionExplained? (.executionexplained? _tutorialsave)))

(event EventSaveData
  (params (SaveGameRef :type BP%20Save%20Game%20Object%20Reference))
  (Variables|/Game/Zak/SaveGame/BP_SaveGame.BP_SaveGame_C|SetTutorialSave SaveGameRef (Utilities|Struct|MakeS_TutorialSave (Variables|Default|GetTutorialComplete?) (Variables|Default|GetBlockExplained?) (Variables|Default|GetHealExplained?) (Variables|Default|GetExecutionExplained?))))

(fn ConstructionScript
  (bind _bpc_damagesystem (Variables|Default|GetBPC_DamageSystem))
  (EventDispatchers|BindEventtoOnDeath _bpc_damagesystem (EventDispatchers|CreateEvent :!event Custom|Death))
  (EventDispatchers|BindEventtoOnDamageResponse _bpc_damagesystem (EventDispatchers|CreateEvent :!event Custom|DamageResponse))
  (EventDispatchers|BindEventtoOnAllTasksComplete (Variables|Default|GetControls) (EventDispatchers|CreateEvent :!event Custom|AllTasksComplete)))

(fn CalculateDamageDirection
  (params (DamagingActor :type Actor%20Object%20Reference) (DamagedActor :type Actor%20Object%20Reference))
  (bind _returnvalue (Transformation|GetActorRotation DamagedActor))
  (bind _returnvalue_2 (Transformation|GetActorLocation DamagingActor))
  (bind _returnvalue_3 (Transformation|GetActorLocation DamagedActor))
  (bind _returnvalue_4 (Math|Rotator|FindLookatRotation _returnvalue_2 _returnvalue_3))
  (bind _returnvalue_5 (Math|Rotator|Delta(Rotator) _returnvalue _returnvalue_4))
  (Utilities|IsValid DamagedActor
    (:Is%20Valid
      (if (or (Math|Float|InRange(Float) (.yaw _returnvalue_5) -1.8e+02 -135.0) (Math|Float|InRange(Float) (.yaw _returnvalue_5) 135.0 1.8e+02))
        (return "NewEnumerator0")
        (elif (Math|Float|InRange(Float) (.yaw _returnvalue_5) 45.0 135.0)
          (return "NewEnumerator2")
          (elif (Math|Float|InRange(Float) (.yaw _returnvalue_5) -135.0 -45.0)
            (return "NewEnumerator1")
            (elif (Math|Float|InRange(Float) (.yaw _returnvalue_5) -45.0 45.0)
              (return "NewEnumerator3"))))))))

(fn CalculateAccumulatedDamage)

(fn SetHitReactionMontage
  (params (DamageDirection :type E_DamageDirection%20Enum :default "NewEnumerator0"))
  (if (Utilities|Enum|Equal(Enum) DamageDirection "NewEnumerator0")
    (return "/Game/Zak/TrainingDummy/Anims/Hit_Large_Combat_F_Seq_Montage.Hit_Large_Combat_F_Seq_Montage")
    (elif (Utilities|Enum|Equal(Enum) DamageDirection "NewEnumerator2")
      (return "/Game/Zak/TrainingDummy/Anims/Hit_Combat_L_Seq_Montage.Hit_Combat_L_Seq_Montage")
      (elif (Utilities|Enum|Equal(Enum) DamageDirection "NewEnumerator1")
        (return "/Game/Zak/TrainingDummy/Anims/Hit_Combat_R_Seq_Montage.Hit_Combat_R_Seq_Montage")
        (elif (Utilities|Enum|Equal(Enum) DamageDirection "NewEnumerator3")
          (return "/Game/Zak/TrainingDummy/Anims/Hit_Combat_B_Seq_Montage.Hit_Combat_B_Seq_Montage"))))))

(fn WithinExecutionThreshold
  (bind _maxhealth (CallFunction|GetMaxHealth))
  (bind _health (CallFunction|GetCurrentHealth))
  (bind _isdead_ (CallFunction|IsDead))
  (if (Math|Boolean|ANDBoolean (not _isdead_) (<= (/ _health _maxhealth) (Variables|Default|GetExecutionThreshold)) (not (Variables|Default|GetExecuted?)))
    (if (Variables|Type|GetAttacker?)
      (if (not (Variables|Default|GetExecutionExplained?))
        (Class|VerticalBox|AddChildtoVerticalBox (Variables|/Game/Zak/UI/W_PlayerHUD.W_PlayerHUD_C|GetHints (Variables|/Game/Zak/UI/BPC_PlayerHUD.BPC_PlayerHUD_C|GetPlayerHUD (Variables|Default|GetAs%20BPC%20Player%20HUD))) (Variables|Default|GetHintExecute))
        (Variables|Default|SetExecutionExplained? true)
        (Default|RequestSave (Variables|Default|GetAs%20BP%20Game%20Instance%202) true)
        (Audio|PlaySound2D "/Engine/VREditor/Sounds/UI/Camera_Shutter.Camera_Shutter" 1.0 1.0 0.0 0 0)
        (Game|SetGamePaused true)
        (return true)
        (else
          (return true))))
    (else
      (return false))))

(fn ExecuteAnim)

(fn CanbeExecuted
  (bind _canbeexecuted_ (CallFunction|WithinExecutionThreshold))
  (if (and _canbeexecuted_ (<= (Math|Vector|Distance(Vector) (Transformation|GetActorLocation (Variables|Default|GetAs%20BP%20Player)) (Transformation|GetActorLocation)) 2e+02))
    (Variables|Default|SetCanBeExecuted? true)
    (Development|SetHiddeninGame (Variables|Default|GetExecuteWidget) false false)
    (return true)
    (else
      (Variables|Default|SetCanBeExecuted? false)
      (Development|SetHiddeninGame (Variables|Default|GetExecuteWidget) true false)
      (return false))))

(fn GetCurrentHealth
  (bind _bpc_damagesystem (Variables|Default|GetBPC_DamageSystem))
  (Utilities|IsValid _bpc_damagesystem
    (:Is%20Valid
      (return (Variables|/Game/Zak/DamageSystem/BPC_DamageSystem.BPC_DamageSystem_C|GetHealth _bpc_damagesystem)))))

(fn GetMaxHealth
  (bind _bpc_damagesystem (Variables|Default|GetBPC_DamageSystem))
  (Utilities|IsValid _bpc_damagesystem
    (:Is%20Valid
      (return (Variables|/Game/Zak/DamageSystem/BPC_DamageSystem.BPC_DamageSystem_C|GetMaxHealth _bpc_damagesystem)))))

(fn Heal
  (params (Amount :type Float%20%28double-precision%29))
  (return 0.0))

(fn IsAttacking
  (return false))

(fn IsDead
  (return false))

(fn IsInvincible
  (return false))

(fn TakeDamage
  (params (DamageInfo :type S%20Damage%20Info%20Structure))
  (bind (_wasdamaged_ _damageamount _wasparried_ _healthremaining) (Default|TakeDamage (Variables|Default|GetBPC_DamageSystem) DamageInfo))
  (if _wasparried_
    (return false 0.0 true 0.0)
    (elif _wasdamaged_
      (Variables|Default|SetDamageTaken _damageamount)
      (CallFunction|CalculateAccumulatedDamage)
      (Camera|PlayWorldCameraShake "/Game/Zak/VFX/BP_HitCameraShake.BP_HitCameraShake_C" (Transformation|GetActorLocation (Game|GetPlayerCharacter 0)) 0.0 5e+02)
      (Audio|PlaySound2D "/Game/Zak/Audio/sword_hit.sword_hit" 2.0 1.0 0.1 0 0)
      (return true _damageamount false _healthremaining))))