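; Boss arena trigger that seals a barrier, shows its Niagara effect and broadcasts fight start when the player enters.
; It adds an audio component with Timeline-driven volume on entry, and binds to death events of all EnemyFour and AbyssalWarden actors at BeginPlay.
; Restart reopens the barrier and removes effect and audio, while BossDefeated only destroys the audio.
; The construction script sizes the effect from root scale.
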(event OnComponentBeginOverlap(Box)
  (params (OverlappedComponent :type Primitive%20Component%20Object%20Reference) (OtherActor :type Actor%20Object%20Reference) (OtherComp :type Primitive%20Component%20Object%20Reference) (OtherBodyIndex :type Integer) (bFromSweep :type Boolean) (SweepResult :type Hit%20Result%20Structure%20%28by%20ref%29))
  (Utilities|Casting|CastToBP_Player OtherActor)
  (Collision|SetCollisionResponsetoAllChannels (Variables|Default|GetBox1) "ECR_Block")
  (Development|SetHiddeninGame (Variables|Default|GetNiagara) false false)
  (Default|CallOnBossFightStarted)
  (bind _returnvalue (AddComponent|AddAudioComponent false))
  (bind _output_get (Variables|Default|SetAudio _returnvalue))
  (bind _newtrack_0 (Timeline|Timeline PlayFromStart)
    (:Update
      (Audio|Components|Audio|SetVolumeMultiplier _output_get _newtrack_0 :!class /Script/Engine.AudioComponent))))

(event Custom|BossDefeated
  (Components|DestroyComponent (Variables|Default|GetAudio)))

(event EventBeginPlay
  (Utilities|FlowControl|Sequence
    (:then_0
      (bind _outactors (Actor|GetAllActorsOfClass "/Game/Mason/AI_SystemTwo/Enemy4/BP_EnemyFour.BP_EnemyFour_C"))
      (for _array_element _outactors
        (EventDispatchers|BindEventtoOnBossDeath _array_element (EventDispatchers|CreateEvent :!event Custom|BossDefeated))))
    (:then_1
      (bind _outactors_2 (Actor|GetAllActorsOfClass "/Game/Zak/AbyssalWarden/BP_AbyssalWarden.BP_AbyssalWarden_C"))
      (for _array_element_2 _outactors_2
        (EventDispatchers|BindEventtoOnBossDeath _array_element_2 (EventDispatchers|CreateEvent :!event Custom|BossDefeated))))))

(event EventRestart
  (Collision|SetCollisionResponsetoAllChannels (Variables|Default|GetBox1) "ECR_Overlap")
  (Development|SetHiddeninGame (Variables|Default|GetNiagara) true false)
  (bind _audio (Variables|Default|GetAudio)
    (:then
      (Components|DestroyComponent _audio))
    (:else)))

(fn ConstructionScript
  (bind _defaultsceneroot (Variables|Default|GetDefaultSceneRoot))
  (bind _returnvalue (Transformation|GetWorldScale _defaultsceneroot))
  (Class|NiagaraComponent|SetVariableVec2 (Variables|Default|GetNiagara) "Scale" (Math|Vector2D|MakeVector2D (* (.x _returnvalue) 6e+02) (* (.z _returnvalue) 9e+02))))