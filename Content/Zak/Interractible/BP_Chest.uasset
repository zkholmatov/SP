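; BP_Chest is an interactable chest that opens once, spawns a BP_Item and persists its opened state.
; A sphere overlap toggles the interact widget for the player while the chest is closed.
; Interact runs a timeline that rotates the lid, then spawns the item at an arrow's transform.
; It requests loading on BeginPlay and uses its display name in the save data to restore the open lid without respawning the item.
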(event OnComponentBeginOverlap(Sphere)
  (params (OverlappedComponent :type Primitive%20Component%20Object%20Reference) (OtherActor :type Actor%20Object%20Reference) (OtherComp :type Primitive%20Component%20Object%20Reference) (OtherBodyIndex :type Integer) (bFromSweep :type Boolean) (SweepResult :type Hit%20Result%20Structure%20%28by%20ref%29))
  (Utilities|Casting|CastToBP_Player OtherActor)
  (if (not (Variables|Default|GetOpen?))
    (Rendering|SetVisibility (Variables|Default|GetInteractWidget) true false)))

(event OnComponentEndOverlap(Sphere)
  (params (OverlappedComponent :type Primitive%20Component%20Object%20Reference) (OtherActor :type Actor%20Object%20Reference) (OtherComp :type Primitive%20Component%20Object%20Reference) (OtherBodyIndex :type Integer))
  (Utilities|Casting|CastToBP_Player OtherActor)
  (if (not (Variables|Default|GetOpen?))
    (Rendering|SetVisibility (Variables|Default|GetInteractWidget) false false)))

(event EventLoadData
  (params (SaveGameRef :type BP%20Save%20Game%20Object%20Reference))
  (for _array_element (.chestname (Variables|/Game/Zak/SaveGame/BP_SaveGame.BP_SaveGame_C|GetChestSave SaveGameRef))
    (if (Utilities|Enum|Equal(Enum) _array_element (Utilities|GetDisplayName self))
      (Variables|Default|SetOpen? true)
      (Transformation|SetRelativeRotation (Variables|Default|GetTop) (Math|Rotator|MakeRotator 0.0 -7e+01 -89.999999) false false))))

(event EventSaveData
  (params (SaveGameRef :type BP%20Save%20Game%20Object%20Reference))
  (if (Variables|Default|GetInteracted?)
    (Utilities|Array|AddUnique (.chestname (Variables|/Game/Zak/SaveGame/BP_SaveGame.BP_SaveGame_C|GetChestSave SaveGameRef)) (Utilities|GetDisplayName self))))

(event EventBeginPlay
  (Class|BPIPersistence|RequestLoad(Message) (Game|GetGameInstance) self))

(event EventInteract
  (bind _arrow (Variables|Default|GetArrow))
  (if (not (Variables|Default|GetOpen?))
    (Variables|Default|SetInteracted? true)
    (Variables|Default|SetOpen? true)
    (bind _newtrack_0 (Timeline|Timeline PlayFromStart)
      (:Update
        (Transformation|SetRelativeRotation (Variables|Default|GetTop) (Math|Rotator|MakeRotator 0.0 _newtrack_0 -89.999999) false false))
      (:Finished
        (Game|SpawnActorfromClass "/Game/Omar/Inventory/Blueprints/BP_Item.BP_Item_C" (Math|Transform|MakeTransform (Transformation|GetWorldLocation _arrow) (Transformation|GetWorldRotation _arrow) "1.000000,1.000000,1.000000") "AdjustIfPossibleButAlwaysSpawn" "MultiplyWithRoot" 0 (Variables|Default|GetItem) "(R=1.000000,G=1.000000,B=1.000000,A=1.000000)" 0)
        (Rendering|SetVisibility (Variables|Default|GetInteractWidget) false false)))))

(fn ConstructionScript)