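; BP_Enemy is a stationary-logic enemy with very high health that automatically attacks whatever Pawn is ahead of it.
; A looping timer runs a debug-drawn forward sphere trace while alive, sending damage through an interface message.
; Damage and health queries forward to BPCDamageSystem, while Heal and state queries, including IsDead, are stubs.
; It spawns a BP_TargetLock actor above itself and toggles its widget each Tick from IsLocked.
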(event Custom|Attack
  (bind _returnvalue (Transformation|GetActorLocation))
  (if (not (Variables|/Game/Zak/DamageSystem/BPC_DamageSystem.BPC_DamageSystem_C|GetDead? (Variables|Default|GetBPC_DamageSystem)))
    (bind (_outhit _returnvalue_2) (Collision|SphereTraceForObjects _returnvalue (+ _returnvalue (* (Transformation|GetActorForwardVector) 2e+02)) 2e+01 (Utilities|Array|MakeArray "ObjectTypeQuery3") false 0 "ForDuration" true "(R=1.000000,G=0.000000,B=0.000000,A=1.000000)" "(R=0.000000,G=1.000000,B=0.000000,A=1.000000)" 0.1))
    (if _returnvalue_2
      (Class|BPIDamageable|TakeDamage(Message) (.HitActor (Collision|BreakHitResult _outhit)) (Utilities|Struct|MakeS_DamageInfo (Variables|Default|GetAttackDamage) "NewEnumerator1" "NewEnumerator0" false true true)))))

(event EventBeginPlay
  (Utilities|Time|SetTimerbyEvent (delegate Custom|Attack) 0.5 true)
  (Default|SetMaxHealth (Variables|Default|GetBPC_DamageSystem) 2.9999e+06)
  (bind _returnvalue (Game|SpawnActorfromClass "/Game/Zak/UI/BP_TargetLock.BP_TargetLock_C" (Math|Conversions|ToTransform(Vector) (+ (Transformation|GetActorLocation) "0.000000,0.000000,30.000000")) "Undefined" "MultiplyWithRoot" 0 0))
  (Variables|Default|SetTargetLockWidget _returnvalue))

(event EventTick
  (params (DeltaSeconds :type Float%20%28single-precision%29))
  (bind _targetlockwidget (Variables|Default|GetTargetLockWidget))
  (bind _targetlockwidget_2 (Variables|/Game/Zak/UI/BP_TargetLock.BP_TargetLock_C|GetTargetLockWidget _targetlockwidget))
  (if (Variables|Default|GetIsLocked?)
    (Rendering|SetVisibility _targetlockwidget_2 true false)
    (else
      (Rendering|SetVisibility _targetlockwidget_2 false false))))

(fn ConstructionScript)

(fn GetCurrentHealth
  (bind _bpc_damagesystem (Variables|Default|GetBPC_DamageSystem))
  (Utilities|IsValid _bpc_damagesystem
    (:Is%20Valid
      (return (Variables|/Game/Zak/DamageSystem/BPC_DamageSystem.BPC_DamageSystem_C|GetHealth _bpc_damagesystem)))))

(fn GetMaxHealth
  (bind _bpc_damagesystem (Variables|Default|GetBPC_DamageSystem))
  (Utilities|IsValid _bpc_damagesystem
    (:Is%20Valid
      (return (Variables|/Game/Zak/DamageSystem/BPC_DamageSystem.BPC_DamageSystem_C|GetMaxHealth _bpc_damagesystem)))))

(fn Heal
  (params (Amount :type Float%20%28double-precision%29))
  (return 0.0))

(fn IsAttacking
  (return false))

(fn IsDead
  (return false))

(fn IsInvincible
  (return false))

(fn TakeDamage
  (params (DamageInfo :type S%20Damage%20Info%20Structure))
  (bind (_wasdamaged_ _damageamount) (Default|TakeDamage (Variables|Default|GetBPC_DamageSystem) DamageInfo))
  (return _wasdamaged_ _damageamount))