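; Checkpoint actor that updates the player's respawn point and saves the game on interaction.
; Entering its sphere sets the player's SpawnTransform, shows an interact widget and fires OnPlayerOverlap; leaving hides the widget.
; Interacting marks it checked, requests a save through BP_GameInstance and switches on a Niagara butterfly glow.
; Checked checkpoints are saved by display name, and loading matches that name to restore the glow, without setting Checked.
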(event OnComponentBeginOverlap(Sphere)
  (params (OverlappedComponent :type Primitive%20Component%20Object%20Reference) (OtherActor :type Actor%20Object%20Reference) (OtherComp :type Primitive%20Component%20Object%20Reference) (OtherBodyIndex :type Integer) (bFromSweep :type Boolean) (SweepResult :type Hit%20Result%20Structure%20%28by%20ref%29))
  (bind _asbp_player (Utilities|Casting|CastToBP_Player OtherActor))
  (Variables|/Game/Zak/BP_Player.BP_Player_C|SetSpawnTransform _asbp_player (Transformation|GetWorldTransform (Variables|Default|GetSpawnLocation)))
  (Rendering|SetVisibility (Variables|Default|GetInteractWidget) true false)
  (Default|CallOnPlayerOverlap))

(event OnComponentEndOverlap(Sphere)
  (params (OverlappedComponent :type Primitive%20Component%20Object%20Reference) (OtherActor :type Actor%20Object%20Reference) (OtherComp :type Primitive%20Component%20Object%20Reference) (OtherBodyIndex :type Integer))
  (Utilities|Casting|CastToBP_Player OtherActor)
  (Rendering|SetVisibility (Variables|Default|GetInteractWidget) false false))

(event EventInteract
  (Variables|Default|SetChecked? true)
  (bind _asbp_game_instance (Utilities|Casting|CastToBP_GameInstance (Game|GetGameInstance)))
  (Default|RequestSave _asbp_game_instance true)
  (if (Variables|Default|GetChecked?)
    (CallFunction|SpawnParticles)))

(event EventBeginPlay
  (Class|BPIPersistence|RequestLoad(Message) (Game|GetGameInstance) self)
  (bind _asbpc_player_hud (Utilities|Casting|CastToBPC_PlayerHUD (HUD|GetHUD (Game|GetPlayerController 0))))
  (Variables|Default|SetAs%20BPC%20Player%20HUD _asbpc_player_hud)
  (bind _asbp_game_instance (Utilities|Casting|CastToBP_GameInstance (Game|GetGameInstance)))
  (Variables|Default|SetAs%20BP%20Game%20Instance _asbp_game_instance))

(event EventSaveData
  (params (SaveGameRef :type BP%20Save%20Game%20Object%20Reference))
  (if (Variables|Default|GetChecked?)
    (Utilities|Array|AddUnique (.checkpointname (Variables|/Game/Zak/SaveGame/BP_SaveGame.BP_SaveGame_C|GetCheckpointSave SaveGameRef)) (Utilities|GetDisplayName self))))

(event EventLoadData
  (params (SaveGameRef :type BP%20Save%20Game%20Object%20Reference))
  (for _array_element (.checkpointname (Variables|/Game/Zak/SaveGame/BP_SaveGame.BP_SaveGame_C|GetCheckpointSave SaveGameRef))
    (if (Utilities|Enum|Equal(Enum) _array_element (Utilities|GetDisplayName self))
      (CallFunction|SpawnParticles))))

(fn ConstructionScript)

(fn SpawnParticles
  (bind _niagara (Variables|Default|GetNiagara))
  (Class|NiagaraComponent|SetAsset _niagara "/Game/ButterflySwarmFX/FX/NS_Butterfly_Glow_1.NS_Butterfly_Glow_1" true)
  (Niagara|SetNiagaraVariable(Float) _niagara "Emissive" 2e+02)
  (Niagara|SetNiagaraVariable(Float) _niagara "Lifetime" 2.0)
  (Niagara|SetNiagaraVariable(Float) _niagara "Radius" 1e+02)
  (Niagara|SetNiagaraVariable(Float) _niagara "Size" 1.0))