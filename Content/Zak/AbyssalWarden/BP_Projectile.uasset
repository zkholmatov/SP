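; BP_Projectile is a configurable projectile for the AbyssalWarden content that flies at an optional target and reports its first overlap.
; The construction script applies speed and gravity to ProjectileMovement and, for a valid homing target, enables homing and sets Niagara jitter and trail colors.
; On BeginPlay it ignores its owner when moving and aims velocity at the target.
; The first sphere overlap calls OnProjectileHit, then destroys the actor.
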(event OnComponentBeginOverlap(Sphere)
  (params (OverlappedComponent :type Primitive%20Component%20Object%20Reference) (OtherActor :type Actor%20Object%20Reference) (OtherComp :type Primitive%20Component%20Object%20Reference) (OtherBodyIndex :type Integer) (bFromSweep :type Boolean) (SweepResult :type Hit%20Result%20Structure%20%28by%20ref%29))
  (Utilities|FlowControl|DoOnce false
    (:Completed
      (Default|CallOnProjectileHit OtherActor SweepResult)
      (Actor|DestroyActor))))

(event Custom|RotateToTarget
  (Variables|/Script/Engine.MovementComponent|SetVelocity (Variables|Default|GetProjectileMovement) (* (Math|Vector|GetUnitDirection(Vector) (Transformation|GetActorLocation) (Transformation|GetActorLocation (Variables|Default|GetTarget))) (Variables|Default|GetSpeed))))

(event EventBeginPlay
  (Collision|IgnoreActorwhenMoving (Variables|Default|GetSphere) (Components|GetOwner) true)
  (Variables|Default|GetTarget
    (:then
      (CallFunction|RotatetoTarget))
    (:else)))

(fn ConstructionScript
  (bind _projectilemovement (Variables|Default|GetProjectileMovement))
  (bind _speed (Variables|Default|GetSpeed))
  (Variables|/Script/Engine.ProjectileMovementComponent|SetInitialSpeed _projectilemovement _speed)
  (Variables|/Script/Engine.ProjectileMovementComponent|SetMaxSpeed _projectilemovement _speed)
  (Variables|/Script/Engine.ProjectileMovementComponent|SetProjectileGravityScale _projectilemovement (Variables|Default|GetGravity))
  (Variables|Default|GetTarget
    (:then
      (if (Variables|Default|GetIsHoming?)
        (Variables|/Script/Engine.ProjectileMovementComponent|SetbIsHomingProjectile _projectilemovement true)
        (Variables|/Script/Engine.ProjectileMovementComponent|SetHomingTargetComponent _projectilemovement (Variables|/Script/Engine.Actor|GetRootComponent (Variables|Default|GetTarget)))
        (Niagara|SetNiagaraVariable(LinearColor) (Variables|Default|GetNiagara) "JitterColor" (Variables|Default|GetJitterColor))
        (Niagara|SetNiagaraVariable(LinearColor) (Variables|Default|GetNiagara) "TrailColor" (Variables|Default|GetTrailColor))))
    (:else)))