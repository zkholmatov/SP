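; BPC_PlayerSettings is a component that holds the player's controller sensitivity and sprint toggle settings and persists them through save data.
; On BeginPlay it registers a load request with BP_GameInstance, passing itself.
; SaveData and LoadData events copy both values to and from the SettingsSave struct on the supplied save game object.
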(event EventBeginPlay
  (bind _asbp_game_instance (Utilities|Casting|CastToBP_GameInstance (Game|GetGameInstance)))
  (Default|RequestLoad _asbp_game_instance self))

(event EventSaveData
  (params (SaveGameRef :type BP%20Save%20Game%20Object%20Reference))
  (Variables|/Game/Zak/SaveGame/BP_SaveGame.BP_SaveGame_C|SetSettingsSave SaveGameRef (Utilities|Struct|MakeS_SettingsSave (Variables|Default|GetControllerSensitivity) (Variables|Default|GetSprintToggle?))))

(event EventLoadData
  (params (SaveGameRef :type BP%20Save%20Game%20Object%20Reference))
  (bind _settingssave (Variables|/Game/Zak/SaveGame/BP_SaveGame.BP_SaveGame_C|GetSettingsSave SaveGameRef))
  (Variables|Default|SetControllerSensitivity (.controllersensitivity _settingssave))
  (Variables|Default|SetSprintToggle? (.sprinttoggle? _settingssave)))