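; Tutorial component that shows one-time, game-pausing hints for souls, checkpoints, blocking, healing, executions, items and inventory.
; On BeginPlay it hides the HUD souls counter until explained and binds to enemy, checkpoint, player and inventory events.
; Each Explain event sets a flag, adds a HUD hint and requests a save, with items chaining into inventory.
; SaveData and LoadData persist the flags, except those for items and inventory.
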(event Custom|ExplainCheckpoint
  (if (not (Variables|Default|GetCheckpointExplained?))
    (Variables|Default|SetCheckpointExplained? true)
    (Class|VerticalBox|AddChildtoVerticalBox (Variables|/Game/Zak/UI/Wigets/W_PlayerHUD.W_PlayerHUD_C|GetHints (Variables|/Game/Zak/UI/BPC_PlayerHUD.BPC_PlayerHUD_C|GetPlayerHUD (Variables|Default|GetAs%20BPC%20Player%20HUD))) (Variables|Default|GetContent))
    (Game|SetGamePaused true)
    (Default|RequestSave (Variables|Default|GetAs%20BP%20Game%20Instance) true)))

(event Custom|ExplainSouls
  (if (not (Variables|Default|GetSoulsExplained?))
    (Variables|Default|SetSoulsExplained? true)
    (Utilities|FlowControl|Delay 2.0)
    (Class|VerticalBox|AddChildtoVerticalBox (Variables|/Game/Zak/UI/Wigets/W_PlayerHUD.W_PlayerHUD_C|GetHints (Variables|/Game/Zak/UI/BPC_PlayerHUD.BPC_PlayerHUD_C|GetPlayerHUD (Variables|Default|GetAs%20BPC%20Player%20HUD))) (Variables|Default|GetSoulsHint))
    (Widget|SetVisibility (Variables|/Game/Zak/UI/Wigets/W_PlayerHUD.W_PlayerHUD_C|GetSoulsPurgedBox (Variables|/Game/Zak/UI/BPC_PlayerHUD.BPC_PlayerHUD_C|GetPlayerHUD (Variables|Default|GetAs%20BPC%20Player%20HUD))) "Visible")
    (Default|RequestSave (Variables|Default|GetAs%20BP%20Game%20Instance) true)
    (Game|SetGamePaused true)))

(event Custom|ExplainBlock
  (Utilities|FlowControl|Delay 0.5)
  (if (not (Variables|Default|GetBlockExplained?))
    (Class|VerticalBox|AddChildtoVerticalBox (Variables|/Game/Zak/UI/Wigets/W_PlayerHUD.W_PlayerHUD_C|GetHints (Variables|/Game/Zak/UI/BPC_PlayerHUD.BPC_PlayerHUD_C|GetPlayerHUD (Variables|Default|GetAs%20BPC%20Player%20HUD))) (Variables|Default|GetHintBlock))
    (Variables|Default|SetBlockExplained? true)
    (Game|SetGamePaused true)
    (Default|RequestSave (Variables|Default|GetAs%20BP%20Game%20Instance) true)))

(event Custom|ExplainHeal
  (if (not (Variables|Default|GetHealExplained?))
    (Class|VerticalBox|AddChildtoVerticalBox (Variables|/Game/Zak/UI/Wigets/W_PlayerHUD.W_PlayerHUD_C|GetHints (Variables|/Game/Zak/UI/BPC_PlayerHUD.BPC_PlayerHUD_C|GetPlayerHUD (Variables|Default|GetAs%20BPC%20Player%20HUD))) (Variables|Default|GetHintHeal))
    (Variables|Default|SetHealExplained? true)
    (Default|RequestSave (Variables|Default|GetAs%20BP%20Game%20Instance) true)
    (Game|SetGamePaused true)))

(event Custom|ExplainExecution
  (if (not (Variables|Default|GetExecutionExplained?))
    (Class|VerticalBox|AddChildtoVerticalBox (Variables|/Game/Zak/UI/Wigets/W_PlayerHUD.W_PlayerHUD_C|GetHints (Variables|/Game/Zak/UI/BPC_PlayerHUD.BPC_PlayerHUD_C|GetPlayerHUD (Variables|Default|GetAs%20BPC%20Player%20HUD))) (Variables|Default|GetHintExecute))
    (Variables|Default|SetExecutionExplained? true)
    (Default|RequestSave (Variables|Default|GetAs%20BP%20Game%20Instance) true)
    (Game|SetGamePaused true)))

(event Custom|ExplainInventory
  (if (not (Variables|Default|GetInventoryExplained?))
    (Class|VerticalBox|AddChildtoVerticalBox (Variables|/Game/Zak/UI/Wigets/W_PlayerHUD.W_PlayerHUD_C|GetHints (Variables|/Game/Zak/UI/BPC_PlayerHUD.BPC_PlayerHUD_C|GetPlayerHUD (Variables|Default|GetAs%20BPC%20Player%20HUD))) (Variables|Default|GetHintInventory))
    (Variables|Default|SetInventoryExplained? true)
    (Default|RequestSave (Variables|Default|GetAs%20BP%20Game%20Instance) true)
    (Game|SetGamePaused true)))

(event Custom|ExplainItems
  (if (not (Variables|Default|GetItemsExplained?))
    (Class|VerticalBox|AddChildtoVerticalBox (Variables|/Game/Zak/UI/Wigets/W_PlayerHUD.W_PlayerHUD_C|GetHints (Variables|/Game/Zak/UI/BPC_PlayerHUD.BPC_PlayerHUD_C|GetPlayerHUD (Variables|Default|GetAs%20BPC%20Player%20HUD))) (Variables|Default|GetHintItems))
    (Variables|Default|SetItemsExplained? true)
    (Default|RequestSave (Variables|Default|GetAs%20BP%20Game%20Instance) true)
    (Game|SetGamePaused true)
    (Utilities|FlowControl|Delay 5.0)
    (CallFunction|ExplainInventory)))

(event EventBeginPlay
  (bind _asbp_game_instance (Utilities|Casting|CastToBP_GameInstance (Game|GetGameInstance)))
  (Variables|Default|SetAs%20BP%20Game%20Instance _asbp_game_instance)
  (Class|BPIPersistence|RequestLoad(Message) (Game|GetGameInstance) self)
  (bind _asbpc_player_hud (Utilities|Casting|CastToBPC_PlayerHUD (HUD|GetHUD (Game|GetPlayerController 0))))
  (Variables|Default|SetAs%20BPC%20Player%20HUD _asbpc_player_hud)
  (Utilities|FlowControl|Delay 0.1)
  (if (not (Variables|Default|GetSoulsExplained?))
    (Widget|SetVisibility (Variables|/Game/Zak/UI/Wigets/W_PlayerHUD.W_PlayerHUD_C|GetSoulsPurgedBox (Variables|/Game/Zak/UI/BPC_PlayerHUD.BPC_PlayerHUD_C|GetPlayerHUD (Variables|Default|GetAs%20BPC%20Player%20HUD))) "Hidden")
    (else
      (Widget|SetVisibility (Variables|/Game/Zak/UI/Wigets/W_PlayerHUD.W_PlayerHUD_C|GetSoulsPurgedBox (Variables|/Game/Zak/UI/BPC_PlayerHUD.BPC_PlayerHUD_C|GetPlayerHUD (Variables|Default|GetAs%20BPC%20Player%20HUD))) "Visible")))
  (Utilities|FlowControl|Sequence
    (:then_0
      (bind _outactors (Actor|GetAllActorsOfClass "/Game/Mason/AI_SystemTwo/BP_EnemyOne.BP_EnemyOne_C"))
      (for _array_element _outactors
        (EventDispatchers|BindEventtoOnEnemyDeath _array_element (EventDispatchers|CreateEvent :!event Custom|ExplainSouls))))
    (:then_1
      (bind _outactors_2 (Actor|GetAllActorsOfClass "/Game/Zak/SaveGame/BP_Checkpoint.BP_Checkpoint_C"))
      (for _array_element_2 _outactors_2
        (EventDispatchers|BindEventtoOnPlayerOverlap _array_element_2 (EventDispatchers|CreateEvent :!event Custom|ExplainCheckpoint))))
    (:then_2
      (bind _returnvalue (Actor|GetActorOfClass "/Game/Zak/BP_Player.BP_Player_C"))
      (EventDispatchers|BindEventtoOnDamageTaken _returnvalue (EventDispatchers|CreateEvent :!event Custom|ExplainHeal))
      (EventDispatchers|BindEventtoOnExplainExecution _returnvalue (EventDispatchers|CreateEvent :!event Custom|ExplainExecution))
      (EventDispatchers|BindEventtoOnBlock _returnvalue (EventDispatchers|CreateEvent :!event Custom|ExplainBlock)))
    (:then_3
      (bind _asbp_player (Utilities|Casting|CastToBP_Player (Game|GetPlayerCharacter 0)))
      (EventDispatchers|BindEventtoOnItemFound (Variables|/Game/Zak/BP_Player.BP_Player_C|GetBPC_Inventory _asbp_player) (EventDispatchers|CreateEvent :!event Custom|ExplainItems)))))

(event EventSaveData
  (params (SaveGameRef :type BP%20Save%20Game%20Object%20Reference))
  ;[1 1 1] Save System
  (Variables|/Game/Zak/SaveGame/BP_SaveGame.BP_SaveGame_C|SetTutorialSave SaveGameRef (Utilities|Struct|MakeS_TutorialSave (Variables|Default|GetBlockExplained?) (Variables|Default|GetHealExplained?) (Variables|Default|GetExecutionExplained?) (Variables|Default|GetCheckpointExplained?) (Variables|Default|GetSoulsExplained?))))

(event EventLoadData
  (params (SaveGameRef :type BP%20Save%20Game%20Object%20Reference))
  (bind _tutorialsave (Variables|/Game/Zak/SaveGame/BP_SaveGame.BP_SaveGame_C|GetTutorialSave SaveGameRef))
  ;[1 1 1] Save System
  (Variables|Default|SetBlockExplained? (.blockexplained? _tutorialsave))
  (Variables|Default|SetHealExplained? (.healexplained? _tutorialsave))
  (Variables|Default|SetExecutionExplained? (.executionexplained? _tutorialsave))
  (Variables|Default|SetCheckpointExplained? (.checkpointexplained? _tutorialsave))
  (Variables|Default|SetSoulsExplained? (.soulsexplained? _tutorialsave)))