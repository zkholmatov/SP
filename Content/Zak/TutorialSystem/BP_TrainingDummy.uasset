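; Tutorial training dummy that shows a controls checklist on the HUD, then draws its sword and attacks the player once all tasks are complete, saving that progress.
; Montage notifies drive block hints and timer-based sphere traces that deal parryable, directional damage.
; BPC_DamageSystem feeds directional hit stuns and delayed health refills, and death just resets health.
; At low health it offers an execution, whose montage swaps it for a fractured dummy.
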(event OnComponentBeginOverlap(CombatRadius)
  (params (OverlappedComponent :type Primitive%20Component%20Object%20Reference) (OtherActor :type Actor%20Object%20Reference) (OtherComp :type Primitive%20Component%20Object%20Reference) (OtherBodyIndex :type Integer) (bFromSweep :type Boolean) (SweepResult :type Hit%20Result%20Structure%20%28by%20ref%29))
  ;[1 1 1] Within Radius Overlap
  (Utilities|Casting|CastToBP_Player OtherActor)
  (Rendering|SetVisibility (Variables|Default|GetHealthWidget) true false)
  (if (not (Variables|Default|GetControlsComplete?))
    (Class|VerticalBox|AddChildtoVerticalBox (Variables|/Game/Zak/UI/Wigets/W_PlayerHUD.W_PlayerHUD_C|GetControls (Variables|/Game/Zak/UI/BPC_PlayerHUD.BPC_PlayerHUD_C|GetPlayerHUD (Variables|Default|GetAs%20BPC%20Player%20HUD))) (Variables|Default|GetControls))))

(event OnComponentEndOverlap(CombatRadius)
  (params (OverlappedComponent :type Primitive%20Component%20Object%20Reference) (OtherActor :type Actor%20Object%20Reference) (OtherComp :type Primitive%20Component%20Object%20Reference) (OtherBodyIndex :type Integer))
  ;[1 1 1] Within Radius Overlap
  (Utilities|Casting|CastToBP_Player OtherActor)
  (Rendering|SetVisibility (Variables|Default|GetHealthWidget) false false)
  (bind _controls (Variables|Default|GetControls)
    (:then
      (Class|PanelWidget|RemoveChild (Variables|/Game/Zak/UI/Wigets/W_PlayerHUD.W_PlayerHUD_C|GetControls (Variables|/Game/Zak/UI/BPC_PlayerHUD.BPC_PlayerHUD_C|GetPlayerHUD (Variables|Default|GetAs%20BPC%20Player%20HUD))) _controls))
    (:else)))

(event OnComponentBeginOverlap(AttackRadius)
  (params (OverlappedComponent :type Primitive%20Component%20Object%20Reference) (OtherActor :type Actor%20Object%20Reference) (OtherComp :type Primitive%20Component%20Object%20Reference) (OtherBodyIndex :type Integer) (bFromSweep :type Boolean) (SweepResult :type Hit%20Result%20Structure%20%28by%20ref%29))
  ;[1 1 1] Within Radius Overlap
  (Utilities|Casting|CastToBP_Player OtherActor)
  (Variables|Default|SetWithinRange? true))

(event OnComponentEndOverlap(AttackRadius)
  (params (OverlappedComponent :type Primitive%20Component%20Object%20Reference) (OtherActor :type Actor%20Object%20Reference) (OtherComp :type Primitive%20Component%20Object%20Reference) (OtherBodyIndex :type Integer))
  ;[1 1 1] Within Radius Overlap
  (Utilities|Casting|CastToBP_Player OtherActor)
  (Variables|Default|SetWithinRange? false))

(event Custom|StopAttack
  ;[1 1 1] Attack
  (Utilities|Time|ClearandInvalidateTimerbyHandle (stale Custom|Attack _returnvalue)))

(event Custom|StopSwordTrace
  ;[1 0.3137 0.3137 1 30] Trace
  (Utilities|Time|ClearandInvalidateTimerbyHandle (Variables|Default|GetNewVar)))

(event Custom|DamageResponse
  (params (DamageResponse :type E_DamageResponse%20Enum :default "NewEnumerator0") (DamageDirection :type E_DamageDirection%20Enum :default "NewEnumerator0") (DamageCauser :type Actor%20Object%20Reference))
  ;[1 1 1] Hit Reaction
  (CallFunction|StartRegen)
  (CallFunction|StopSwordTrace)
  (Variables|Default|SetStunned? true)
  (bind _newparam (CallFunction|SetHitReactionMontage DamageDirection))
  (Animation|Montage|PlayMontage (Variables|Character|GetMesh) _newparam
    (:OnCompleted
      (Variables|Default|SetStunned? false))))

(event Custom|Death
  (bind _bpc_damagesystem (Variables|Default|GetBPC_DamageSystem))
  ;[1 1 1] Death
  (Variables|/Game/Zak/DamageSystem/BPC_DamageSystem.BPC_DamageSystem_C|SetDead? _bpc_damagesystem false)
  (Default|SetMaxHealth _bpc_damagesystem (Variables|Default|GetHealth) true))

(event Custom|RegenLoop
  ;[1 1 1] Regen
  (bind _output_get (Variables|Default|SetTemp (+ (Variables|Default|GetTemp) 0.1)))
  (if (>= _output_get 5.0)
    (Default|SetMaxHealth (Variables|Default|GetBPC_DamageSystem) (Variables|Default|GetHealth) true)
    (Variables|Default|SetTemp 0.0)
    (Utilities|Time|ClearandInvalidateTimerbyHandle (stale Custom|StartRegen _returnvalue))))

(event Custom|AllTasksComplete
  (Default|SetMaxHealth (Variables|Default|GetBPC_DamageSystem) (Variables|Default|GetHealth) true)
  (Variables|Default|SetControlsComplete? true)
  (Default|RequestSave (Variables|Default|GetAs%20BP%20Game%20Instance) true)
  (Variables|Default|SetStunned? false)
  (Class|PanelWidget|RemoveChild (Variables|/Game/Zak/UI/Wigets/W_PlayerHUD.W_PlayerHUD_C|GetControls (Variables|/Game/Zak/UI/BPC_PlayerHUD.BPC_PlayerHUD_C|GetPlayerHUD (Variables|Default|GetAs%20BPC%20Player%20HUD))) (Variables|Default|GetControls))
  (bind _notifyname (Animation|Montage|PlayMontage (Variables|Character|GetMesh) "/Game/Zak/TutorialSystem/Anims/Idle_To_Idle_Combat_Seq_Montage.Idle_To_Idle_Combat_Seq_Montage")
    (:OnCompleted
      (Variables|Type|SetAttacker? true :!label _label))
    (:OnInterrupted
      (goto _label))
    (:OnNotifyBegin
      (switch name _notifyname
        (:Attack
          (goto _label))
        (:Wield
          (Transformation|AttachComponentToComponent (Variables|Default|GetAs%20BP%20Weapon) (Variables|Character|GetMesh) "WeaponSocket" "SnapToTarget" "SnapToTarget" "SnapToTarget" true))))))

(event Custom|StartSwordTrace
  ;[1 0.3137 0.3137 1 30] Trace
  (Default|EnableTrail (Variables|Default|GetAs%20BP%20Weapon))
  (bind _returnvalue (Utilities|Time|SetTimerbyEvent (delegate Custom|SwordTraceLoop) 0.01 true))
  (Variables|Default|SetNewVar _returnvalue))

(event Custom|SwordTraceLoop
  (bind _as_bp_weapon (Variables|Default|GetAs%20BP%20Weapon))
  (bind _weapon (Variables|/Game/Zak/Weapons/BP_Weapon.BP_Weapon_C|GetWeapon _as_bp_weapon))
  ;[1 0.3137 0.3137 1 30] Trace
  (bind (_outhit _returnvalue) (Collision|SphereTraceForObjects (Transformation|GetSocketLocation _weapon "TrailStart") (Transformation|GetSocketLocation _weapon "TrailEnd") 1e+01 (Utilities|Array|MakeArray "ObjectTypeQuery3") false 0 "None" true "(R=1.000000,G=0.000000,B=0.000000,A=1.000000)" "(R=0.000000,G=1.000000,B=0.000000,A=1.000000)" 2.0))
  (if _returnvalue
    (CallFunction|StopSwordTrace)
    (bind _wasdamaged_ (Class|BPIDamageable|TakeDamage(Message) (.HitActor (Collision|BreakHitResult _outhit)) (Utilities|Struct|MakeS_DamageInfo 1e+02 "NewEnumerator1" "NewEnumerator3" true false (CallFunction|CalculateDamageDirection (Variables|Default|GetAs%20BP%20Weapon) (.HitActor (Collision|BreakHitResult _outhit))) self)))
    (if _wasdamaged_
      (Niagara|SpawnSystematLocation "/Game/Zak/VFX/Niagara/NS_Hit.NS_Hit" (.ImpactPoint (Collision|BreakHitResult _outhit))))))

(event Custom|LockLoop
  (bind _mesh (Variables|Character|GetMesh))
  ;[1 1 1] Target Lock
  (Utilities|IsValid _mesh
    (:Is%20Valid
      (Transformation|SetWorldLocation (Variables|/Game/Zak/UI/BP_TargetLock.BP_TargetLock_C|GetTargetLockWidget (Variables|Default|GetTargetLockWidget)) (Transformation|GetSocketLocation _mesh "spine_05") false false))))

(event Custom|AttackLoop
  ;[1 1 1] Attack
  (if (Math|Boolean|ANDBoolean (not (Variables|Default|GetAttacking?)) (not (Variables|Default|GetStunned?)) (not (Variables|Default|GetExecuted?)) (Variables|Default|GetWithinRange?) (Variables|Type|GetAttacker?))
    (Variables|Default|SetAttacking? true)
    (bind _notifyname (Animation|Montage|PlayMontage (Variables|Character|GetMesh) "/Game/Zak/TutorialSystem/Anims/Combo_Attack_04_01_Seq_Montage.Combo_Attack_04_01_Seq_Montage")
      (:OnCompleted
        (Variables|Default|SetAttacking? false :!label _label)
        (if (Variables|Default|GetWithinRange?)
          _))
      (:OnInterrupted
        (goto _label))
      (:OnNotifyBegin
        (switch name _notifyname
          (:Hint
            (Default|CallOnExplainBlock))
          (:TraceStart
            (CallFunction|StartSwordTrace))
          (:TraceEnd
            (CallFunction|StopSwordTrace)))))))

(event Custom|StartRegen
  ;[1 1 1] Regen
  (Variables|Default|SetTemp 0.0)
  (bind _returnvalue (Utilities|Time|SetTimerbyEvent (delegate Custom|RegenLoop) 0.1 true)))

(event Custom|Attack
  ;[1 1 1] Attack
  (bind _returnvalue (Utilities|Time|SetTimerbyEvent (delegate Custom|AttackLoop) 0.1 true false -2.0)))

(event EventBeginPlay
  ;[1 1 1] Setup
  (bind _returnvalue (Game|SpawnActorfromClass "/Game/Zak/Weapons/RedSword/BP_RedSword.BP_RedSword_C" (Transformation|GetActorTransform) "Undefined" "MultiplyWithRoot" 0 0))
  (Variables|Default|SetAs%20BP%20Weapon _returnvalue)
  (bind _asbp_game_instance (Utilities|Casting|CastToBP_GameInstance (Game|GetGameInstance)))
  (Variables|Default|SetAs%20BP%20Game%20Instance _asbp_game_instance)
  (Class|BPIPersistence|RequestLoad(Message) (Game|GetGameInstance) self)
  (Variables|/Game/Zak/DamageSystem/BPC_DamageSystem.BPC_DamageSystem_C|SetInvincible? (Variables|Default|GetBPC_DamageSystem) false)
  (bind _asbpc_player_hud (Utilities|Casting|CastToBPC_PlayerHUD (HUD|GetHUD (Game|GetPlayerController 0))))
  (Variables|Default|SetAs%20BPC%20Player%20HUD _asbpc_player_hud)
  (Utilities|FlowControl|Sequence
    (:then_0
      (if (Variables|Default|GetControlsComplete?)
        (Variables|Type|SetAttacker? true)
        (Transformation|AttachComponentToComponent (Variables|Default|GetAs%20BP%20Weapon) (Variables|Character|GetMesh) "WeaponSocket" "SnapToTarget" "SnapToTarget" "SnapToTarget" true)
        (else
          (Transformation|AttachComponentToComponent (Variables|Default|GetAs%20BP%20Weapon) (Variables|Character|GetMesh) "weaponUnwield" "SnapToTarget" "SnapToTarget" "SnapToTarget" true))))
    (:then_1
      (bind _returnvalue_2 (Game|SpawnActorfromClass "/Game/Zak/UI/BP_TargetLock.BP_TargetLock_C" (Math|Transform|MakeTransform (Transformation|GetSocketLocation (Variables|Character|GetMesh) "spine_05") "0, 0, 0" "1.000000,1.000000,1.000000") "Undefined" "MultiplyWithRoot" 0 0))
      (Variables|Default|SetTargetLockWidget _returnvalue_2)
      (Default|SetMaxHealth (Variables|Default|GetBPC_DamageSystem) (Variables|Default|GetHealth) true)
      (bind _returnvalue_3 (UserInterface|CreateWidget "/Game/Omar/UI/WidgetBlueprints/WB_HealthBar.WB_HealthBar_C" 0 self))
      (bind _output_get (Variables|Default|SetHealthbarWidget _returnvalue_3))
      (UserInterface|SetWidget (Variables|Default|GetHealthWidget) _output_get)
      (CallFunction|Attack))))

(event EventUnlock
  ;[1 1 1] Target Lock
  (Rendering|SetVisibility (Variables|/Game/Zak/UI/BP_TargetLock.BP_TargetLock_C|GetTargetLockWidget (Variables|Default|GetTargetLockWidget)) false false)
  (Utilities|Time|ClearandInvalidateTimerbyHandle (stale EventLock _returnvalue)))

(event EventLock
  ;[1 1 1] Target Lock
  (Rendering|SetVisibility (Variables|/Game/Zak/UI/BP_TargetLock.BP_TargetLock_C|GetTargetLockWidget (Variables|Default|GetTargetLockWidget)) true false)
  (bind _returnvalue (Utilities|Time|SetTimerbyEvent (delegate Custom|LockLoop) 0.01 true)))

(event EventExecution
  (params (ExecutionSequence :type Integer))
  ;[1 1 1 1 30] Execution
  (switch int ExecutionSequence
    (:0
      (Variables|Default|SetExecutionSequence 0))
    (:1
      (Variables|Default|SetExecutionSequence 1))
    (:2
      (Variables|Default|SetExecutionSequence 2)))
  (Transformation|SetActorRotation (Math|Rotator|MakeRotator 0.0 0.0 (.yaw (Math|Rotator|FindLookatRotation (Transformation|GetActorLocation) (Transformation|GetActorLocation (Game|Player|GetPlayerPawn 0))))))
  (Variables|Default|SetExecuted? true)
  (Variables|/Game/Zak/DamageSystem/BPC_DamageSystem.BPC_DamageSystem_C|SetInvincible? (Variables|Default|GetBPC_DamageSystem) true)
  (Transformation|DetachFromComponent (Variables|Default|GetStaticMesh) "KeepWorld" "KeepWorld" "KeepWorld" true)
  (bind _notifyname (Animation|Montage|PlayMontage (Variables|Character|GetMesh) (Utilities|Select :Index (Variables|Default|GetExecutionSequence) :Option%200 "/Game/Great_Sword/Animations/Sequence2/02_Attack/15_Execution/02_Target/AS_Execution_Target_03_Seq_Montage.AS_Execution_Target_03_Seq_Montage" :Option%201 "/Game/Zak/TutorialSystem/Anims/Execution_Target_02_RM_Seq_Montage.Execution_Target_02_RM_Seq_Montage" :Option%202 "/Game/Dual_Sword/Animations/Sequence2/02_Attack/16_Exeution/02_Target/AS_Exeution_Target_02_Seq_Montage.AS_Exeution_Target_02_Seq_Montage") 0.7)
    (:OnNotifyBegin
      (switch name _notifyname
        (:Fracture
          (Utilities|FlowControl|Sequence
            (:then_0
              (Components|DestroyComponent (Variables|Character|GetMesh))
              (bind _as_bp_weapon (Variables|Default|GetAs%20BP%20Weapon)
                (:then
                  (Components|DestroyComponent (Variables|/Script/Engine.Actor|GetRootComponent _as_bp_weapon)))
                (:else
                  _))
              (Game|SpawnActorfromClass "/Game/Zak/Fracture/BP_FractureDummy.BP_FractureDummy_C" (Transformation|GetActorTransform) "Undefined" "OverrideRootScale" 0 0)
              (Game|SpawnActorfromClass "/Game/Zak/Interractible/FS_Impact.FS_Impact_C" (Transformation|GetActorTransform) "AlwaysSpawn" "MultiplyWithRoot" 0 0)
              (CallFunction|Death)
              (Actor|DestroyActor))
            (:then_1
              (bind _as_bp_weapon_2 (Variables|Default|GetAs%20BP%20Weapon)
                (:then
                  (Transformation|DetachFromActor _as_bp_weapon_2 "KeepWorld" "KeepWorld" "KeepWorld")
                  (Collision|SetCollisionEnabled (Variables|/Game/Zak/Weapons/BP_Weapon.BP_Weapon_C|GetWeapon _as_bp_weapon_2) "QueryAndPhysics")
                  (Physics|SetSimulatePhysics (Variables|/Game/Zak/Weapons/BP_Weapon.BP_Weapon_C|GetWeapon _as_bp_weapon_2) true))
                (:else)))))))))

(event EventLoadData
  (params (SaveGameRef :type BP%20Save%20Game%20Object%20Reference))
  (Variables|Default|SetControlsComplete? (Variables|/Game/Zak/SaveGame/BP_SaveGame.BP_SaveGame_C|GetControlsSave SaveGameRef)))

(event EventSaveData
  (params (SaveGameRef :type BP%20Save%20Game%20Object%20Reference))
  (Variables|/Game/Zak/SaveGame/BP_SaveGame.BP_SaveGame_C|SetControlsSave SaveGameRef (Variables|Default|GetControlsComplete?)))

(fn ConstructionScript
  (bind _bpc_damagesystem (Variables|Default|GetBPC_DamageSystem))
  (EventDispatchers|BindEventtoOnDeath _bpc_damagesystem (EventDispatchers|CreateEvent :!event Custom|Death))
  (EventDispatchers|BindEventtoOnDamageResponse _bpc_damagesystem (EventDispatchers|CreateEvent :!event Custom|DamageResponse))
  (EventDispatchers|BindEventtoOnAllTasksComplete (Variables|Default|GetControls) (EventDispatchers|CreateEvent :!event Custom|AllTasksComplete)))

(fn CalculateDamageDirection
  (params (DamagingActor :type Actor%20Object%20Reference) (DamagedActor :type Actor%20Object%20Reference))
  (bind _returnvalue (Transformation|GetActorRotation DamagedActor))
  (bind _returnvalue_2 (Transformation|GetActorLocation DamagingActor))
  (bind _returnvalue_3 (Transformation|GetActorLocation DamagedActor))
  (bind _returnvalue_4 (Math|Rotator|FindLookatRotation _returnvalue_2 _returnvalue_3))
  (bind _returnvalue_5 (Math|Rotator|Delta(Rotator) _returnvalue _returnvalue_4))
  (Utilities|IsValid DamagedActor
    (:Is%20Valid
      (if (or (Math|Float|InRange(Float) (.yaw _returnvalue_5) -1.8e+02 -135.0) (Math|Float|InRange(Float) (.yaw _returnvalue_5) 135.0 1.8e+02))
        (return "NewEnumerator0")
        (elif (Math|Float|InRange(Float) (.yaw _returnvalue_5) 45.0 135.0)
          (return "NewEnumerator2")
          (elif (Math|Float|InRange(Float) (.yaw _returnvalue_5) -135.0 -45.0)
            (return "NewEnumerator1")
            (elif (Math|Float|InRange(Float) (.yaw _returnvalue_5) -45.0 45.0)
              (return "NewEnumerator3"))))))))

(fn CalculateAccumulatedDamage)

(fn SetHitReactionMontage
  (params (DamageDirection :type E_DamageDirection%20Enum :default "NewEnumerator0"))
  (if (Utilities|Enum|Equal(Enum) DamageDirection "NewEnumerator0")
    (return "/Game/Zak/TutorialSystem/Anims/Hit_Large_Combat_F_Seq_Montage.Hit_Large_Combat_F_Seq_Montage")
    (elif (Utilities|Enum|Equal(Enum) DamageDirection "NewEnumerator2")
      (return "/Game/Zak/TutorialSystem/Anims/Hit_Combat_L_Seq_Montage.Hit_Combat_L_Seq_Montage")
      (elif (Utilities|Enum|Equal(Enum) DamageDirection "NewEnumerator1")
        (return "/Game/Zak/TutorialSystem/Anims/Hit_Combat_R_Seq_Montage.Hit_Combat_R_Seq_Montage")
        (elif (Utilities|Enum|Equal(Enum) DamageDirection "NewEnumerator3")
          (return "/Game/Zak/TutorialSystem/Anims/Hit_Combat_B_Seq_Montage.Hit_Combat_B_Seq_Montage"))))))

(fn WithinExecutionThreshold
  (bind _maxhealth (CallFunction|GetMaxHealth))
  (bind _health (CallFunction|GetCurrentHealth))
  (bind _isdead_ (CallFunction|IsDead))
  (if (Math|Boolean|ANDBoolean (not _isdead_) (<= (/ _health _maxhealth) (Variables|Default|GetExecutionThreshold)) (not (Variables|Default|GetExecuted?)))
    (if (Variables|Type|GetAttacker?)
      (Default|CallOnExplainExecution)
      (return true))
    (else
      (return false))))

(fn ExecuteAnim)

(fn CanbeExecuted
  (bind _healthbarwidget (Variables|Default|GetHealthbarWidget))
  (bind _executionwidget (Variables|Default|GetExecutionWidget))
  (bind _executionbox (Variables|/Game/Omar/UI/WidgetBlueprints/WB_HealthBar.WB_HealthBar_C|GetExecutionBox _healthbarwidget))
  (bind _canbeexecuted_ (CallFunction|WithinExecutionThreshold))
  (if (and _canbeexecuted_ (<= (Math|Vector|Distance(Vector) (Transformation|GetActorLocation (Game|GetPlayerCharacter 0)) (Transformation|GetActorLocation)) 2e+02))
    (if (not (Variables|Default|GetCanBeExecuted?))
      (Class|HorizontalBox|AddChildtoHorizontalBox _executionbox _executionwidget)
      (Variables|Default|SetCanBeExecuted? true)
      (return true))
    (else
      (Class|PanelWidget|RemoveChild _executionbox _executionwidget)
      (Variables|Default|SetCanBeExecuted? false)
      (return false))))

(fn GetCurrentHealth
  (bind _bpc_damagesystem (Variables|Default|GetBPC_DamageSystem))
  (Utilities|IsValid _bpc_damagesystem
    (:Is%20Valid
      (return (Variables|/Game/Zak/DamageSystem/BPC_DamageSystem.BPC_DamageSystem_C|GetCurrentHealth _bpc_damagesystem)))))

(fn GetMaxHealth
  (bind _bpc_damagesystem (Variables|Default|GetBPC_DamageSystem))
  (Utilities|IsValid _bpc_damagesystem
    (:Is%20Valid
      (return (Variables|/Game/Zak/DamageSystem/BPC_DamageSystem.BPC_DamageSystem_C|GetMaxHealth _bpc_damagesystem)))))

(fn Heal
  (params (Amount :type Float%20%28double-precision%29))
  (return 0.0))

(fn IsAttacking
  (return false))

(fn IsDead
  (return false))

(fn IsInvincible
  (return false))

(fn TakeDamage
  (params (DamageInfo :type S%20Damage%20Info%20Structure))
  (bind (_wasdamaged_ _damageamount _wasparried_ _healthremaining) (Default|TakeDamage (Variables|Default|GetBPC_DamageSystem) DamageInfo))
  (if _wasparried_
    (return false 0.0 true 0.0)
    (elif _wasdamaged_
      (Variables|Default|SetDamageTaken _damageamount)
      (CallFunction|CalculateAccumulatedDamage)
      (return true _damageamount false _healthremaining))))