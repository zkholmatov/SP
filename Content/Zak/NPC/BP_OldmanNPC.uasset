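; Old man NPC that shows a widget while the player is within its sphere and triggers a world change on first interaction.
; Interacting broadcasts an NPC-interacted event and uses World Partition data layers to drop one layer to Loaded.
; If the falling-stone flag is set, it also plays an earthquake shake and sound, activates the incoming layer and switches music triggers from tutorial to dungeon music.
; Dialogue is only a debug print; its audio-and-destroy chain is unconnected.
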(event OnComponentBeginOverlap(Sphere)
  (params (OverlappedComponent :type Primitive%20Component%20Object%20Reference) (OtherActor :type Actor%20Object%20Reference) (OtherComp :type Primitive%20Component%20Object%20Reference) (OtherBodyIndex :type Integer) (bFromSweep :type Boolean) (SweepResult :type Hit%20Result%20Structure%20%28by%20ref%29))
  (Utilities|Casting|CastToBP_Player OtherActor)
  (Rendering|SetVisibility (Variables|Default|GetWidget) true false))

(event OnComponentEndOverlap(Sphere)
  (params (OverlappedComponent :type Primitive%20Component%20Object%20Reference) (OtherActor :type Actor%20Object%20Reference) (OtherComp :type Primitive%20Component%20Object%20Reference) (OtherBodyIndex :type Integer))
  (Utilities|Casting|CastToBP_Player OtherActor)
  (Rendering|SetVisibility (Variables|Default|GetWidget) false false))

(event EventInteract
  (if true
    (Utilities|FlowControl|DoOnce false
      (:Completed
        (Development|PrintString "Dialogue")
        (Default|CallOnNPCInterracted)
        (bind _returnvalue (WorldPartition|GetDataLayerManager)) ; get data layer manager for world level partition as reference to set data layer in runtime
        (DataLayers|SetDataLayerRuntimeState _returnvalue (Variables|Default|GetOutDataLayerAsset) "Loaded" false :!class /Script/Engine.DataLayerManager) ; Function to toggle data layers
        (if (Variables|Default|GetbPlayFallingStone)
          (Variables|Default|SetbPlayFallingStone false) ; set falling stone boolean to false after single use so it cant be used again to determine functionality that follows
          (Camera|PlayWorldCameraShake "/Game/Zak/VFX/BP_EarthQuakeShake.BP_EarthQuakeShake_C" (Transformation|GetActorLocation (Game|GetPlayerCharacter 0)) 0.0 5e+02)
          (Audio|PlaySound2D "/Game/IntroMap/quake-and-break-99034.quake-and-break-99034" 1.0 1.0 0.0 0 0) ; Play sound of old data layer ie tower being moved
          (bind _returnvalue_2 (WorldPartition|GetDataLayerManager)) ; get data layer manager for world level partition as reference to set data layer in runtime
          (DataLayers|SetDataLayerRuntimeState _returnvalue_2 (Variables|Default|GetInDataLayerAsset) "Activated" false :!class /Script/Engine.DataLayerManager) ; Function to toggle data layers
          (bind _outactors (Actor|GetAllActorsOfClass "/Game/IntroMap/Blueprints/BP_MusicTrigger.BP_MusicTrigger_C")) ; get reference to actor of class BP Music toggle to call event s
          (Default|CallTriggerStopTutorialMusic _outactors) ; call event to stop current intro music
          (Default|CallTriggerStartDungeonMusic _outactors) ; call event to start new dungeon music
        )))))

(fn ConstructionScript)