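; Interactable NPC that shows a widget while the player is nearby and, on first interaction, fires a placeholder dialogue and notifies listeners.
; Flagged NPCs also reveal the next level area by swapping runtime Data Layers, switching tutorial music to dungeon music, and playing a one-time quake.
; Loading through the GameInstance reapplies a saved reveal without the quake and destroys NPCs already interacted with, matched by display name.
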(event OnComponentBeginOverlap(Sphere)
  (params (OverlappedComponent :type Primitive%20Component%20Object%20Reference) (OtherActor :type Actor%20Object%20Reference) (OtherComp :type Primitive%20Component%20Object%20Reference) (OtherBodyIndex :type Integer) (bFromSweep :type Boolean) (SweepResult :type Hit%20Result%20Structure%20%28by%20ref%29))
  (Utilities|Casting|CastToBP_Player OtherActor)
  (Rendering|SetVisibility (Variables|Default|GetWidget) true false))

(event OnComponentEndOverlap(Sphere)
  (params (OverlappedComponent :type Primitive%20Component%20Object%20Reference) (OtherActor :type Actor%20Object%20Reference) (OtherComp :type Primitive%20Component%20Object%20Reference) (OtherBodyIndex :type Integer))
  (Utilities|Casting|CastToBP_Player OtherActor)
  (Rendering|SetVisibility (Variables|Default|GetWidget) false false))

(event Custom|RevealLevel
  (Variables|Default|SetLevelRevealed? true)
  (bind _returnvalue (WorldPartition|GetDataLayerManager)) ; get data layer manager for world level partition as reference to set data layer in runtime
  (DataLayers|SetDataLayerRuntimeState _returnvalue (Variables|Default|GetOutDataLayerAsset) "Loaded" false :!class /Script/Engine.DataLayerManager) ; Function to toggle data layers
  (bind _returnvalue_2 (WorldPartition|GetDataLayerManager)) ; get data layer manager for world level partition as reference to set data layer in runtime
  (DataLayers|SetDataLayerRuntimeState _returnvalue_2 (Variables|Default|GetInDataLayerAsset) "Activated" false :!class /Script/Engine.DataLayerManager) ; Function to toggle data layers
  (bind _outactors (Actor|GetAllActorsOfClass "/Game/IntroMap/Blueprints/BP_MusicTrigger.BP_MusicTrigger_C")) ; get reference to actor of class BP Music toggle to call event s
  (Default|CallTriggerStopTutorialMusic _outactors) ; call event to stop current intro music
  (Default|CallTriggerStartDungeonMusic _outactors) ; call event to start new dungeon music
  (if (Variables|Default|GetbPlayFallingStone)
    (Variables|Default|SetbPlayFallingStone false) ; set falling stone boolean to false after single use so it cant be used again to determine functionality that follows
    (Camera|PlayWorldCameraShake "/Game/Zak/VFX/BP_EarthQuakeShake.BP_EarthQuakeShake_C" (Transformation|GetActorLocation (Game|GetPlayerCharacter 0)) 0.0 5e+02)
    (Audio|PlaySoundatLocation "/Game/IntroMap/quake-and-break-99034.quake-and-break-99034" "12994.174594,3367.013513,2293.326311" "0, 0, 0" 1.0 1.0 0.0 "/Game/Zak/NPC/Earthquake.Earthquake" 0 0 0)))

(event EventSaveData
  (params (SaveGameRef :type BP%20Save%20Game%20Object%20Reference))
  (Variables|/Game/Zak/SaveGame/BP_SaveGame.BP_SaveGame_C|SetLevelRevealed? SaveGameRef (Variables|Default|GetLevelRevealed?))
  (if (Variables|Default|GetInterracted?)
    (Utilities|Array|AddUnique (.npcname (Variables|/Game/Zak/SaveGame/BP_SaveGame.BP_SaveGame_C|GetNPCSave SaveGameRef)) (Utilities|GetDisplayName self))))

(event EventInteract
  (Variables|Default|SetInterracted? true)
  (Utilities|FlowControl|DoOnce false
    (:Completed
      (Development|PrintString "Dialogue")
      (Default|CallOnNPCInterracted)
      (if (Variables|Default|GetShouldMoveRock?)
        (CallFunction|RevealLevel)))))

(event EventLoadData
  (params (SaveGameRef :type BP%20Save%20Game%20Object%20Reference))
  (Variables|Default|SetbPlayFallingStone (not (Variables|/Game/Zak/SaveGame/BP_SaveGame.BP_SaveGame_C|GetLevelRevealed? SaveGameRef)))
  (bind _output_get (Variables|Default|SetLevelRevealed? (Variables|/Game/Zak/SaveGame/BP_SaveGame.BP_SaveGame_C|GetLevelRevealed? SaveGameRef)))
  (if _output_get
    (CallFunction|RevealLevel))
  (for _array_element (.npcname (Variables|/Game/Zak/SaveGame/BP_SaveGame.BP_SaveGame_C|GetNPCSave SaveGameRef))
    (if (Utilities|Enum|Equal(Enum) _array_element (Utilities|GetDisplayName self))
      (Actor|DestroyActor))))

(event EventBeginPlay
  (bind _asbp_game_instance (Utilities|Casting|CastToBP_GameInstance (Game|GetGameInstance)))
  (Default|RequestLoad _asbp_game_instance self))

(fn ConstructionScript)