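; Fracture base actor that breaks a Geometry Collection with impact effects and supports dissolving it.
; On BeginPlay it spawns the FS_Impact field at FractureLoc, plus a one-shot NS_Execute Niagara burst and parry camera shake centered on the player.
; Dissolve feeds alpha and edge color to both the collection's materials and DissolveFX, boosting the material color, then creates dynamic instances for each material slot after those parameter writes.
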(event EventBeginPlay
  (Game|SpawnActorfromClass "/Game/Zak/WorldInterractible/FS_Impact.FS_Impact_C" (Math|Transform|MakeTransform (Transformation|GetWorldLocation (Variables|Default|GetFractureLoc)) "0, 0, 0" "1.000000,1.000000,1.000000") "AlwaysSpawn" "MultiplyWithRoot" 0 0)
  (Utilities|FlowControl|DoOnce false
    (:Completed
      (Niagara|SpawnSystematLocation "/Game/Zak/VFX/Niagara/NS_Execute.NS_Execute" (Transformation|GetWorldLocation (Variables|Default|GetFractureLoc)))
      (Camera|PlayWorldCameraShake "/Game/Zak/VFX/BP_ParryCameraShake.BP_ParryCameraShake_C" (Transformation|GetActorLocation (Game|GetPlayerCharacter 0)) 0.0 5e+02))))

(fn ConstructionScript)

(fn Dissolve
  (params (Alpha :type Float%20%28double-precision%29) (EdgeColor :type Linear%20Color%20Structure) (ColorBoost :type Float%20%28double-precision%29))
  (bind _dissolvefx (Variables|Default|GetDissolveFX))
  (bind _geometrycollection (Variables|Default|GetGeometryCollection))
  (Rendering|Material|SetScalarParameterValueonMaterials (Variables|Default|GetGeometryCollection) "Alpha" Alpha)
  (Niagara|SetNiagaraVariable(Float) _dissolvefx "Alpha" Alpha)
  (Niagara|SetNiagaraVariable(LinearColor) _dissolvefx "EdgeColor" EdgeColor)
  (Rendering|Material|SetVectorParameterValueonMaterials _geometrycollection "EdgeColor" (* (Math|Conversions|ToVector(LinearColor) EdgeColor) ColorBoost))
  (for (_array_element _array_index) (Rendering|Material|GetMaterials _geometrycollection)
    (Rendering|Material|CreateDynamicMaterialInstance (Variables|Default|GetGeometryCollection) _array_index _array_element "None" :!class /Script/Engine.PrimitiveComponent)))