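; After-image VFX actor that leaves a frozen, fading copy of a character holding Frostmourne.
; On BeginPlay it snaps the child-actor sword to the PoseableMesh's SwordSocket and copies the pose from MeshToCopy.
; It creates dynamic materials for the body, an extra SkeletalMesh and the weapon, with separate timelines driving their Fade parameters.
; Whichever timeline finishes first destroys the actor.
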(event EventBeginPlay
  (bind _poseablemesh (Variables|Default|GetPoseableMesh))
  (bind _skeletalmesh (Variables|Default|GetSkeletalMesh))
  (bind _asbp_frostmourne (Utilities|Casting|CastToBP_Frostmourne (Variables|/Script/Engine.ChildActorComponent|GetChildActor (Variables|Default|GetChildActor))))
  (bind _output_get (Variables|Default|SetAs%20BP%20Frostmourne _asbp_frostmourne))
  (Transformation|AttachComponentToComponent _output_get (Variables|Default|GetPoseableMesh) "SwordSocket" "SnapToTarget" "SnapToTarget" "SnapToTarget" true)
  (bind _meshtocopy (Variables|Default|GetMeshToCopy)
    (:then
      (Class|PoseableMeshComponent|CopyPosefromSkeletalComponent (Variables|Default|GetPoseableMesh) _meshtocopy)
      (for (_array_element _array_index) (Rendering|Material|GetMaterials _poseablemesh)
        (bind _returnvalue (Rendering|Material|CreateDynamicMaterialInstance _poseablemesh _array_index _array_element "None" :!class /Script/Engine.PrimitiveComponent))
        (Utilities|Array|SetArrayElem (Variables|Default|GetDynamicMaterials) _array_index _returnvalue true)
        (Utilities|FlowControl|Sequence
          (:then_0
            (bind _fadetrack (Timeline|FadeTimeline Play)
              (:Update
                (Rendering|Material|SetScalarParameterValue (Utilities|Array|Get(acopy) (Variables|Default|GetDynamicMaterials) 1) "Fade" _fadetrack :!class /Script/Engine.MaterialInstanceDynamic))
              (:Finished
                (Actor|DestroyActor))))
          (:then_1
            (bind _fadetrack_2 (Timeline|Timeline Play)
              (:Update
                (Rendering|Material|SetScalarParameterValue (Utilities|Array|Get(acopy) (Variables|Default|GetDynamicMaterials)) "Fade" _fadetrack_2 :!class /Script/Engine.MaterialInstanceDynamic))
              (:Finished
                (Actor|DestroyActor))))
          (:then_2
            (bind _returnvalue_2 (Rendering|Material|CreateDynamicMaterialInstance _skeletalmesh 0 (Rendering|Material|GetMaterial _skeletalmesh 0) "None" :!class /Script/Engine.PrimitiveComponent))
            (bind _fadetrack_3 (Timeline|Timeline_0 Play)
              (:Update
                (Rendering|Material|SetScalarParameterValue _returnvalue_2 "Fade" _fadetrack_3 :!class /Script/Engine.MaterialInstanceDynamic))
              (:Finished
                (Actor|DestroyActor))))
          (:then_3
            (bind _returnvalue_3 (Rendering|Material|CreateDynamicMaterialInstance (Variables|/Game/Zak/Weapons/Frostmourne/BP_Frostmourne.BP_Frostmourne_C|GetWeapon (Variables|Default|GetAs%20BP%20Frostmourne)) 0 (Rendering|Material|GetMaterial (Variables|/Game/Zak/Weapons/Frostmourne/BP_Frostmourne.BP_Frostmourne_C|GetWeapon (Variables|Default|GetAs%20BP%20Frostmourne)) 0) "None" :!class /Script/Engine.PrimitiveComponent))
            (bind _fadetrack_4 (Timeline|Timeline_1 Play)
              (:Update
                (Rendering|Material|SetScalarParameterValue _returnvalue_3 "Fade" _fadetrack_4 :!class /Script/Engine.MaterialInstanceDynamic))
              (:Finished
                (Actor|DestroyActor)))))))
    (:else)))

(fn ConstructionScript)