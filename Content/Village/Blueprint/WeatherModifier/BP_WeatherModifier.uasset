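; Level actor that controls village weather by writing snow, rain and wind values into the MPC_Weather material parameter collection.
; The construction script detects changed weather or wind presets, resets the matching variables, prints a notice, then pushes all values to the collection.
; BeginPlay pushes them again for play mode.
; A construction-time check destroys the actor, with a warning, if another instance already exists in the level.
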(event EventBeginPlay
  ;[1 1 1] Sets weathers options in play mode
  (1.0.WeatherSettings|ApplytoMaterialParameterCollection))

(event Collision|EventActorBeginOverlap
  (params (OtherActor :type Actor%20Object%20Reference)))

(event EventTick
  (params (DeltaSeconds :type Float%20%28single-precision%29)))

(fn ConstructionScript
  (1.0.WeatherSettings|ForceOneInstance)
  (1.0.WeatherSettings|WeatherPresetChanged true)
  (1.0.WeatherSettings|WindPresetChanged true)
  (1.0.WeatherSettings|ApplytoMaterialParameterCollection))

(fn ApplytoMaterialParameterCollection
  ;[0.03646 0.03646 0.03646] Snow
  (Rendering|Material|SetScalarParameterValue "/Game/Village/MPC/MPC_Weather.MPC_Weather" "SnowAmount" (Variables|1.0.WeatherSettings|WorldMaterialParameters|Snow|GetsnowAmount) :!class /Script/Engine.KismetMaterialLibrary)
  (Rendering|Material|SetScalarParameterValue "/Game/Village/MPC/MPC_Weather.MPC_Weather" "SnowAmount_Ground" (Variables|1.0.WeatherSettings|WorldMaterialParameters|Snow|GetsnowAmount_Ground) :!class /Script/Engine.KismetMaterialLibrary)
  (Rendering|Material|SetScalarParameterValue "/Game/Village/MPC/MPC_Weather.MPC_Weather" "Snow?" (Math|Conversions|ToFloat(Boolean) (Variables|1.0.WeatherSettings|WorldMaterialParameters|Snow|Getsnow?)) :!class /Script/Engine.KismetMaterialLibrary)
  (Rendering|Material|SetScalarParameterValue "/Game/Village/MPC/MPC_Weather.MPC_Weather" "SnowTopMask" (Variables|1.0.WeatherSettings|WorldMaterialParameters|Snow|GetsnowTopMask) :!class /Script/Engine.KismetMaterialLibrary)
  ;[0.03646 0.03646 0.03646] Wind
  (Rendering|Material|SetScalarParameterValue "/Game/Village/MPC/MPC_Weather.MPC_Weather" "WindRotation_Tree" (Variables|1.0.WeatherSettings|WorldMaterialParameters|Wind|GetwindRotation_Tree) :!class /Script/Engine.KismetMaterialLibrary)
  (Rendering|Material|SetScalarParameterValue "/Game/Village/MPC/MPC_Weather.MPC_Weather" "WindSpeed_Tree" (Variables|1.0.WeatherSettings|WorldMaterialParameters|Wind|GetwindSpeed_Tree) :!class /Script/Engine.KismetMaterialLibrary)
  (Rendering|Material|SetScalarParameterValue "/Game/Village/MPC/MPC_Weather.MPC_Weather" "WindIntensity_Grass" (Variables|1.0.WeatherSettings|WorldMaterialParameters|Wind|GetwindIntensity_Grass) :!class /Script/Engine.KismetMaterialLibrary)
  (Rendering|Material|SetScalarParameterValue "/Game/Village/MPC/MPC_Weather.MPC_Weather" "WindSpeed_Grass" (Variables|1.0.WeatherSettings|WorldMaterialParameters|Wind|GetwindSpeed_Grass) :!class /Script/Engine.KismetMaterialLibrary)
  ;[0.03646 0.03646 0.03646] Rain
  (Rendering|Material|SetScalarParameterValue "/Game/Village/MPC/MPC_Weather.MPC_Weather" "RainWetness?" (Math|Conversions|ToFloat(Boolean) (Variables|1.0.WeatherSettings|WorldMaterialParameters|Rain|GetrainWetness?)) :!class /Script/Engine.KismetMaterialLibrary)
  (Rendering|Material|SetScalarParameterValue "/Game/Village/MPC/MPC_Weather.MPC_Weather" "RainTrail_Speed" (Variables|1.0.WeatherSettings|WorldMaterialParameters|Rain|GetrainTrail_Speed) :!class /Script/Engine.KismetMaterialLibrary)
  (Rendering|Material|SetScalarParameterValue "/Game/Village/MPC/MPC_Weather.MPC_Weather" "RainRipple?" (Math|Conversions|ToFloat(Boolean) (Variables|1.0.WeatherSettings|WorldMaterialParameters|Rain|GetrainRipple?)) :!class /Script/Engine.KismetMaterialLibrary))

(fn WeatherPresetChanged
  (params (bPrint :type Boolean))
  (if (!= (Variables|1.0.WeatherSettings|GetweatherPreset) (Variables|1.0.WeatherSettings|GetweatherPreset[DoNotChange]))
    (Variables|1.0.WeatherSettings|SetweatherPreset[DoNotChange] (Variables|1.0.WeatherSettings|GetweatherPreset))
    (1.0.WeatherSettings|SetWeatherPresetParameters)
    (if bPrint
      (Development|PrintString (Utilities|String|Append (Utilities|String|Append "[" (Utilities|GetDisplayName self) "]") " Weather preset have been changed to " (Utilities|String|Append "'" (Utilities|String|EnumtoString (Variables|1.0.WeatherSettings|GetweatherPreset)) "'") ". Some of material parameter variables in this blueprint are reset to match the weather preset. Click on ApplyPresetModifications to apply.") true true "(R=0.273651,G=1.000000,B=0.000000,A=1.000000)" 1e+01))))

(fn WindPresetChanged
  (params (bPrint :type Boolean))
  (if (!= (Variables|1.0.WeatherSettings|GetwindPreset) (Variables|1.0.WeatherSettings|GetwindPreset[DoNotChange]))
    (Variables|1.0.WeatherSettings|SetwindPreset[DoNotChange] (Variables|1.0.WeatherSettings|GetwindPreset))
    (1.0.WeatherSettings|SetWindPresetParameters)
    (if bPrint
      (Development|PrintString (Utilities|String|Append (Utilities|String|Append "[" (Utilities|GetDisplayName self) "]") " Wind preset have been changed to " (Utilities|String|Append "'" (Utilities|String|EnumtoString (Variables|1.0.WeatherSettings|GetwindPreset)) "'") ". Some of material parameter variables in this blueprint are reset to match the wind preset. Click on ApplyPresetModifications to apply.") true true "(R=0.273651,G=1.000000,B=0.000000,A=1.000000)" 1e+01))))

(fn ForceOneInstance
  (bind _outactors (Actor|GetAllActorsOfClass "BP_WeatherModifier_C"))
  (if (> (Utilities|Array|Length _outactors) 1)
    (Development|PrintString "Only one instance of Weather Modifier is allowed in the level. The newly added actor was destroyed" true true "(R=1.000000,G=0.000000,B=0.010267,A=1.000000)" 7.0)
    (Actor|DestroyActor)))

(fn SetWeatherPresetParameters
  (switch Utilities|FlowControl|Switch|SwitchonE_WeatherPreset (Variables|1.0.WeatherSettings|GetweatherPreset)
    (:NewEnumerator0
      ;[0.03646 0.03646 0.03646] Dry
      (Variables|1.0.WeatherSettings|WorldMaterialParameters|Snow|Setsnow? false)
      (Variables|1.0.WeatherSettings|WorldMaterialParameters|Snow|SetsnowAmount 0.0)
      (Variables|1.0.WeatherSettings|WorldMaterialParameters|Snow|SetsnowAmount_Ground 0.0)
      (Variables|1.0.WeatherSettings|WorldMaterialParameters|Snow|SetsnowTopMask 0.0)
      (Variables|1.0.WeatherSettings|WorldMaterialParameters|Rain|SetrainWetness? false)
      (Variables|1.0.WeatherSettings|WorldMaterialParameters|Rain|SetrainTrail_Speed 0.0)
      (Variables|1.0.WeatherSettings|WorldMaterialParameters|Rain|SetrainRipple? false))
    (:NewEnumerator1
      ;[1 1 1] Snowing
      (Variables|1.0.WeatherSettings|WorldMaterialParameters|Snow|Setsnow? true)
      (Variables|1.0.WeatherSettings|WorldMaterialParameters|Snow|SetsnowAmount 1.0)
      (Variables|1.0.WeatherSettings|WorldMaterialParameters|Snow|SetsnowAmount_Ground 1.0)
      (Variables|1.0.WeatherSettings|WorldMaterialParameters|Snow|SetsnowTopMask 0.0)
      (Variables|1.0.WeatherSettings|WorldMaterialParameters|Rain|SetrainWetness? false)
      (Variables|1.0.WeatherSettings|WorldMaterialParameters|Rain|SetrainTrail_Speed 0.0)
      (Variables|1.0.WeatherSettings|WorldMaterialParameters|Rain|SetrainRipple? true))
    (:NewEnumerator2
      ;[0 0.5819 0.5938] Raining
      (Variables|1.0.WeatherSettings|WorldMaterialParameters|Snow|Setsnow? false)
      (Variables|1.0.WeatherSettings|WorldMaterialParameters|Snow|SetsnowAmount 0.0)
      (Variables|1.0.WeatherSettings|WorldMaterialParameters|Snow|SetsnowAmount_Ground 0.0)
      (Variables|1.0.WeatherSettings|WorldMaterialParameters|Snow|SetsnowTopMask 0.0)
      (Variables|1.0.WeatherSettings|WorldMaterialParameters|Rain|SetrainWetness? true)
      (Variables|1.0.WeatherSettings|WorldMaterialParameters|Rain|SetrainTrail_Speed -0.18)
      (Variables|1.0.WeatherSettings|WorldMaterialParameters|Rain|SetrainRipple? true))
    (:NewEnumerator4
      ;[0.5625 0.5625 0.5625] After Snow
      (Variables|1.0.WeatherSettings|WorldMaterialParameters|Snow|Setsnow? true)
      (Variables|1.0.WeatherSettings|WorldMaterialParameters|Snow|SetsnowAmount 1.15)
      (Variables|1.0.WeatherSettings|WorldMaterialParameters|Snow|SetsnowAmount_Ground 1.35)
      (Variables|1.0.WeatherSettings|WorldMaterialParameters|Snow|SetsnowTopMask 0.01)
      (Variables|1.0.WeatherSettings|WorldMaterialParameters|Rain|SetrainWetness? false)
      (Variables|1.0.WeatherSettings|WorldMaterialParameters|Rain|SetrainTrail_Speed 0.0)
      (Variables|1.0.WeatherSettings|WorldMaterialParameters|Rain|SetrainRipple? false))
    (:NewEnumerator3
      ;[0 0.164 0.2031] After Rain
      (Variables|1.0.WeatherSettings|WorldMaterialParameters|Snow|Setsnow? false)
      (Variables|1.0.WeatherSettings|WorldMaterialParameters|Snow|SetsnowAmount 0.0)
      (Variables|1.0.WeatherSettings|WorldMaterialParameters|Snow|SetsnowAmount_Ground 0.0)
      (Variables|1.0.WeatherSettings|WorldMaterialParameters|Snow|SetsnowTopMask 0.0)
      (Variables|1.0.WeatherSettings|WorldMaterialParameters|Rain|SetrainWetness? true)
      (Variables|1.0.WeatherSettings|WorldMaterialParameters|Rain|SetrainTrail_Speed 0.0)
      (Variables|1.0.WeatherSettings|WorldMaterialParameters|Rain|SetrainRipple? false))))

(fn SetWindPresetParameters
  (switch Utilities|FlowControl|Switch|SwitchonE_WindPreset (Variables|1.0.WeatherSettings|GetwindPreset)
    (:NewEnumerator0
      (Variables|1.0.WeatherSettings|WorldMaterialParameters|Wind|SetwindSpeed_Tree 0.0)
      (Variables|1.0.WeatherSettings|WorldMaterialParameters|Wind|SetwindRotation_Tree 0.0)
      (Variables|1.0.WeatherSettings|WorldMaterialParameters|Wind|SetwindSpeed_Grass 0.0)
      (Variables|1.0.WeatherSettings|WorldMaterialParameters|Wind|SetwindIntensity_Grass 0.0))
    (:NewEnumerator1
      (Variables|1.0.WeatherSettings|WorldMaterialParameters|Wind|SetwindSpeed_Tree 3.0)
      (Variables|1.0.WeatherSettings|WorldMaterialParameters|Wind|SetwindRotation_Tree 0.5)
      (Variables|1.0.WeatherSettings|WorldMaterialParameters|Wind|SetwindSpeed_Grass 1.0)
      (Variables|1.0.WeatherSettings|WorldMaterialParameters|Wind|SetwindIntensity_Grass 2.0))
    (:NewEnumerator2
      (Variables|1.0.WeatherSettings|WorldMaterialParameters|Wind|SetwindSpeed_Tree 4.0)
      (Variables|1.0.WeatherSettings|WorldMaterialParameters|Wind|SetwindRotation_Tree 1.0)
      (Variables|1.0.WeatherSettings|WorldMaterialParameters|Wind|SetwindSpeed_Grass 1.5)
      (Variables|1.0.WeatherSettings|WorldMaterialParameters|Wind|SetwindIntensity_Grass 2.5))))