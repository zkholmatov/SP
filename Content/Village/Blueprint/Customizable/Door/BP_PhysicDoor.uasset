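; BP_PhysicDoor is a customizable village door that can swing as a physics object or stay non-simulated.
; Its construction script runs SetupDoor, optionally adding a wall piece at WallSocket and attaching the door mesh there.
; With PhysicsInteraction on, it configures damping, collision and a swing-limited physics constraint; otherwise it destroys the constraint.
; BeginPlay reapplies the physics simulation flag.
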(event EventBeginPlay
  (Physics|SetSimulatePhysics (Variables|Default|GetStaticMeshComponent) (Variables|1.DoorSettings|PhysicInteraction|GetbPhysicsInteraction?)))

(event Collision|EventActorBeginOverlap
  (params (OtherActor :type Actor%20Object%20Reference)))

(event EventTick
  (params (DeltaSeconds :type Float%20%28single-precision%29)))

(fn ConstructionScript
  (CallFunction|SetupDoor)
  (|CallParentFunction))

(fn SetupDoor
  (bind _wallsocket (Variables|Default|GetWallSocket))
  (bind _physicsconstraint (Variables|Default|GetPhysicsConstraint))
  (Utilities|FlowControl|Sequence
    (:then_0
      (if (Variables|1.DoorSettings|GetbWallVersion?)
        (bind _returnvalue (AddComponent|AddStaticMeshComponent false (Transformation|GetRelativeTransform (Variables|Default|GetWallSocket))))
        (Components|StaticMesh|SetStaticMesh _returnvalue (Variables|Components|GetWallPiece))
        (Transformation|AttachComponentToComponent _returnvalue (Variables|Default|GetWallSocket) "None" "SnapToTarget" "SnapToTarget" "SnapToTarget" true)
        (Transformation|AttachComponentToComponent (Variables|Default|GetStaticMeshComponent) _wallsocket "None" "KeepWorld" "KeepWorld" "KeepWorld" true)
        (Transformation|SetRelativeLocation _wallsocket "0, 0, 0" false false)
        (else
          (Transformation|AttachComponentToComponent (Variables|Default|GetStaticMeshComponent) (Variables|Default|GetDefaultSceneRoot) "None" "KeepWorld" "KeepWorld" "KeepWorld" true))))
    (:then_1
      ;[0.0625 0.0625 0.0625] Set Door Simulate Physic Settings
      (if (Variables|1.DoorSettings|PhysicInteraction|GetbPhysicsInteraction?)
        (Physics|SetSimulatePhysics (Variables|Default|GetStaticMeshComponent) true)
        (Class|PhysicsConstraintComponent|SetAngularSwing1Limit (Variables|Default|GetPhysicsConstraint) "ACM_Limited" (Variables|1.DoorSettings|PhysicInteraction|GetmovementAngle))
        (Class|PrimitiveComponent|SetAngularDamping (Variables|Default|GetStaticMeshComponent) (Variables|1.DoorSettings|PhysicInteraction|GetangularDamping))
        (Class|PrimitiveComponent|SetLinearDamping (Variables|Default|GetStaticMeshComponent) (Variables|1.DoorSettings|PhysicInteraction|GetlinearDamping))
        (Collision|SetCollisionProfileName (Variables|Default|GetStaticMeshComponent) (Variables|1.DoorSettings|PhysicInteraction|GetprofileName) true :!class /Script/Engine.PrimitiveComponent)
        (Collision|SetCollisionEnabled (Variables|Default|GetStaticMeshComponent) "QueryAndPhysics")
        (Collision|SetCollisionResponsetoChannel (Variables|Default|GetStaticMeshComponent) (Variables|1.DoorSettings|PhysicInteraction|GetinteractChannel) "ECR_Block")
        (Variables|Default|Setmobility "Movable")
        (else
          (Physics|SetSimulatePhysics (Variables|Default|GetStaticMeshComponent) false)
          (Components|DestroyComponent _physicsconstraint _physicsconstraint))))))