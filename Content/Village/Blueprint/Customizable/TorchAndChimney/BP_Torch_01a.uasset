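; BP_Torch_01a is a customizable village torch prop with a mesh, a point light and a fire effect.
; Its construction script keeps the mesh visible and uses a Fire toggle to show or hide the light and flame.
; A separate StickToWall function line-traces forward from the mesh, snaps the actor to the hit point and turns it to face into the surface along the inverted normal.
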(event EventBeginPlay)

(event Collision|EventActorBeginOverlap
  (params (OtherActor :type Actor%20Object%20Reference)))

(event EventTick
  (params (DeltaSeconds :type Float%20%28single-precision%29)))

(fn ConstructionScript
  (bind _fire_ (Variables|0.1.Customization|GetFire?))
  (Rendering|SetVisibility (Variables|Debug|GetStaticMeshComponent) true true)
  (Rendering|SetVisibility (Variables|Default|GetPointLight) _fire_ false)
  (Rendering|SetVisibility (Variables|Default|GetFire) _fire_ false))

(fn SticktoWall
  (bind (_outhit _returnvalue) (Collision|LineTraceByChannel (Transformation|GetWorldLocation (Variables|Debug|GetStaticMeshComponent)) (+ (* (Math|Vector|GetForwardVector (Variables|Debug|GetStaticMeshComponent)) 3e+03) (Transformation|GetWorldLocation (Variables|Debug|GetStaticMeshComponent))) "TraceTypeQuery1" true (Utilities|Array|MakeArray self) "ForDuration"))
  (if _returnvalue
    (Transformation|SetActorLocation (.Location (Collision|BreakHitResult _outhit)) false false)
    (Transformation|SetActorRotation (Math|Rotator|FindLookatRotation (.Location (Collision|BreakHitResult _outhit)) (+ (.Location (Collision|BreakHitResult _outhit)) (Math|Vector|NegateVector (.Normal (Collision|BreakHitResult _outhit))))))))