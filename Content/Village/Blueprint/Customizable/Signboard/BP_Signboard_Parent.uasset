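; Parent Blueprint for customizable village signboards, showing sign text as a static mesh looked up from an associative map.
; The construction script assigns that mesh to "Text"-tagged components and destroys "TextLocation" child actor components on the side excluded by SignTextSide.
; Scale and pitch apply to the remaining child actor components, while the position offset applies to the text meshes.
; ChildMaterialParametersSetup exposes text color as a material customization through Main_AlbedoTint.
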(event EventBeginPlay
  (|CallParentFunction) ; This node is disabled and will not be called.\nDrag off pins to build functionality.
)

(event Collision|EventActorBeginOverlap
  (params (OtherActor :type Actor%20Object%20Reference))
  (|CallParentFunction OtherActor) ; This node is disabled and will not be called.\nDrag off pins to build functionality.
)

(event EventTick
  (params (DeltaSeconds :type Float%20%28single-precision%29))
  (|CallParentFunction DeltaSeconds) ; This node is disabled and will not be called.\nDrag off pins to build functionality.
)

(fn ConstructionScript
  (CallFunction|SetupSignboard)
  (|CallParentFunction))

(fn ChildMaterialParametersSetup
  (Variables|Default|SetMaterialParameterCustomizations (Utilities|Array|MakeArray (Utilities|Struct|MakeS_MaterialCustomization (Actor|GetComponentsbyTag "/Script/Engine.StaticMeshComponent" "Text") (Utilities|Array|MakeArray (Utilities|Struct|MakeS_MaterialIdentity "NewEnumerator0" 0 "None" "(Main_AlbedoTint_1_D489A7A9459F9D39124498BB4BFBACA7=False,Main_AlbedoTint_CustomName_55_9E1F42A342902CDCCB51A49F2C96CA51=\"\",Main_AlbedoTint_ParameterName_56_40CE91F7469AB63531A3C2A6E1E95A1B=\"\",Main_AlbedoTint_ParameterType_54_59B13B674168F65815B630A49DD7F136=NewEnumerator0,Main_TintColor1_9_5A17B98048C14A59F770B28C6051B1A7=False,Main_TintColor_1_CustomName_57_C4BE043B462E247B1B5860AC19579144=\"\",Main_TintColor_1_ParameterName_58_700F84624AF13C0BA0E4F2B843565BA0=\"\",Main_TintColor_1_ParameterType_52_A90F9E1249CF35A4421393A18D99A2B7=NewEnumerator0,Main_TintColor_2_17_77F2CB35450CC848929C0980D37D8F5C=False,Main_TintColor_2_CustomName_59_C44C633E46FB9FEB5E457BABDBB5A450=\"\",Main_TintColor_2_ParameterName_60_05C6AF00407EDBE9FC0DD9BA0FFF173F=\"\",Main_TintColor_2_ParameterType_49_F30FC7E34645797292BCBF82E26635A5=NewEnumerator0,Main_EmissiveColor_26_762346964F5E278F2CE28CAF44DAAFF5=False,Main_EmissiveColor_CustomName_61_DFF954F949C5BCA0B32AABBF1656C786=\"\",Main_EmissiveColor_ParameterName_62_A0BA7FE347187271E5458596A61DB06A=\"\",Main_EmissiveColor_ParameterType_47_0186E9E743EB1F850278C79AC9491FE5=NewEnumerator0,Main_Tile_34_7CE187F947F3D4EDD0010CAC8A1F5CDA=False,Main_Tile_CustomName_63_A7F32E7744697127C07A248B6B3D6ACE=\"\",Main_Tile_ParameterName_64_6F01B7AB4E90F79186F5E2AFCF253620=\"\",Main_Tile_ParameterType_45_9D740C3E4350825D1A5DCCA48AB43C61=NewEnumerator0)" (Utilities|Array|MakeArray (Utilities|Struct|MakeS_MaterialOptionLocal true "Text Color" "Main_AlbedoTint" "NewEnumerator0"))))))))

(fn SetupSignboard
  (bind _textassoc (Variables|0.1.Customization|GettextAssoc))
  (bind _signtext (Variables|0.1.Customization|GetsignText))
  (bind _initialadditivescale (Variables|0.1.Customization|GetinitialAdditiveScale))
  (bind _textscale (Variables|0.1.Customization|GettextScale))
  (bind _textlocationoffset (Variables|0.1.Customization|GettextLocationOffset))
  (bind (_value _returnvalue) (Utilities|Map|Find _textassoc _signtext))
  (bind _returnvalue_2 (+ _textscale _initialadditivescale))
  ;[0.03646 0.03646 0.03646] Find the correct text mesh from associate array
  (LocalVariables|SetLocal_text _value)
  (if _returnvalue
    ;[0.03646 0.03646 0.03646] Assign text mesh to all static mesh components with "Text" tag
    (for _array_element (Actor|GetComponentsbyTag "/Script/Engine.StaticMeshComponent" "Text")
      (Components|StaticMesh|SetStaticMesh _array_element (LocalVariables|GetLocal_text)))
    (else
      ;[0.03646 0.03646 0.03646] Text scaling applied to child actor that contains the text mesh
      (Development|PrintString "Sign text mesh was not found" true true "(R=1.000000,G=0.000000,B=0.007374,A=1.000000)")))
  (for _array_element_2 (Actor|GetComponentsbyTag "/Script/Engine.ChildActorComponent" "TextLocation")
    (switch Utilities|FlowControl|Switch|SwitchonE_Signboard_Side (Variables|0.1.Customization|GetsignTextSide)
      (:NewEnumerator0
        ;;[0.227 0.000607 0.000607] Destroy Front and Back text according to the enum
        (if (Utilities|Array|ContainsItem (Variables|/Script/Engine.ActorComponent|GetComponentTags _array_element_2) "Back")
          (for _array_element_3 (Components|GetChildrenComponents _array_element_2 true) :!label _label
            (Components|DestroyComponent _array_element_3))
          (Components|DestroyComponent _array_element_2)))
      (:NewEnumerator1
        (if (Utilities|Array|ContainsItem (Variables|/Script/Engine.ActorComponent|GetComponentTags _array_element_2) "Front")
          (goto _label)))))
  (for _array_element_4 (Actor|GetComponentsbyTag "/Script/Engine.ChildActorComponent" "TextLocation")
    (Transformation|SetRelativeScale3D _array_element_4 (Math|Vector|MakeVector (.x _returnvalue_2) 0.0 (.y _returnvalue_2)))
    (Transformation|SetRelativeRotation _array_element_4 (Math|Rotator|MakeRotator 0.0 (Variables|0.1.Customization|GettextRotationOffset) 0.0) false false))
  ;[0.03646 0.03646 0.03646] Relative offset
  (for _array_element_5 (Actor|GetComponentsbyTag "/Script/Engine.StaticMeshComponent" "Text")
    (Utilities|IsValid _array_element_5
      (:Is%20Valid
        (Transformation|SetRelativeLocation _array_element_5 (Math|Vector|MakeVector (.x _textlocationoffset) 0.0 (.y _textlocationoffset)) false false)))))