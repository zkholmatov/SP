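; Lightning and thunder actor that simulates storm strikes by flashing a referenced directional light at random intervals while Active.
; It caches the light's intensity and color, then loops a timeline whose rounded-up multiplier adds a random, clamped intensity boost.
; Each strike's first brightening applies the lightning color and plays thunder; timeline completion restores the color.
; Construction warns about a missing light, and FindDirectionalLight can auto-assign one.
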(event Custom|InitiateLightning
  (bind _directionallight (Variables|1.Lightning|GetdirectionalLight))
  (bind _lightcomponent (Variables|/Script/Engine.Light|GetLightComponent _directionallight))
  (bind _intensity (Variables|/Script/Engine.LightComponentBase|GetIntensity _lightcomponent))
  ;[0.05208 0.05208 0.05208] Cache directional light + initiate lightning
  (CallFunction|CacheDirectionalLightVariables)
  (Utilities|FlowControl|Delay (Math|Random|RandomFloatinRange (Variables|1.Lightning|GetminDurationRepeating) (Variables|1.Lightning|GetmaxDurationRepeating)))
  (if (Variables|1.Lightning|GetbActive?) :!label _label
    (Utilities|FlowControl|Sequence
      (:then_0
        (goto _label_2 Reset))
      (:then_1
        (Variables|1.Lightning|SetlightningIntensity (Math|Random|RandomFloatinRange (Variables|1.Lightning|GetminLightningIntensity) (Variables|1.Lightning|GetmaxLightningIntensity)))
        ;[0.05729 0.05729 0.05729] Timeline to set the intensity and color of the directional light to simulate a lightning.
        (bind _intensitymultiplier (Timeline|LightningTimeline PlayFromStart)
          (:Update
            (if (!= _intensity (Math|Float|Clamp(Float) (+ (* (Math|Float|Ceil _intensitymultiplier) (Variables|1.Lightning|GetlightningIntensity)) (Variables|2.Cached|GetcachedDirectionalLightIntensity)) (Variables|1.Lightning|GetclampMinLightningIntensity) (Variables|1.Lightning|GetclampMaxLightningIntensity)))
              (Utilities|FlowControl|Sequence
                (:then_0
                  (if (> (Math|Float|Clamp(Float) (+ (* (Math|Float|Ceil _intensitymultiplier) (Variables|1.Lightning|GetlightningIntensity)) (Variables|2.Cached|GetcachedDirectionalLightIntensity)) (Variables|1.Lightning|GetclampMinLightningIntensity) (Variables|1.Lightning|GetclampMaxLightningIntensity)) _intensity)
                    (Utilities|FlowControl|DoOnce false :!label _label_2
                      (:Completed
                        (Rendering|Components|Light|SetLightColor (Variables|/Script/Engine.Light|GetLightComponent (Variables|1.Lightning|GetdirectionalLight)) (Variables|1.Lightning|GetlightningColor) true)
                        ;[1 0.3304 0] Play your audio here
                        (2.ThunderSound|PlayThunderSound)))))
                (:then_1
                  (Rendering|Components|Light|SetIntensity (Variables|/Script/Engine.Light|GetLightComponent (Variables|1.Lightning|GetdirectionalLight)) (Math|Float|Clamp(Float) (+ (* (Math|Float|Ceil _intensitymultiplier) (Variables|1.Lightning|GetlightningIntensity)) (Variables|2.Cached|GetcachedDirectionalLightIntensity)) (Variables|1.Lightning|GetclampMinLightningIntensity) (Variables|1.Lightning|GetclampMaxLightningIntensity)))))))
          (:Finished
            (Rendering|Components|Light|SetLightColor (Variables|/Script/Engine.Light|GetLightComponent (Variables|1.Lightning|GetdirectionalLight)) (Variables|2.Cached|GetcachedDirectionalLightColor) true)
            (Utilities|FlowControl|Delay (Math|Random|RandomFloatinRange (Variables|1.Lightning|GetminDurationRepeating) (Variables|1.Lightning|GetmaxDurationRepeating)))
            (goto _label)))))))

(event Custom|CacheDirectionalLightVariables
  (bind _directionallight (Variables|1.Lightning|GetdirectionalLight))
  (bind _lightcomponent (Variables|/Script/Engine.Light|GetLightComponent _directionallight))
  ;[0.0625 0.0625 0.0625] Cache directional light intensity and color
  (Variables|2.Cached|SetcachedDirectionalLightIntensity (Variables|/Script/Engine.LightComponentBase|GetIntensity _lightcomponent))
  (Variables|2.Cached|SetcachedDirectionalLightColor (Rendering|Components|Light|GetLightColor _lightcomponent)))

(event EventBeginPlay
  (if (and (Variables|1.Lightning|GetbActive?) (Utilities|IsValid (Variables|1.Lightning|GetdirectionalLight)))
    (CallFunction|InitiateLightning)))

(fn ConstructionScript
  (1.Lightning|ThunderSound|CheckforDirectionalLight))

(fn FindDirectionalLight
  ;[0.03646 0.03646 0.03646] Tries to find directional light in the level and assign it to the blueprint's detail panel slot
  (bind _returnvalue (Actor|GetActorOfClass "/Script/Engine.DirectionalLight"))
  (Utilities|IsValid _returnvalue
    (:Is%20Valid
      (bind _output_get (Variables|1.Lightning|SetdirectionalLight _returnvalue))
      (Development|PrintString (Utilities|String|Append "[BP_Lightning] Found and assigned " (Utilities|String|Append "\"" (Utilities|GetDisplayName _output_get) "\"") " to the directional light slot") true true "(R=0.000000,G=1.000000,B=0.019523,A=1.000000)" 4.0))
    (:Is%20Not%20Valid
      (Development|PrintString "[BP_Lightning] couldnt find any directional light in the level" true true "(R=1.000000,G=0.000000,B=0.014615,A=1.000000)" 4.0))))

(fn CheckforDirectionalLight
  ;[0.04167 0.04167 0.04167] Check for directional light validity
  (if (Variables|1.Lightning|GetbActive?)
    (Utilities|IsValid (Variables|1.Lightning|GetdirectionalLight)
      (:Is%20Not%20Valid
        (Development|PrintString "[BP_Lightning] is missing reference to DirectionalLight. It cannot simulate lightning effect. Assign a light source in the detail panel" true true "(R=1.000000,G=0.020756,B=0.000000,A=1.000000)" 5.0)))))

(fn PlayThunderSound
  (Utilities|IsValid (Variables|1.Lightning|ThunderSound|GetthunderSound)
    (:Is%20Valid
      (Audio|Components|Audio|SetSound (Variables|Default|GetThunderAudioComponent) (Variables|1.Lightning|ThunderSound|GetthunderSound))
      (Audio|Components|Audio|Play (Variables|Default|GetThunderAudioComponent) 0.0))))