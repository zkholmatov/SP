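; Spline Blueprint that shapes a sagging catenary curve, built in the construction script on top of its parent's spline setup.
; In Directional mode, a line trace along an arrow component finds the end point, and the spline is rebuilt with start, middle and end points.
; Weight, distance, height difference and center shift place the middle point, whose tangents are clamped to control curvature.
; Hand Adjust mode removes the arrow and skips the simulation.
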(event EventBeginPlay
  (|CallParentFunction) ; This node is disabled and will not be called.\nDrag off pins to build functionality.
)

(event Collision|EventActorBeginOverlap
  (params (OtherActor :type Actor%20Object%20Reference))
  (|CallParentFunction OtherActor) ; This node is disabled and will not be called.\nDrag off pins to build functionality.
)

(event EventTick
  (params (DeltaSeconds :type Float%20%28single-precision%29))
  (|CallParentFunction DeltaSeconds) ; This node is disabled and will not be called.\nDrag off pins to build functionality.
)

(event EventFSetMainSpline
  (Variables|Default|SetMainSpline (Variables|Default|GetSpline)))

(fn ConstructionScript
  (CallFunction|CatenarySettings)
  (|CallParentFunction)
  (Utilities|IsValid (Variables|Default|GetMainSpline)
    (:Is%20Valid
      (CallFunction|SimulateCatenary))))

(fn SimulateCatenary
  (bind _arrowcomponent (Variables|Default|GetarrowComponent))
  (bind _arrowcomponent_2 (Variables|Default|GetarrowComponent))
  (bind _returnvalue (Transformation|GetWorldTransform _arrowcomponent_2))
  (bind _returnvalue_2 (Transformation|GetRelativeTransform _arrowcomponent))
  (bind (_location _rotation _scale) (Math|Transform|BreakTransform _returnvalue_2))
  (bind (_location_2 _rotation_2 _scale_2) (Math|Transform|BreakTransform _returnvalue))
  (switch Utilities|FlowControl|Switch|SwitchonE_CatenaryType (Variables|3.CatenarySettings|GetcatenaryType)
    (:NewEnumerator0
      ;[0.01562 0.01562 0.01562] Clear Spline
      (Spline|ClearSplinePoints (Variables|Default|GetMainSpline) true)
      ;[0.01562 0.01562 0.01562] Normalize Spline Weight (Easier to modify from editor)
      (LocalVariables|SetLocal_splineWeight (/ (Variables|3.CatenarySettings|GetsplineWeight) 1e+01))
      ;[1 0.4068 0] Comment
      (LocalVariables|SetLocal_startingPointTransform (Math|Transform|MakeTransform (+ _location_2 (* (Math|Vector|GetForwardVector _rotation_2) (Variables|3.CatenarySettings|DirectionalCaterany|Tracing|GetlineTraceForwardStartOffset))) _rotation_2 _scale_2))
      (LocalVariables|SetLocal_startingPointTransform_Relative (Math|Transform|MakeTransform _location _rotation _scale))
      ;[0 0.02211 0.1302] Add starting point. It start from rear of the Arrow.
      (bind _output_get (LocalVariables|SetLocal_startPoint (Utilities|Struct|MakeSplinePoint 0.0 (.location (LocalVariables|GetLocal_startingPointTransform_Relative)) (Variables|Default|GetsplineType))))
      (Class|SplineComponent|AddPoint (Variables|Default|GetMainSpline) _output_get true)
      ;[0.06663 0.1559 0.2384] Line trace to find walls
      (bind (_outhit _returnvalue_3) (Collision|LineTraceByChannel (.location (LocalVariables|GetLocal_startingPointTransform)) (+ (.location (LocalVariables|GetLocal_startingPointTransform)) (* (Math|Vector|GetForwardVector (.rotation (LocalVariables|GetLocal_startingPointTransform))) (Variables|3.CatenarySettings|DirectionalCaterany|Tracing|GetlineTraceDistanceLimit))) (Variables|3.CatenarySettings|DirectionalCaterany|Tracing|GettraceChannel) (Variables|3.CatenarySettings|DirectionalCaterany|Tracing|GettraceComplex) 0 (Variables|3.CatenarySettings|DirectionalCaterany|Tracing|GettraceDebugType) true (Variables|3.CatenarySettings|DirectionalCaterany|Arrow|GetarrowColor) "(R=0.000000,G=1.000000,B=0.000000,A=1.000000)" 2.0))
      ;[0.2159 0.001518 0.001518] Line Trace Result
      (LocalVariables|SetLocal_traceHit _outhit)
      (LocalVariables|SetLocal_hitResult _returnvalue_3)
      (LocalVariables|SetLocal_hitDistance (.distance (LocalVariables|GetLocal_traceHit)))
      (LocalVariables|SetLocal_impactPoint (+ (select (LocalVariables|GetLocal_hitResult) (.location (LocalVariables|GetLocal_traceHit)) (.traceend (LocalVariables|GetLocal_traceHit))) (* (Math|Vector|GetUnitDirection(Vector) (select (LocalVariables|GetLocal_hitResult) (.location (LocalVariables|GetLocal_traceHit)) (.traceend (LocalVariables|GetLocal_traceHit))) (.tracestart (LocalVariables|GetLocal_traceHit))) (Variables|3.CatenarySettings|DirectionalCaterany|Tracing|GetlineTraceForwardEndOffset))))
      (Spline|AddSplinePoint (Variables|Default|GetMainSpline) (- (+ (* (/ (- (LocalVariables|GetLocal_impactPoint) (.Location (Math|Transform|BreakTransform (LocalVariables|GetLocal_startingPointTransform)))) 2.0) (+ (Math|Float|Clamp(Float) (+ (Variables|3.CatenarySettings|GetshiftCenterWeight) (Math|Float|MapRangeClamped (.Z (Math|Vector|BreakVector (- (LocalVariables|GetLocal_impactPoint) (.Location (Math|Transform|BreakTransform (LocalVariables|GetLocal_startingPointTransform)))))) (/ (* (Math|Float|Absolute(Float) (LocalVariables|GetLocal_splineWeight)) (* (LocalVariables|GetLocal_hitDistance) -1.0)) (Math|Float|Absolute(Float) (LocalVariables|GetLocal_splineWeight))) (/ (* (Math|Float|Absolute(Float) (LocalVariables|GetLocal_splineWeight)) (LocalVariables|GetLocal_hitDistance)) (Math|Float|Absolute(Float) (LocalVariables|GetLocal_splineWeight))) -0.5 0.5)) -0.75 0.75) 1.0)) (.Location (Math|Transform|BreakTransform (LocalVariables|GetLocal_startingPointTransform)))) (Math|Vector|MakeVector 0.0 0.0 (* (LocalVariables|GetLocal_hitDistance) (* (LocalVariables|GetLocal_splineWeight) (Math|Float|MapRangeClamped (.Z (Math|Vector|BreakVector (- (LocalVariables|GetLocal_impactPoint) (.Location (Math|Transform|BreakTransform (LocalVariables|GetLocal_startingPointTransform)))))) (/ (* (Math|Float|Absolute(Float) (LocalVariables|GetLocal_splineWeight)) (* (LocalVariables|GetLocal_hitDistance) -1.0)) (Math|Float|Absolute(Float) (LocalVariables|GetLocal_splineWeight))) (/ (* (Math|Float|Absolute(Float) (LocalVariables|GetLocal_splineWeight)) (LocalVariables|GetLocal_hitDistance)) (Math|Float|Absolute(Float) (LocalVariables|GetLocal_splineWeight))) 0.0 1.0))))) "World" true)
      (Spline|AddSplinePoint (Variables|Default|GetMainSpline) (LocalVariables|GetLocal_impactPoint) "World" true)
      (Spline|SetTangentatSplinePoint (Variables|Default|GetMainSpline) 2 (Math|Vector|MakeVector 0.0 0.0 0.0) "Local" true)
      (Spline|SetTangentsatSplinePoint (Variables|Default|GetMainSpline) 1 (* (Math|Vector|ClampVectorSize (Spline|GetTangentatSplinePoint (Variables|Default|GetMainSpline) 1 "Local") (* (Math|Float|MapRangeClamped (+ (LocalVariables|GetLocal_splineWeight) (Math|Float|Absolute(Float) (Variables|3.CatenarySettings|GetshiftCenterWeight))) 0.0 15.0 1.0 1.5) (Math|Vector|VectorLength (* (/ (- (LocalVariables|GetLocal_impactPoint) (.Location (Math|Transform|BreakTransform (LocalVariables|GetLocal_startingPointTransform)))) 2.0) (+ (Math|Float|Clamp(Float) (+ (Variables|3.CatenarySettings|GetshiftCenterWeight) (Math|Float|MapRangeClamped (.Z (Math|Vector|BreakVector (- (LocalVariables|GetLocal_impactPoint) (.Location (Math|Transform|BreakTransform (LocalVariables|GetLocal_startingPointTransform)))))) (/ (* (Math|Float|Absolute(Float) (LocalVariables|GetLocal_splineWeight)) (* (LocalVariables|GetLocal_hitDistance) -1.0)) (Math|Float|Absolute(Float) (LocalVariables|GetLocal_splineWeight))) (/ (* (Math|Float|Absolute(Float) (LocalVariables|GetLocal_splineWeight)) (LocalVariables|GetLocal_hitDistance)) (Math|Float|Absolute(Float) (LocalVariables|GetLocal_splineWeight))) -0.5 0.5)) -0.75 0.75) 1.0)))) (* (Math|Float|MapRangeClamped (+ (LocalVariables|GetLocal_splineWeight) (Math|Float|Absolute(Float) (Variables|3.CatenarySettings|GetshiftCenterWeight))) 0.0 15.0 1.0 1.5) (Math|Vector|VectorLength (* (/ (- (LocalVariables|GetLocal_impactPoint) (.Location (Math|Transform|BreakTransform (LocalVariables|GetLocal_startingPointTransform)))) 2.0) (+ (Math|Float|Clamp(Float) (+ (Variables|3.CatenarySettings|GetshiftCenterWeight) (Math|Float|MapRangeClamped (.Z (Math|Vector|BreakVector (- (LocalVariables|GetLocal_impactPoint) (.Location (Math|Transform|BreakTransform (LocalVariables|GetLocal_startingPointTransform)))))) (/ (* (Math|Float|Absolute(Float) (LocalVariables|GetLocal_splineWeight)) (* (LocalVariables|GetLocal_hitDistance) -1.0)) (Math|Float|Absolute(Float) (LocalVariables|GetLocal_splineWeight))) (/ (* (Math|Float|Absolute(Float) (LocalVariables|GetLocal_splineWeight)) (LocalVariables|GetLocal_hitDistance)) (Math|Float|Absolute(Float) (LocalVariables|GetLocal_splineWeight))) -0.5 0.5)) -0.75 0.75) 1.0))))) (Variables|3.CatenarySettings|GetcurvatureCenterTensionMultiplier)) (* (Math|Vector|ClampVectorSize (Spline|GetTangentatSplinePoint (Variables|Default|GetMainSpline) 1 "Local") (* (Math|Float|MapRangeClamped (+ (LocalVariables|GetLocal_splineWeight) (Math|Float|Absolute(Float) (Variables|3.CatenarySettings|GetshiftCenterWeight))) 0.0 15.0 1.0 1.5) (Math|Vector|VectorLength (* (/ (- (LocalVariables|GetLocal_impactPoint) (.Location (Math|Transform|BreakTransform (LocalVariables|GetLocal_startingPointTransform)))) 2.0) (+ (Math|Float|Clamp(Float) (+ (Variables|3.CatenarySettings|GetshiftCenterWeight) (Math|Float|MapRangeClamped (.Z (Math|Vector|BreakVector (- (LocalVariables|GetLocal_impactPoint) (.Location (Math|Transform|BreakTransform (LocalVariables|GetLocal_startingPointTransform)))))) (/ (* (Math|Float|Absolute(Float) (LocalVariables|GetLocal_splineWeight)) (* (LocalVariables|GetLocal_hitDistance) -1.0)) (Math|Float|Absolute(Float) (LocalVariables|GetLocal_splineWeight))) (/ (* (Math|Float|Absolute(Float) (LocalVariables|GetLocal_splineWeight)) (LocalVariables|GetLocal_hitDistance)) (Math|Float|Absolute(Float) (LocalVariables|GetLocal_splineWeight))) -0.5 0.5)) -0.75 0.75) 1.0)))) (* (Math|Float|MapRangeClamped (+ (LocalVariables|GetLocal_splineWeight) (Math|Float|Absolute(Float) (Variables|3.CatenarySettings|GetshiftCenterWeight))) 0.0 15.0 1.0 1.5) (Math|Vector|VectorLength (* (/ (- (LocalVariables|GetLocal_impactPoint) (.Location (Math|Transform|BreakTransform (LocalVariables|GetLocal_startingPointTransform)))) 2.0) (+ (Math|Float|Clamp(Float) (+ (Variables|3.CatenarySettings|GetshiftCenterWeight) (Math|Float|MapRangeClamped (.Z (Math|Vector|BreakVector (- (LocalVariables|GetLocal_impactPoint) (.Location (Math|Transform|BreakTransform (LocalVariables|GetLocal_startingPointTransform)))))) (/ (* (Math|Float|Absolute(Float) (LocalVariables|GetLocal_splineWeight)) (* (LocalVariables|GetLocal_hitDistance) -1.0)) (Math|Float|Absolute(Float) (LocalVariables|GetLocal_splineWeight))) (/ (* (Math|Float|Absolute(Float) (LocalVariables|GetLocal_splineWeight)) (LocalVariables|GetLocal_hitDistance)) (Math|Float|Absolute(Float) (LocalVariables|GetLocal_splineWeight))) -0.5 0.5)) -0.75 0.75) 1.0))))) (Variables|3.CatenarySettings|GetcurvatureCenterTensionMultiplier)) "Local" true))
    (:NewEnumerator1)))

(fn SetupArrow
  (bind _masterdrawdebug (Variables|Default|GetmasterDrawDebug))
  (bind _bshowarrow (Variables|3.CatenarySettings|DirectionalCaterany|Arrow|GetbShowArrow))
  (bind _masterdrawdebug_2 (Variables|Default|GetmasterDrawDebug))
  (bind _bshowarrow_2 (Variables|3.CatenarySettings|DirectionalCaterany|Arrow|GetbShowArrow))
  (bind _returnvalue (or _bshowarrow _masterdrawdebug_2))
  (bind _returnvalue_2 (or _bshowarrow_2 _masterdrawdebug))
  (switch Utilities|FlowControl|Switch|SwitchonE_CatenaryType (Variables|3.CatenarySettings|GetcatenaryType)
    (:NewEnumerator0
      ;[0.04167 0.04167 0.04167] Set arrow
      (bind _output_get (Variables|Default|SetarrowComponent (Variables|Default|GetArrow)))
      ;[0.04167 0.04167 0.04167] Hide the arrow if show arrow is disabled
      (Rendering|SetVisibility _output_get _returnvalue _returnvalue)
      (Development|SetHiddeninGame (Variables|Default|GetarrowComponent) _returnvalue_2 _returnvalue_2)
      ;[0.04167 0.04167 0.04167] Create the arrow
      (Components|Arrow|SetArrowColor(LinearColor) (Variables|Default|GetarrowComponent) (Variables|3.CatenarySettings|DirectionalCaterany|Arrow|GetarrowColor))
      (Variables|/Script/Engine.ArrowComponent|SetArrowSize (Variables|Default|GetarrowComponent) (Variables|3.CatenarySettings|DirectionalCaterany|Arrow|GetarrowSize))
      (Transformation|SetRelativeLocationAndRotation (Variables|Default|GetArrow) "0, 0, 0" "0, 0, 0" false false))
    (:NewEnumerator1
      (Components|DestroyComponent (Variables|Default|GetArrow)))))

(fn CatenarySettings
  (CallFunction|SetupArrow)
  (switch Utilities|FlowControl|Switch|SwitchonE_CatenaryType (Variables|3.CatenarySettings|GetcatenaryType)
    (:NewEnumerator0
      (Variables|Default|SetmaxSplinePoints 0)
      (Variables|Default|SetsplineType "CurveClamped"))
    (:NewEnumerator1
      ;[1 1 1] 0 = Infinite spline point
      (Variables|Default|SetmaxSplinePoints 0))))