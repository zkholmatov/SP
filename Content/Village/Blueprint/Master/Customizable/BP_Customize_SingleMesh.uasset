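; BP_Customize_SingleMesh is a customizable Blueprint child for a single static mesh with tintable material parameters.
; Its construction script runs the parent's, then applies the Mobility setting to the mesh component.
; The ChildMaterialParametersSetup override turns each TintParameters entry into a material option named from TintCustomName and a one-based index.
; It stores these options as one MaterialParameterCustomizations entry bound to that mesh, with no active event logic.
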(event EventBeginPlay
  (|CallParentFunction) ; This node is disabled and will not be called.\nDrag off pins to build functionality.
)

(event Collision|EventActorBeginOverlap
  (params (OtherActor :type Actor%20Object%20Reference))
  (|CallParentFunction OtherActor) ; This node is disabled and will not be called.\nDrag off pins to build functionality.
)

(event EventTick
  (params (DeltaSeconds :type Float%20%28single-precision%29))
  (|CallParentFunction DeltaSeconds) ; This node is disabled and will not be called.\nDrag off pins to build functionality.
)

(fn ConstructionScript
  (|CallParentFunction)
  (Transformation|SetMobility (Variables|Default|GetStaticMeshComponent) (Variables|0.0.Master|Getmobility)))

(fn ChildMaterialParametersSetup
  (|CallParentFunction)
  (Utilities|Array|Clear (LocalVariables|GetLocal_materialOptions))
  (for (_array_element _array_index) (Variables|0.1.Customization|GettintParameters)
    (Utilities|Array|Add (LocalVariables|GetLocal_materialOptions) (Utilities|Struct|MakeS_MaterialOptionLocal true (Utilities|String|StringToName (Utilities|String|Append (Utilities|String|ToString(Name) (Variables|0.1.Customization|GettintCustomName)) "_Tint_" (Utilities|String|ToString(Integer) (+ _array_index 1)))) _array_element "NewEnumerator0")))
  (Variables|Default|SetMaterialParameterCustomizations (Utilities|Array|MakeArray (Utilities|Struct|MakeS_MaterialCustomization (Utilities|Array|MakeArray (Variables|Default|GetStaticMeshComponent)) (Utilities|Array|MakeArray (Utilities|Struct|MakeS_MaterialIdentity "NewEnumerator0" 0 "None" "(Main_AlbedoTint_1_D489A7A9459F9D39124498BB4BFBACA7=False,Main_AlbedoTint_CustomName_55_9E1F42A342902CDCCB51A49F2C96CA51=\"\",Main_AlbedoTint_ParameterName_56_40CE91F7469AB63531A3C2A6E1E95A1B=\"\",Main_AlbedoTint_ParameterType_54_59B13B674168F65815B630A49DD7F136=NewEnumerator0,Main_TintColor1_9_5A17B98048C14A59F770B28C6051B1A7=False,Main_TintColor_1_CustomName_57_C4BE043B462E247B1B5860AC19579144=\"\",Main_TintColor_1_ParameterName_58_700F84624AF13C0BA0E4F2B843565BA0=\"\",Main_TintColor_1_ParameterType_52_A90F9E1249CF35A4421393A18D99A2B7=NewEnumerator0,Main_TintColor_2_17_77F2CB35450CC848929C0980D37D8F5C=False,Main_TintColor_2_CustomName_59_C44C633E46FB9FEB5E457BABDBB5A450=\"\",Main_TintColor_2_ParameterName_60_05C6AF00407EDBE9FC0DD9BA0FFF173F=\"\",Main_TintColor_2_ParameterType_49_F30FC7E34645797292BCBF82E26635A5=NewEnumerator0,Main_EmissiveColor_26_762346964F5E278F2CE28CAF44DAAFF5=False,Main_EmissiveColor_CustomName_61_DFF954F949C5BCA0B32AABBF1656C786=\"\",Main_EmissiveColor_ParameterName_62_A0BA7FE347187271E5458596A61DB06A=\"\",Main_EmissiveColor_ParameterType_47_0186E9E743EB1F850278C79AC9491FE5=NewEnumerator0,Main_Tile_34_7CE187F947F3D4EDD0010CAC8A1F5CDA=False,Main_Tile_CustomName_63_A7F32E7744697127C07A248B6B3D6ACE=\"\",Main_Tile_ParameterName_64_6F01B7AB4E90F79186F5E2AFCF253620=\"\",Main_Tile_ParameterType_45_9D740C3E4350825D1A5DCCA48AB43C61=NewEnumerator0)" (LocalVariables|GetLocal_materialOptions)))))))