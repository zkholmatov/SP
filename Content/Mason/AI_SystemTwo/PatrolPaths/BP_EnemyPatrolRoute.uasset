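; Spline-based patrol route actor that supplies enemy AI with waypoints to walk.
; A current index steps along the PatrolPath spline's points by a Direction value, which flips at the last and first points so the route ping-pongs.
; A getter returns the current spline point as a world-space position for the AI to move toward.
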(event Custom|IncrementPatrolPath
  (bind _output_get (Variables|Default|SetPatrolPathIndex (+ (Variables|Default|GetPatrolPathIndex) (Variables|Default|GetDirection))))
  (if (== _output_get (- (Spline|GetNumberOfSplinePoints (Variables|Default|GetPatrolPath)) 1))
    (Variables|Default|SetDirection -1)
    (elif (== (Variables|Default|GetPatrolPathIndex) 0)
      (Variables|Default|SetDirection 1))))

(fn ConstructionScript)

(fn GetSplinePointasWorldPos
  (return (Spline|GetLocationatSplinePoint (Variables|Default|GetPatrolPath) (Variables|Default|GetPatrolPathIndex) "World")))