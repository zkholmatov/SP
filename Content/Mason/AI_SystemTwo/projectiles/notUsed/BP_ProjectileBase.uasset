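; BP_ProjectileBase is a projectile actor, filed under notUsed, that flies toward a Target and damages what it overlaps.
; The construction script copies its speeds to ProjectileMovement, and BeginPlay sets velocity once toward the Target's location, with no effective validity guard.
; Overlaps call HandleBeginOverlap, then send parryable damage through a TakeDamage message.
; The hit event is empty, leaving its collision callback and impact emitter disconnected.
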(event OnComponentBeginOverlap(CollisionComponent)
  (params (OverlappedComponent :type Primitive%20Component%20Object%20Reference) (OtherActor :type Actor%20Object%20Reference) (OtherComp :type Primitive%20Component%20Object%20Reference) (OtherBodyIndex :type Integer) (bFromSweep :type Boolean) (SweepResult :type Hit%20Result%20Structure%20%28by%20ref%29))
  (Class|EnemyProjectile|HandleBeginOverlap OtherActor)
  (bind _damageamount (Class|BPIDamageable|TakeDamage(Message) OtherActor (Utilities|Struct|MakeS_DamageInfo (Variables|Default|GetProjectileDamage) "NewEnumerator2" "NewEnumerator3" true false "NewEnumerator0" self "/Game/Zak/AbyssalWarden/BP_Projectile.BP_Projectile_C")))
  (Class|BPIDamageable|GetCurrentHealth(Message) OtherActor))

(event OnComponentHit(CollisionComponent)
  (params (HitComponent :type Primitive%20Component%20Object%20Reference) (OtherActor :type Actor%20Object%20Reference) (OtherComp :type Primitive%20Component%20Object%20Reference) (NormalImpulse :type Vector :default "0, 0, 0") (Hit :type Hit%20Result%20Structure%20%28by%20ref%29)))

(event Custom|RotateToTarget
  ;[0 1 0.5922] rotate target -> Move to target
  (Variables|/Script/Engine.MovementComponent|SetVelocity (Variables|Default|GetProjectileMovement) (* (Math|Vector|GetUnitDirection(Vector) (Transformation|GetActorLocation) (Transformation|GetActorLocation (Variables|Default|GetTarget))) (Variables|Stats|GetInitial%20Speed))))

(event EventBeginPlay
  ;[1 1 1] Begin Play
  (Variables|Default|GetTarget
    (:then
      _)
    (:else
      _))
  ;;[0 1 0.5922] Rotate Target Function Call
  (CallFunction|RotatetoTarget))

(fn ConstructionScript
  (bind _projectilemovement (Variables|Default|GetProjectileMovement))
  (Variables|/Script/Engine.ProjectileMovementComponent|SetInitialSpeed _projectilemovement (Variables|Stats|GetInitial%20Speed))
  (Variables|/Script/Engine.ProjectileMovementComponent|SetMaxSpeed _projectilemovement (Variables|Stats|GetMax%20Speed)))