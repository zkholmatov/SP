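; Skull projectile, apparently for a summon attack, built as a child of a parent projectile Blueprint.
; The construction script sets its damage and homing acceleration, and BeginPlay sets its death timer after the parent logic runs.
; It overrides RotatetoTarget to launch in a random direction within a hemisphere centered on a fixed world-space diagonal between +X and up, scaled by InitialSpeed.
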(event EventBeginPlay
  (|CallParentFunction)
  (Variables|Default|SetProjectileDeathTimer 2.5))

(event Collision|EventActorBeginOverlap
  (params (OtherActor :type Actor%20Object%20Reference)))

(event EventTick
  (params (DeltaSeconds :type Float%20%28single-precision%29))
  (|CallParentFunction DeltaSeconds) ; This node is disabled and will not be called.\nDrag off pins to build functionality.
)

(event EventRotatetoTarget
  (Variables|/Script/Engine.MovementComponent|SetVelocity (Variables|Default|GetProjectileMovement) (* (Math|Random|RandomUnitVectorinConeinDegrees "1.000000,0.000000,1.000000" 9e+01) (Variables|Default|GetInitial%20Speed))))

(fn ConstructionScript
  (Variables|Default|SetProjectileDamage 5e+01)
  (Variables|/Script/Engine.ProjectileMovementComponent|SetHomingAccelerationMagnitude (Variables|Default|GetProjectileMovement) 2e+03)
  (|CallParentFunction))