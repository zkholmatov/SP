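; Base enemy area-of-effect actor that detects pawns within a sphere around itself when triggered.
; TriggerSpawn calls SpawnAOESphere, which draws a debug sphere and runs a one-shot overlap query at the actor's location, ignoring the instigator.
; Each pawn found is broadcast through OnAOEOverlap, and this Blueprint applies no damage or effect itself.
; BeginPlay is empty and the delayed-spawn timer is disconnected, so detection relies on an external trigger.
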(event Custom|SpawnAOESphere
  (Rendering|Debug|DrawDebugSphere (Transformation|GetActorLocation) (Variables|Default|GetSphere%20Radius) 12 "(R=0.204356,G=0.104106,B=1.000000,A=1.000000)" 2.0 3.0)
  (bind _outactors (Collision|SphereOverlapActors (Transformation|GetActorLocation) (Variables|Default|GetSphere%20Radius) (Utilities|Array|MakeArray "ObjectTypeQuery3") 0 (Utilities|Array|MakeArray (Game|GetInstigator))))
  (for _array_element _outactors
    (Default|CallOnAOEOverlap _array_element)))

(event Custom|TriggerSpawn
  (CallFunction|SpawnAOESphere))

(event EventBeginPlay)

(event Collision|EventActorBeginOverlap
  (params (OtherActor :type Actor%20Object%20Reference)))

(event EventTick
  (params (DeltaSeconds :type Float%20%28single-precision%29)))

(fn ConstructionScript)