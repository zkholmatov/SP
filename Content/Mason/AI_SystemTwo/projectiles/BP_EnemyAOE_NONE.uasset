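; BP_EnemyAOE_NONE is an enemy area-of-effect Blueprint that defers sphere spawning to its parent and handles the blast visual.
; SpawnBlast attaches the particle emitter to its root, passing player 0's location, or destroys the actor after a short delay if no template is valid.
; The Niagara spawn and the binding for destroy-on-finish are unconnected, so the emitter path never destroys the actor here.
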(event Custom|OnSystemFinished_Event
  (params (PSystem :type Particle%20System%20Component%20Object%20Reference))
  (Actor|DestroyActor))

(event Custom|Spawn%20Blast
  (bind _emitter_template (Variables|Default|GetEmitter%20Template)
    (:then
      (bind _returnvalue (Effects|SpawnEmitterAttached _emitter_template (Variables|Default|GetDefaultSceneRoot) "None" (Transformation|GetActorLocation (Game|GetPlayerCharacter 0)))))
    (:else
      (Utilities|FlowControl|Delay 0.2)
      (Actor|DestroyActor))))

(event EventBeginPlay
  (|CallParentFunction) ; This node is disabled and will not be called.\nDrag off pins to build functionality.
)

(event Collision|EventActorBeginOverlap
  (params (OtherActor :type Actor%20Object%20Reference))
  (|CallParentFunction OtherActor) ; This node is disabled and will not be called.\nDrag off pins to build functionality.
)

(event EventTick
  (params (DeltaSeconds :type Float%20%28single-precision%29))
  (|CallParentFunction DeltaSeconds) ; This node is disabled and will not be called.\nDrag off pins to build functionality.
)

(event EventSpawnAOESphere
  (|CallParentFunction))

(fn ConstructionScript
  (|CallParentFunction))