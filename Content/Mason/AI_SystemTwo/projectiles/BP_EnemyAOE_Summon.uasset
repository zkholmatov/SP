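; Enemy AOE summon attack that marks the player's position with a Niagara circle and light, then spawns skull projectiles there.
; BeginPlay captures the player's location once, waits, then starts a self-recalling delayed loop that spawns homing BP_SummonSkull1 projectiles at short intervals up to a maximum count.
; Speed, damage and decay time pass to each skull.
; After a further delay, the circle, light and root component are destroyed.
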(event Custom|DelayedSpawnLoop
  ;[1 0.1098 0.2627] Recursivley spawn projectiles
  (if (> (Variables|Default|GetMax%20Num%20of%20projectiles) (Variables|Default|GetCurrent%20Num%20of%20projectiles))
    (Variables|Default|SetHomingToggle true)
    (CallFunction|SpawnManyProjectiles (Variables|Default|GetPlayer%20location) (Variables|Default|GetMax%20Speed) (Variables|Default|GetInitial%20Speed) (Variables|Default|GetHomingToggle))
    (Math|Integer|IncrementInt (Variables|Default|GetCurrent%20Num%20of%20projectiles)
      (:%20%20
        (Variables|Default|SetHomingToggle false)
        (Utilities|FlowControl|Delay 0.2)
        (CallFunction|DelayedSpawnLoop)))))

(event EventBeginPlay
  ;[0.2083 0.5692 1] Spawn AOE area then spawn projectiles
  (|CallParentFunction)
  (Variables|Default|SetProjectile%20Damage (Variables|Default|GetProjectile%20Damage))
  (Variables|Default|SetPlayer%20location (Transformation|GetActorLocation (Game|GetPlayerCharacter 0)))
  ;;[0.1302 0.1302 0.1302] Spawn summon circle
  (bind _returnvalue (Niagara|SpawnSystematLocation "/Game/StylizedVFXMagicPack/VFX/MagicCircleVFX/NS_TP-Circle_05.NS_TP-Circle_05" (- (Variables|Default|GetPlayer%20location) "0.000000,0.000000,80.000000")))
  (bind _returnvalue_2 (Game|SpawnActorfromClass "/Game/Mason/AI_SystemTwo/BP_CustomLight.BP_CustomLight_C" (Math|Conversions|ToTransform(Vector) (- (Variables|Default|GetPlayer%20location) "0.000000,0.000000,80.000000")) "Undefined" "MultiplyWithRoot" 0 0))
  (Utilities|FlowControl|Delay (Variables|Default|GetDelay%20Before%20summon))
  ;;[1 0.1098 0.2627] Spawn projectiles
  (CallFunction|DelayedSpawnLoop)
  (Utilities|IsValid _returnvalue
    (:Is%20Valid
      (Utilities|FlowControl|Delay (Variables|Default|GetDelay%20before%20destroy%20))
      (Components|DestroyComponent _returnvalue)
      (Actor|DestroyActor _returnvalue_2)
      (Components|DestroyComponent (Variables|Default|GetDefaultSceneRoot)))))

(event Collision|EventActorBeginOverlap
  (params (OtherActor :type Actor%20Object%20Reference))
  (|CallParentFunction OtherActor) ; This node is disabled and will not be called.\nDrag off pins to build functionality.
)

(fn ConstructionScript
  (|CallParentFunction))

(fn SpawnManyProjectiles
  (params (Actor%20location :type Vector) (Max%20Speed :type Float%20%28double-precision%29) (initial%20Speed :type Float%20%28double-precision%29) (is%20homing :type Boolean))
  (Game|SpawnActorfromClass "/Game/Mason/AI_SystemTwo/projectiles/new/BP_SummonSkull1.BP_SummonSkull1_C" (Math|Conversions|ToTransform(Vector) Actor%20location) "Undefined" "MultiplyWithRoot" 0 initial%20Speed Max%20Speed is%20homing (Variables|Default|GetProjectile%20Damage) (Variables|Default|GetDecay%20Time) 0))