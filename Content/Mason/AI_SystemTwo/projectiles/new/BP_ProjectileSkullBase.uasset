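; Base skull projectile that launches at the player and deals parryable damage on contact.
; On BeginPlay it aims velocity at the player's position and starts a decay timer that ends in an impact effect and destruction.
; The construction script applies speed settings and optional homing toward BP_Player's root component.
; Player overlap sends damage by message, plays impact VFX and sound, then destroys it; other overlaps are ignored.
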(event OnComponentBeginOverlap(SphereCollider)
  (params (OverlappedComponent :type Primitive%20Component%20Object%20Reference) (OtherActor :type Actor%20Object%20Reference) (OtherComp :type Primitive%20Component%20Object%20Reference) (OtherBodyIndex :type Integer) (bFromSweep :type Boolean) (SweepResult :type Hit%20Result%20Structure%20%28by%20ref%29))
  (bind _returnvalue (Transformation|GetActorLocation OtherActor))
  (if (and (== OtherActor (Game|GetPlayerCharacter 0)) (!= OtherActor self))
    (Class|BPIDamageable|TakeDamage(Message) OtherActor (Utilities|Struct|MakeS_DamageInfo (Variables|Default|GetProjectileDamage) "NewEnumerator1" "NewEnumerator3" true false "NewEnumerator0" self "/Game/Zak/AbyssalWarden/BP_Projectile.BP_Projectile_C"))
    (Niagara|SpawnSystematLocation "/Game/SciFi_Impacts/FX/NS_Energy_Impact_9.NS_Energy_Impact_9" _returnvalue)
    (Audio|PlaySoundatLocation "/Game/AmbientMusic/Sounds/Magic/MagicImpact.MagicImpact" _returnvalue "0, 0, 0" 0.3 1.0 0.0 0 0 0 0)
    (Class|BPIDamageable|GetCurrentHealth(Message) OtherActor)
    (Actor|DestroyActor)
    (elif (not true)
      (Development|PrintString "Hello")
      (Actor|DestroyActor))))

(event Custom|RotateToTarget
  (Variables|/Script/Engine.MovementComponent|SetVelocity (Variables|Default|GetProjectileMovement) (* (Math|Vector|GetUnitDirection(Vector) (Transformation|GetActorLocation) (Transformation|GetActorLocation (Game|GetPlayerCharacter 0))) (Variables|Default|GetInitial%20Speed))))

(event Custom|destroy
  (Niagara|SpawnSystematLocation "/Game/SciFi_Impacts/FX/NS_Energy_Impact_9.NS_Energy_Impact_9" (Transformation|GetActorLocation))
  (Actor|DestroyActor))

(event EventBeginPlay
  (CallFunction|RotatetoTarget)
  (Variables|Default|SetProjectileDeathTimer 2.0)
  (Utilities|Time|SetTimerbyEvent (delegate Custom|destroy) (Variables|Default|GetDecayTime)))

(event EventRestart
  (Actor|DestroyActor))

(fn ConstructionScript
  (bind _bishoming (Variables|Default|GetbIsHoming))
  (bind _projectilemovement (Variables|Default|GetProjectileMovement))
  (Variables|/Script/Engine.ProjectileMovementComponent|SetInitialSpeed _projectilemovement (Variables|Default|GetInitial%20Speed))
  (Variables|/Script/Engine.ProjectileMovementComponent|SetMaxSpeed _projectilemovement (Variables|Default|GetMax%20Speed))
  (if _bishoming
    (Variables|/Script/Engine.ProjectileMovementComponent|SetbIsHomingProjectile _projectilemovement _bishoming)
    (bind _returnvalue (Actor|GetActorOfClass "/Game/Zak/BP_Player.BP_Player_C"))
    (Variables|/Script/Engine.ProjectileMovementComponent|SetHomingTargetComponent _projectilemovement (Variables|/Script/Engine.Actor|GetRootComponent _returnvalue))
    (Variables|/Script/Engine.ProjectileMovementComponent|SetHomingAccelerationMagnitude _projectilemovement 3e+03)))