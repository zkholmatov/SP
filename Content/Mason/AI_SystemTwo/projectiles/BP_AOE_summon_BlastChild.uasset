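; AOE summon attack that marks the player's position with a Niagara effect, then releases a burst of summoned skull projectiles from that spot.
; BeginPlay captures the player's location, places the effect just below it, waits, starts the spawn loop and later destroys the effect.
; A self-calling delayed event spawns BP_SummonSkull actors in quick succession up to a maximum, passing speed settings and alternating homing by count parity.
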(event Custom|DelayedSpawnLoop
  ;[1 0.1098 0.2627] Recursivley spawn projectiles
  (if (> (Variables|Default|GetMax%20Num%20of%20projectiles) (Variables|Default|GetCurrent%20Num%20of%20projectiles))
    (CallFunction|SpawnManyProjectiles (Variables|Default|GetPlayer%20location) (Variables|Default|GetMax%20Speed) (Variables|Default|GetInitial%20Speed) (Variables|Default|GetHomingToggle))
    (if (== (Math|Integer|%(Integer) (Variables|Default|GetCurrent%20Num%20of%20projectiles) 2) 0)
      (Variables|Default|SetHomingToggle true)
      (else
        (Variables|Default|SetHomingToggle false)))
    (Math|Integer|IncrementInt (Variables|Default|GetCurrent%20Num%20of%20projectiles)
      (:%20%20
        (Utilities|FlowControl|Delay 0.05)
        (CallFunction|DelayedSpawnLoop)))))

(event EventBeginPlay
  ;[0.2083 0.5692 1] Spawn AOE area then spawn projectiles
  (|CallParentFunction)
  (Variables|Default|SetPlayer%20location (Transformation|GetActorLocation (Game|GetPlayerCharacter 0)))
  (bind _returnvalue (Niagara|SpawnSystematLocation "/Game/Mason/AI_SystemTwo/NiagaraMage1.NiagaraMage1" (- (Variables|Default|GetPlayer%20location) "0.000000,0.000000,80.000000")))
  (Utilities|FlowControl|Delay (Variables|Default|GetDelay%20Before%20summon))
  ;;[1 0.1098 0.2627] Spawn projectiles
  (CallFunction|DelayedSpawnLoop)
  (Utilities|IsValid _returnvalue
    (:Is%20Valid
      (Utilities|FlowControl|Delay (Variables|Default|GetDelay%20before%20destroy%20))
      (Components|DestroyComponent _returnvalue))))

(event Collision|EventActorBeginOverlap
  (params (OtherActor :type Actor%20Object%20Reference))
  (|CallParentFunction OtherActor) ; This node is disabled and will not be called.\nDrag off pins to build functionality.
)

(event EventTick
  (params (DeltaSeconds :type Float%20%28single-precision%29))
  (|CallParentFunction DeltaSeconds))

(fn ConstructionScript
  (|CallParentFunction))

(fn SpawnManyProjectiles
  (params (Actor%20location :type Vector) (Max%20Speed :type Float%20%28double-precision%29) (initial%20Speed :type Float%20%28double-precision%29) (is%20homing :type Boolean))
  (Game|SpawnActorfromClass "/Game/Mason/AI_SystemTwo/projectiles/BP_SummonSkull.BP_SummonSkull_C" (Math|Conversions|ToTransform(Vector) Actor%20location) "Undefined" "MultiplyWithRoot" 0 Max%20Speed initial%20Speed is%20homing 0))