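; BP_EnemyMage is a mage enemy built on a C++ enemy class that carries a staff and fights with ranged projectile attacks.
; A projectile notify from C++ spawns a skull projectile at the staff's TrailEnd socket.
; A summon notify spawns an AOE summon at the player's location when CanSummon is set, otherwise falls back to the skull shot.
; Overrides supply the staff class, its socket and attack ranges.
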(event Custom|spawnProjectile
  ;[1 0.07926 0.7768] Range Attack
  (Game|SpawnActorfromClass "/Game/Mason/AI_SystemTwo/projectiles/BP_ProjectileSkull.BP_ProjectileSkull_C" (Math|Conversions|ToTransform(Vector) (Transformation|GetSocketLocation (Variables|/Game/Zak/Weapons/BP_Weapon.BP_Weapon_C|GetWeapon (Variables|Default|GetBP_Weapon_var)) "TrailEnd")) "Undefined" "MultiplyWithRoot" 0 (Variables|EnemyStats|GetMaxProjectileSpeed) (Variables|EnemyStats|GetProjectileStartSpeed) false 0) ; Damage Set in Class Construction
)

(event Custom|FireProjectileTwo
  ;[1 0.07926 0.7768] Range Attack
  (if (Variables|Default|GetCanSummon)
    (CallFunction|SummonProjectiles)
    (else
      (CallFunction|SpawnProjectile))))

(event Custom|SummonProjectiles
  ;[1 0.07926 0.7768] Range Attack
  (Game|SpawnActorfromClass "/Game/Mason/AI_SystemTwo/projectiles/BP_EnemyAOE_Summon.BP_EnemyAOE_Summon_C" (Math|Conversions|ToTransform(Vector) (Transformation|GetActorLocation (Game|GetPlayerCharacter 0))) "Undefined" "MultiplyWithRoot" 0 2.0 5.0 (Variables|EnemyStats|GetMax%20Summoned%20Projectile%20Speed) (Variables|EnemyStats|GetInitial%20Summoned%20Projectile%20Speed) 0) ; Damage Set in Class Construction
)

(event EventBeginPlay
  (Variables|Default|SetEnemyMaxHealth (Variables|Default|GetEnemyMaxHealth))
  (Variables|Default|SetWeaponDamage (Variables|Default|GetWeaponDamage))
  (Variables|Default|SetTraceColliderRadius 15.0)
  (|CallParentFunction))

(event Collision|EventActorBeginOverlap
  (params (OtherActor :type Actor%20Object%20Reference)))

(event EventMyFireProjectileEvent
  ;[1 0.07926 0.7768] Range Attack
  ;;[1 1 1] Spawn Projectile is notify info
  (CallFunction|SpawnProjectile))

(fn ConstructionScript
  (|CallParentFunction))

(fn SetWeaponSetSocket
  (Variables|Default|SetWeapon%20Socket%20Name "StaffSocket")
  (bind _output_get (Variables|Default|SetWeaponClass "/Game/Mason/AI_SystemTwo/weapon_BluePrints/BP_MageStaff.BP_MageStaff_C"))
  (return _output_get))

(fn GetPatrolRoute
  (return 0))

(fn GetIdealRange
  (return 5e+02 0.0 1.5e+03 2e+03))