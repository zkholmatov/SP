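; Base melee enemy character that equips a child-overridable weapon (great axe by default) and runs combat AI through blackboard state.
; BPC damage system events drive directional hit reactions and death with ragdoll and portal.
; Timer-looped sphere traces between weapon sockets damage only the player, with parries staggering the enemy.
; It also provides health bar, target lock marker, randomized speed, execution with fracture, and respawn reset.
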(event Custom|CanBeExecuted_1_1
  ;[0.3843 0.4745 1] Execution
)

(event Custom|DamageResponse
  (params (DamageResponse :type E_DamageResponse%20Enum :default "NewEnumerator0") (DamageDirection :type E_DamageDirection%20Enum :default "NewEnumerator0") (DamageCauser :type Actor%20Object%20Reference))
  ;[0.3843 0.4745 1] DamageResponse / stunned
  (if true
    (AI|Components|Blackboard|SetValueasBool (AI|GetBlackboard (AI|GetAIController self)) (Variables|Default|GetBlackBoardKeyName) true) ; set black baord decorator bIsStaggered to true for BT to adjust behavior path
    (Variables|Stagger|SetLastDamageTime (Utilities|Time|GetGameTimeinSeconds)) ; reset time since last damage stimuli
    (Components|Movement|StopMovementImmediately (Variables|Character|GetCharacterMovement)) ; Stop movement of enemy before queuing animation for stagger
    (bind _hitreactionmontage (CallFunction|SetHitReactionMontage DamageDirection))
    (Animation|Montage|PlayMontage (Variables|Character|GetMesh) _hitreactionmontage 0.5
      (:OnCompleted
        _)
      (:OnBlendOut
        _)
      (:OnInterrupted
        _))
    (AI|Components|Blackboard|SetValueasBool (AI|GetBlackboard (AI|GetAIController self)) (Variables|Default|GetBlackBoardKeyName) false) ; reset value of is staggered to false
    (Class|AISenseDamage|ReportDamageEvent self (Game|GetPlayerCharacter 0) 0.0 (Transformation|GetActorLocation) "0, 0, 0" "None") ; Report damage event to AI controller assocaited with enemy
  ))

(event Custom|CheckIfExecutableLoop
  ;[0.3843 0.4745 1] Execution
)

(event Custom|ChangeToRandomSpeed
  ;[0.3843 0.4745 1] Event begin play
  (bind _output_get (Variables|/Script/Engine.CharacterMovementComponent|SetMaxWalkSpeed (Variables|Character|GetCharacterMovement) (Math|Random|RandomFloatinRange (Variables|EnemyStats|GetMinRandSpeed) (Variables|EnemyStats|GetMaxRandSpeed))))
  (AI|Components|Blackboard|SetValueasFloat (AI|GetBlackboard 0) (Variables|Default|GetOriginalSpeed) _output_get) ; this is set in aic on sight
)

(event Custom|LockLoop
  (bind _targetlockwidget (Variables|Default|GetTargetLockWidget))
  (bind _mesh (Variables|Character|GetMesh))
  (bind _targetlockwidget_2 (Variables|/Game/Zak/UI/BP_TargetLock.BP_TargetLock_C|GetTargetLockWidget _targetlockwidget))
  ;[0.3843 0.4745 1] For target lock
  (Utilities|IsValid _targetlockwidget_2
    (:Is%20Valid
      (Utilities|IsValid _mesh
        (:Is%20Valid
          (Transformation|SetWorldLocation _targetlockwidget_2 (Transformation|GetSocketLocation _mesh "Spine_03") false false))))))

(event Custom|Death
  ;[0.3843 0.4745 1] Death
)

(event Custom|SwordTraceLoop
  ;[1 0.4849 0.4351 1 30] Trace + apply damage
  (bind (_start _end) (CallFunction|SetSocketLocation))
  (bind (_outhit _returnvalue) (Collision|SphereTraceForObjects _start _end (Variables|EnemyStats|GetTraceColliderRadius) (Utilities|Array|MakeArray "ObjectTypeQuery4") false 0 "None" true "(R=1.000000,G=0.045752,B=0.620198,A=1.000000)" "(R=0.000000,G=1.000000,B=0.000000,A=1.000000)" 2.0))
  (if _returnvalue
    (Utilities|FlowControl|DoOnce false :!label _label
      (:Completed
        ;;[1 1 1] enemies cant attack eachother
        (if (== (Game|GetPlayerCharacter 0) (.HitActor (Collision|BreakHitResult _outhit)))
          (bind _wasparried_ (Class|BPIDamageable|TakeDamage(Message) (.HitActor (Collision|BreakHitResult _outhit)) (Utilities|Struct|MakeS_DamageInfo (Variables|EnemyStats|GetWeaponDamage) "NewEnumerator1" "NewEnumerator3" (not (Variables|EnemyStats|GetbNotParriable)) false (CallFunction|CalculateDamageDirection self (.HitActor (Collision|BreakHitResult _outhit))) self)))
          (Class|BPIDamageable|GetCurrentHealth(Message) (.HitActor (Collision|BreakHitResult _outhit)))
          (if _wasparried_
            (AI|Components|Blackboard|SetValueasBool (AI|GetBlackboard (AI|GetAIController self)) (Variables|Default|GetBlackBoardKeyName) true)
            (Class|MyEnemy|MySwordTraceStopEvent)
            (bind _hitreactionmontage (CallFunction|SetHitReactionMontage "NewEnumerator0"))
            (Animation|Montage|PlayMontage (Variables|Character|GetMesh) _hitreactionmontage
              (:OnCompleted
                _)
              (:OnInterrupted
                _))
            (AI|Components|Blackboard|SetValueasBool (AI|GetBlackboard (AI|GetAIController self)) (Variables|Default|GetBlackBoardKeyName) false)
            (else
              (Class|MyEnemy|MySwordTraceStopEvent))))))
    (else
      (goto _label Reset))))

(event Custom|OnDead
  ;[0.3843 0.4745 1] Death
  (bind _asaic_cpp_enemy_base (Utilities|Casting|CastToAIC_CPP_EnemyBase (AI|GetAIController self)))
  (Class|AIPerceptionComponent|SetSenseEnabled (Variables|/Script/Githubtest.AIController_CPP|GetCppPerceptionComponent _asaic_cpp_enemy_base) "/Script/AIModule.AISense_Sight" false)
  (AI|Logic|StopLogic (Variables|/Script/AIModule.AIController|GetBrainComponent _asaic_cpp_enemy_base) "")
  (AI|Components|Blackboard|SetValueasEnum (AI|GetBlackboard 0) (Variables|Default|GetCurrent%20State) (Utilities|Enum|LiteralenumEnumEnemyState "Death"))
  (Components|DestroyComponent (Variables|Default|GetHealthBar))
  (Components|DestroyComponent (Variables|Default|GetCapsuleComponent))
  (bind _ref_to_portal (CallFunction|DeathExtend))
  (Utilities|FlowControl|Delay (Variables|Default|GetDeathDelay))
  (CallFunction|DestroyActors _ref_to_portal))

(event Custom|ExecuteAnim
  ;[1 1 1] Execute - zak
  (Variables|/Game/Zak/DamageSystem/BPC_DamageSystem.BPC_DamageSystem_C|SetInvincible? (Variables|Default|GetBPC_DamageSystem) true)
  (Default|CallOnExecuted)
  (Animation|Montage|PlayMontage (Variables|Character|GetMesh) (Utilities|Select :Index (Variables|Default|GetExecutionSequence) :Option%200 "/Game/Great_Sword/Animations/Sequence2/02_Attack/15_Execution/02_Target/AS_Execution_Target_03_Seq_Montage.AS_Execution_Target_03_Seq_Montage" :Option%201 "/Game/Sword_Animations/Animations/Sequence2/02_Attack/15_Execution/02_Target/Execution_Target_02_Seq_Montage.Execution_Target_02_Seq_Montage" :Option%202 "/Game/Dual_Sword/Animations/Sequence2/02_Attack/16_Exeution/02_Target/AS_Exeution_Target_02_Seq_Montage.AS_Exeution_Target_02_Seq_Montage") 0.7))

(event Custom|ChangeToIdle
  ;[0.3843 0.4745 1] Event begin play
  (Variables|/Script/Engine.CharacterMovementComponent|SetMaxWalkSpeed (Variables|Character|GetCharacterMovement) (Variables|EnemyStats|GetIdleWalkSpeed)))

(event EventBeginPlay
  (bind _healthbar (Variables|Default|GetHealthBar))
  ;[0.3843 0.4745 1] Event begin play
  (Variables|BehaviorTree|SetBehaviorTree "/Game/Mason/AI_SystemTwo/BT_BB/BT_EnemyCombatBehavior.BT_EnemyCombatBehavior")
  (bind _weapon (CallFunction|WeaponEquip (Variables|Weapon|GetprimaryWeaponSocket))) ; calls interface function
  (Variables|Weapon|SetBP_PrimaryWeapon _weapon)
  (bind _asaic_cpp_enemy_base (Utilities|Casting|CastToAIC_CPP_EnemyBase (AI|GetAIController self)))
  (Variables|Default|SetAIC_CPP_Obj _asaic_cpp_enemy_base)
  (Variables|EnemyStats|SetStaggerTimer 4.0)
  (Variables|/Script/Engine.CharacterMovementComponent|SetMaxWalkSpeed (Variables|Character|GetCharacterMovement) (Variables|EnemyStats|GetIdleWalkSpeed))
  (EventDispatchers|BindEventtoOnDeath (Variables|Default|GetBPC_DamageSystem) (EventDispatchers|CreateEvent :!event Custom|OnDead))
  (Default|SetMaxHealth (Variables|Default|GetBPC_DamageSystem) (Variables|EnemyStats|GetEnemyMaxHealth))
  (Utilities|FlowControl|Sequence
    (:then_0
      ;;[1 0.6059 0.2209] health bar
      (if (not (Variables|Default|GetbIsBoss))
        _
        (else
          _))
      (bind _returnvalue (UserInterface|CreateWidget "/Game/Omar/UI/WidgetBlueprints/WB_HealthBar.WB_HealthBar_C" 0 self))
      (UserInterface|SetWidget _healthbar _returnvalue)
      (Rendering|SetVisibility _healthbar false false)
      (bind _asbp_player (Utilities|Casting|CastToBP_Player (Game|GetPlayerCharacter 0)))
      (Variables|Default|SetAs%20BP%20Player _asbp_player)
      (bind _returnvalue_2 (UserInterface|CreateWidget "/Game/Zak/UI/Wigets/W_Execution.W_Execution_C"))
      (UserInterface|SetWidget (Variables|Default|GetExecuteWidget) _returnvalue_2)
      (EventDispatchers|BindEventtoIdleSpeed (delegate Custom|ChangeToIdle))
      (EventDispatchers|BindEventtoRandomWalkSpeed (delegate Custom|ChangeToRandomSpeed)))
    (:then_1
      (bind _returnvalue_3 (Game|SpawnActorfromClass "/Game/Zak/UI/BP_TargetLock.BP_TargetLock_C" (Math|Transform|MakeTransform (Transformation|GetSocketLocation (Variables|Character|GetMesh) "Spine_03") "0, 0, 0" "1.000000,1.000000,1.000000") "Undefined" "MultiplyWithRoot" 0 0))
      (Variables|Default|SetTargetLockWidget _returnvalue_3))))

(event EventDisplayHealthBar
  (bind _healthbar (Variables|Default|GetHealthBar))
  ;[0.3843 0.4745 1] Event begin play
  ;;[1 0.6059 0.2209] health bar
  (Utilities|IsValid _healthbar
    (:Is%20Valid
      (Rendering|SetVisibility _healthbar true false))))

(event EventRestart
  ;[1 1 1] Respawn System for enemies - Zak
  (Transformation|SetActorTransform (Variables|Default|GetSpawnTransform) false true)
  (Default|SetMaxHealth (Variables|Default|GetBPC_DamageSystem) (Variables|EnemyStats|GetEnemyMaxHealth))
  (Components|Movement|StopMovementImmediately (Variables|Character|GetCharacterMovement))
  (bind _asaic_cpp_enemy_base (Utilities|Casting|CastToAIC_CPP_EnemyBase (AI|GetAIController self)))
  (Class|AIControllerCPP|SetStateasIdle _asaic_cpp_enemy_base))

(event EventHideHealthbar
  (bind _healthbar (Variables|Default|GetHealthBar))
  ;[0.3843 0.4745 1] Event begin play
  ;;[1 0.6059 0.2209] health bar
  (Utilities|IsValid _healthbar
    (:Is%20Valid
      (Rendering|SetVisibility _healthbar false false))))

(event EventFracture
  (bind _bp_primaryweapon (Variables|Weapon|GetBP_PrimaryWeapon))
  (bind _weapon (Variables|/Game/Zak/Weapons/BP_Weapon.BP_Weapon_C|GetWeapon _bp_primaryweapon))
  ;[1 1 1] Execute - zak
  (Utilities|FlowControl|Sequence
    (:then_0
      (Components|DestroyComponent (Variables|Character|GetMesh))
      (Components|DestroyComponent (Variables|/Script/Engine.Actor|GetRootComponent (Variables|Weapon|GetBP_PrimaryWeapon)))
      (Game|SpawnActorfromClass "/Game/Zak/Fracture/BP_FractureBase.BP_FractureBase_C" (Transformation|GetActorTransform) "Undefined" "OverrideRootScale" 0 0)
      (Game|SpawnActorfromClass "/Game/Zak/Interractible/FS_Impact.FS_Impact_C" (Transformation|GetActorTransform) "AlwaysSpawn" "MultiplyWithRoot" 0 0)
      (CallFunction|OnDead))
    (:then_1
      (Transformation|DetachFromActor _bp_primaryweapon "KeepWorld" "KeepWorld" "KeepWorld")
      (Collision|SetCollisionEnabled _weapon "QueryAndPhysics")
      (Physics|SetSimulatePhysics _weapon true))))

(event EventMySwordTraceEvent
  ;[1 0.4849 0.4351 1 30] Trace + apply damage
  (bind _returnvalue (Utilities|Time|SetTimerbyEvent (delegate Custom|SwordTraceLoop) 0.01 true))
  (Variables|Default|SetTraceTimerHandle _returnvalue))

(event EventLock
  ;[0.3843 0.4745 1] For target lock
  (Rendering|SetVisibility (Variables|/Game/Zak/UI/BP_TargetLock.BP_TargetLock_C|GetTargetLockWidget (Variables|Default|GetTargetLockWidget)) true false)
  (bind _returnvalue (Utilities|Time|SetTimerbyEvent (delegate Custom|LockLoop) 0.01 true)))

(event EventUnlock
  ;[0.3843 0.4745 1] For target lock
  (Rendering|SetVisibility (Variables|/Game/Zak/UI/BP_TargetLock.BP_TargetLock_C|GetTargetLockWidget (Variables|Default|GetTargetLockWidget)) false false)
  (Utilities|Time|ClearandInvalidateTimerbyHandle (stale EventLock _returnvalue)))

(event EventMySwordTraceStopEvent
  ;[1 0.4849 0.4351 1 30] Trace + apply damage
  (Utilities|Time|ClearandInvalidateTimerbyHandle (Variables|Default|GetTraceTimerHandle)))

(fn ConstructionScript
  (bind _bpc_damagesystem (Variables|Default|GetBPC_DamageSystem))
  (EventDispatchers|BindEventtoOnDeath _bpc_damagesystem (EventDispatchers|CreateEvent :!event Custom|OnDead))
  (EventDispatchers|BindEventtoOnDamageResponse _bpc_damagesystem (EventDispatchers|CreateEvent :!event Custom|DamageResponse)) ; calls event when actor takes damage
  (Variables|Default|SetSpawnTransform (Transformation|GetWorldTransform (Variables|Default|GetCapsuleComponent))))

(fn PredictTrace
  (params (Location :type Vector))
  (bind (_outhit _returnvalue) (Collision|SphereTraceForObjects Location Location 1.5e+02 (Utilities|Array|MakeArray "ObjectTypeQuery3") false 0 "None"))
  (if _returnvalue
    (return (.HitActor (Collision|BreakHitResult _outhit)))
    (else
      (return 0))))

(fn CalculateDamageDirection
  (params (DamageCauser :type Actor%20Object%20Reference) (DamagedActor :type Actor%20Object%20Reference))
  (bind _returnvalue (Transformation|GetActorRotation DamagedActor))
  (bind _returnvalue_2 (Transformation|GetActorLocation DamageCauser))
  (bind _returnvalue_3 (Transformation|GetActorLocation DamagedActor))
  (bind _returnvalue_4 (Math|Rotator|FindLookatRotation _returnvalue_2 _returnvalue_3))
  (bind _returnvalue_5 (Math|Rotator|Delta(Rotator) _returnvalue _returnvalue_4))
  (Utilities|IsValid DamagedActor
    (:Is%20Valid
      (if (or (Math|Float|InRange(Float) (.yaw _returnvalue_5) -1.8e+02 -135.0) (Math|Float|InRange(Float) (.yaw _returnvalue_5) 135.0 1.8e+02))
        (return "NewEnumerator0")
        (elif (Math|Float|InRange(Float) (.yaw _returnvalue_5) 45.0 135.0)
          (return "NewEnumerator2")
          (elif (Math|Float|InRange(Float) (.yaw _returnvalue_5) -135.0 -45.0)
            (return "NewEnumerator1")
            (elif (Math|Float|InRange(Float) (.yaw _returnvalue_5) -45.0 45.0)
              (return "NewEnumerator3"))))))))

(fn SetHitReactionMontage
  (params (NewParam :type E_DamageDirection%20Enum :default "NewEnumerator0"))
  (LocalVariables|SetLocalDamageDirection NewParam)
  (if (Utilities|Enum|Equal(Enum) (LocalVariables|GetLocalDamageDirection) "NewEnumerator0")
    (return "/Game/Mason/AI_SystemTwo/Animations/Reactions/ReactionF_Montage.ReactionF_Montage")
    (elif (Utilities|Enum|Equal(Enum) (LocalVariables|GetLocalDamageDirection) "NewEnumerator1")
      (return "/Game/Mason/AI_SystemTwo/Animations/Reactions/ReactionL_Montage.ReactionL_Montage")
      (elif (Utilities|Enum|Equal(Enum) (LocalVariables|GetLocalDamageDirection) "NewEnumerator2")
        (return "/Game/Mason/AI_SystemTwo/Animations/Reactions/ReactionR_Montage.ReactionR_Montage")
        (elif (Utilities|Enum|Equal(Enum) (LocalVariables|GetLocalDamageDirection) "NewEnumerator3")
          (return "/Game/Mason/AI_SystemTwo/Animations/Reactions/ReactionB_Montage.ReactionB_Montage"))))))

(fn WithinExecutionThreshold
  (bind _maxhealth (CallFunction|GetMaxHealth))
  (bind _health (CallFunction|GetCurrentHealth))
  (bind _isdead_ (CallFunction|IsDead))
  (if (and (not _isdead_) (<= (/ _health _maxhealth) (Variables|EnemyStats|GetExecutionHealth)))
    (return true)
    (else
      (return false))))

(fn WeaponEquip
  (params (Socket :type Name%20%28by%20ref%29))
  (bind _weaponclass (CallFunction|SetWeaponSetSocket :!pinned true)) ; redefined in each child
  (bind _returnvalue (Game|SpawnActorfromClass _weaponclass (Transformation|GetActorTransform) "AlwaysSpawn" "MultiplyWithRoot" 0 0))
  (bind _output_get (LocalVariables|Settempweapon _returnvalue)) ; idk why error
  (Transformation|AttachComponentToComponent _output_get (Variables|Character|GetMesh) Socket "SnapToTarget" "SnapToTarget" "SnapToTarget" true)
  (return (LocalVariables|Gettempweapon)))

(fn SetSocketLocation
  (bind _bp_primaryweapon (Variables|Weapon|GetBP_PrimaryWeapon))
  (bind _bp_thirdweapon (Variables|Weapon|GetBP_ThirdWeapon))
  (bind _bp_secondaryweapon (Variables|Weapon|GetBP_SecondaryWeapon))
  (bind _weapon (Variables|/Game/Zak/Weapons/BP_Weapon.BP_Weapon_C|GetWeapon _bp_thirdweapon))
  (bind _weapon_2 (Variables|/Game/Zak/Weapons/BP_Weapon.BP_Weapon_C|GetWeapon _bp_primaryweapon))
  (bind _weapon_3 (Variables|/Game/Zak/Weapons/BP_Weapon.BP_Weapon_C|GetWeapon _bp_secondaryweapon))
  ;[1 1 1] This is set up with notifies that need to placed inside of montages. There is a begin notify which sets value and socket, then the end notify which toggles to false
  (if (Variables|Weapon|GetPrimary)
    (return (Transformation|GetSocketLocation _weapon_2 "TrailStart") (Transformation|GetSocketLocation _weapon_2 "TrailEnd"))
    (elif (Variables|Weapon|GetSecondary)
      (return (Transformation|GetSocketLocation _weapon_3 "TrailStart") (Transformation|GetSocketLocation _weapon_3 "TrailEnd"))
      (elif (Variables|Weapon|GetThird)
        (return (Transformation|GetSocketLocation _weapon "TrailStart") (Transformation|GetSocketLocation _weapon "TrailEnd"))
        (else
          (Development|PrintString "No bp weapon ref" true true "(R=0.000000,G=0.660000,B=1.000000,A=1.000000)" 5.0))))))

(fn DeathExtend
  (bind _self self)
  (bind _mesh (Variables|Character|GetMesh))
  (bind _returnvalue (Transformation|GetActorLocation _self))
  (bind _mesh_2 (Variables|Character|GetMesh _self))
  (bind _returnvalue_2 (Transformation|GetSocketTransform _mesh_2 "pelvis" "RTS_World"))
  (Utilities|IsValid _mesh
    (:Is%20Valid
      (Physics|SetSimulatePhysics _mesh true)
      (bind _returnvalue_3 (Game|SpawnActorfromClass "/Game/Mason/AI_SystemTwo/BP_DeathPortal.BP_DeathPortal_C" (Math|Transform|MakeTransform (Math|Vector|MakeVector (.x _returnvalue) (.y _returnvalue) (+ (- 0.0 (- (.z _returnvalue) (Components|Capsule|GetScaledCapsuleHalfHeight (Variables|/Script/Engine.Character|GetCapsuleComponent _self)))) 3e+01)) (Math|Rotator|MakeRotator 0.0 0.0 (.yaw (.rotation _returnvalue_2))) (.scale _returnvalue_2)) "AdjustIfPossibleButAlwaysSpawn" "MultiplyWithRoot" 0 0))
      (AI|Components|Blackboard|SetValueasEnum (AI|GetBlackboard 0) (Variables|Default|GetCurrent%20State) (Utilities|Enum|LiteralenumEnumEnemyState "Death"))
      (return _returnvalue_3))))

(fn DestroyActors
  (params (ref%20to%20portal%20 :type BP%20Death%20Portal%20Object%20Reference))
  (Components|DestroyComponent (Variables|Character|GetMesh))
  (Collision|SetCollisionEnabled (Variables|Default|GetCapsuleComponent) "NoCollision")
  (Actor|DestroyActor ref%20to%20portal%20)
  (Components|DestroyComponent (Variables|/Script/Engine.Actor|GetRootComponent (Variables|Weapon|GetBP_PrimaryWeapon)))
  (Actor|DestroyActor))

(fn GetCurrentHealth
  (bind _bpc_damagesystem (Variables|Default|GetBPC_DamageSystem))
  (Utilities|IsValid _bpc_damagesystem
    (:Is%20Valid
      (return (Variables|/Game/Zak/DamageSystem/BPC_DamageSystem.BPC_DamageSystem_C|GetHealth _bpc_damagesystem)))))

(fn GetIdealRange
  (return 2e+02 5e+02 4e+02 7e+02 0.0))

(fn GetMaxHealth
  (bind _bpc_damagesystem (Variables|Default|GetBPC_DamageSystem))
  (Utilities|IsValid _bpc_damagesystem
    (:Is%20Valid
      (return (Variables|/Game/Zak/DamageSystem/BPC_DamageSystem.BPC_DamageSystem_C|GetMaxHealth _bpc_damagesystem)))))

(fn GetPatrolRoute
  (return (Variables|Default|GetPatrolRoute)))

(fn Heal
  (params (Amount :type Float%20%28double-precision%29))
  (return 0.0))

(fn IsAttacking
  (return false))

(fn IsDead
  (return (Variables|/Game/Zak/DamageSystem/BPC_DamageSystem.BPC_DamageSystem_C|GetDead? (Variables|Default|GetBPC_DamageSystem))))

(fn IsInvincible
  (return false))

(fn SetWeaponSetSocket
  (Variables|Weapon|SetprimaryWeaponSocket "AxeSocket")
  (bind _output_get (Variables|EnemyStats|SetWeaponClass "/Game/Mason/AI_SystemTwo/weapon_BluePrints/BP_GreatAxe.BP_GreatAxe_C"))
  (return _output_get))

(fn TakeDamage
  (params (DamageInfo :type S%20Damage%20Info%20Structure))
  ;[1 1 1] Comment
  (bind (_wasdamaged_ _damageamount _wasparried_) (Default|TakeDamage (Variables|Default|GetBPC_DamageSystem) DamageInfo))
  (if _wasdamaged_
    (Camera|PlayWorldCameraShake "/Game/Zak/VFX/BP_HitCameraShake.BP_HitCameraShake_C" (Transformation|GetActorLocation) 0.0 5e+02)
    (return true _damageamount false 0.0)
    (elif _wasparried_
      (return false 0.0 true 0.0))))