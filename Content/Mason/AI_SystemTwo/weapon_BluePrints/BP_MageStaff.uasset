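; BP_MageStaff is a weapon Blueprint for a mage's staff, tied to the "WoodenStaff" data table row.
; On BeginPlay it sets that row name, calls the parent, then fills inherited-style settings for animation set, greatsword socket, four-montage light combo, stamina cost, trace radius, charge accumulation and replenish amounts.
; It holds only configuration, with no combat logic of its own.
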(event EventBeginPlay
  (Variables|Default|SetDataTableRowName "WoodenStaff")
  (|CallParentFunction)
  (Variables|Default|SetAnimationSet 0)
  (Variables|Default|SetSocketName "GreatswordSocket_0")
  (Variables|Default|SetAttackCombo (Utilities|Array|MakeArray "/Game/Zak/Player/AnimGreatsword/AttackCombo1/AS_Combo_Attack_01_01_Seq_Montage.AS_Combo_Attack_01_01_Seq_Montage" "/Game/Zak/Player/AnimGreatsword/AttackCombo1/AS_Combo_Attack_01_02_Seq_Montage.AS_Combo_Attack_01_02_Seq_Montage" "/Game/Zak/Player/AnimGreatsword/AttackCombo1/AS_Combo_Attack_01_03_Seq_Montage.AS_Combo_Attack_01_03_Seq_Montage" "/Game/Zak/Player/AnimGreatsword/AttackCombo1/AS_Combo_Attack_01_04_Seq_Montage.AS_Combo_Attack_01_04_Seq_Montage"))
  (Variables|Default|SetLightAttackStaminaCost 15.0)
  (Variables|Default|SetTraceRadius 25.0)
  (Variables|Default|SetChargeAccumulationMultiplier (Utilities|Array|MakeArray 0.3 0.35 0.3 0.5 0.5))
  (Variables|Default|SetReplenishAmount (Utilities|Array|MakeArray 0.125 0.13 0.12 0.14 0.25)))

(event Collision|EventActorBeginOverlap
  (params (OtherActor :type Actor%20Object%20Reference)))

(event EventTick
  (params (DeltaSeconds :type Float%20%28single-precision%29)))

(fn ConstructionScript
  (|CallParentFunction))