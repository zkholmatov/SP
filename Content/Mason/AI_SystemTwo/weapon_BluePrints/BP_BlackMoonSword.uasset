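; Black Moon Sword weapon Blueprint, a data-only style child of a parent weapon class, keyed to the MiniBossSword data table row.
; BeginPlay sets the row name before calling the parent, then assigns animation set, attach socket, four-montage attack combo, light attack stamina cost, trace radius, and charge and replenish arrays.
; It adds no behavior of its own: Tick and overlap are disabled, and the construction script only calls the parent.
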(event EventBeginPlay
  (Variables|Default|SetDataTableRowName "MiniBossSword")
  (|CallParentFunction)
  (Variables|Default|SetAnimationSet 1)
  (Variables|Default|SetSocketName "SwordSocket_0")
  (Variables|Default|SetAttackCombo (Utilities|Array|MakeArray "/Game/Zak/Player/AnimSword/AttackCombo4/Combo_Attack_04_01_Seq1_Montage.Combo_Attack_04_01_Seq1_Montage" "/Game/Zak/Player/AnimSword/AttackCombo4/Combo_Attack_04_02_Seq1_Montage.Combo_Attack_04_02_Seq1_Montage" "/Game/Zak/Player/AnimSword/AttackCombo4/Combo_Attack_04_03_Seq_Montage.Combo_Attack_04_03_Seq_Montage" "/Game/Zak/Player/AnimSword/AttackCombo4/Combo_Attack_04_04_Seq_Montage.Combo_Attack_04_04_Seq_Montage"))
  (Variables|Default|SetLightAttackStaminaCost 1e+01)
  (Variables|Default|SetTraceRadius 15.0)
  (Variables|Default|SetChargeAccumulationMultiplier (Utilities|Array|MakeArray 0.2 0.25 0.3 0.2 0.5))
  (Variables|Default|SetReplenishAmount (Utilities|Array|MakeArray 0.075 0.08 0.085 0.1 0.25)))

(event Collision|EventActorBeginOverlap
  (params (OtherActor :type Actor%20Object%20Reference)))

(event EventTick
  (params (DeltaSeconds :type Float%20%28single-precision%29)))

(fn ConstructionScript
  (|CallParentFunction))