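; Skull projectile that launches toward the player on spawn and deals parryable damage to actors it overlaps.
; Construction applies speeds to ProjectileMovement and, if IsHoming is set, targets BP_Player's root for homing.
; Overlaps and hits both fire the collision callback and spawn an emitter, but only overlaps send damage.
; Tick clears IsHoming after a time limit without updating the movement component.
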(event OnComponentBeginOverlap(CollisionComponent)
  (params (OverlappedComponent :type Primitive%20Component%20Object%20Reference) (OtherActor :type Actor%20Object%20Reference) (OtherComp :type Primitive%20Component%20Object%20Reference) (OtherBodyIndex :type Integer) (bFromSweep :type Boolean) (SweepResult :type Hit%20Result%20Structure%20%28by%20ref%29))
  (Default|CallOnProjectileCollision OtherActor)
  (Effects|SpawnEmitteratLocation (Variables|Default|GetCollisionEmitter) (.Location (Collision|BreakHitResult SweepResult)))
  (Class|EnemyProjectile|HandleBeginOverlap OtherActor)
  (Class|BPIDamageable|TakeDamage(Message) OtherActor (Utilities|Struct|MakeS_DamageInfo (Variables|Default|GetProjectileDamage) "NewEnumerator2" "NewEnumerator3" true false "NewEnumerator0" 0 "/Game/Zak/Enemy/BP_Projectile.BP_Projectile_C"))
  (Class|BPIDamageable|GetCurrentHealth(Message) OtherActor))

(event OnComponentHit(CollisionComponent)
  (params (HitComponent :type Primitive%20Component%20Object%20Reference) (OtherActor :type Actor%20Object%20Reference) (OtherComp :type Primitive%20Component%20Object%20Reference) (NormalImpulse :type Vector :default "0, 0, 0") (Hit :type Hit%20Result%20Structure%20%28by%20ref%29))
  (Default|CallOnProjectileCollision OtherActor Hit)
  (Effects|SpawnEmitteratLocation (Variables|Default|GetCollisionEmitter) (.Location (Collision|BreakHitResult Hit))))

(event Custom|RotateToTarget
  (Variables|/Script/Engine.MovementComponent|SetVelocity (Variables|Default|GetProjectileMovement) (* (Math|Vector|GetUnitDirection(Vector) (Transformation|GetActorLocation) (Transformation|GetActorLocation (Game|GetPlayerCharacter 0))) (Variables|Stats|GetInitial%20Speed))))

(event EventBeginPlay
  (CallFunction|RotatetoTarget)
  (Variables|Default|SetProjectileDeathTimer 1.5))

(event EventTick
  (params (DeltaSeconds :type Float%20%28single-precision%29))
  (if (>= (- (Utilities|Time|GetGameTimeinSeconds) (Variables|Default|GetProjectileSpawnTime)) (Variables|Default|GetMaxProjectileSpawnTime))
    (Variables|Default|SetProjectileSpawnTime (Utilities|Time|GetGameTimeinSeconds))
    (Variables|Default|SetbIsHoming false)))

(fn ConstructionScript
  (bind _projectilemovement (Variables|Default|GetProjectileMovement))
  (Variables|/Script/Engine.ProjectileMovementComponent|SetInitialSpeed _projectilemovement (Variables|Stats|GetInitial%20Speed))
  (Variables|/Script/Engine.ProjectileMovementComponent|SetMaxSpeed _projectilemovement (Variables|Stats|GetMax%20Speed))
  (if (Variables|Default|GetbIsHoming)
    (Variables|/Script/Engine.ProjectileMovementComponent|SetbIsHomingProjectile _projectilemovement true)
    (bind _returnvalue (Actor|GetActorOfClass "/Game/Zak/BP_Player.BP_Player_C"))
    (Variables|/Script/Engine.ProjectileMovementComponent|SetHomingTargetComponent _projectilemovement (Variables|/Script/Engine.Actor|GetRootComponent _returnvalue))))