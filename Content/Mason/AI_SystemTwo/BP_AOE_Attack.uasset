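; BP_AOE_Attack is a spawned area-of-effect attack actor that checks whether the player is inside its radius.
; TriggerAoe sets particle, radius and scale after spawn, replacing an older size-flag event marked obsolete.
; A sphere overlap ignoring the instigator fires a dispatcher on finding the player, leaving damage to the bound enemy.
; It shows a Niagara component at tiny scales, otherwise attaches the scaled emitter and destroys itself on finish or timeout.
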(event Custom|SpawnAOE_Sphere
  (bind _scale (Variables|Default|GetScale))
  ;[0.1598 0.398 1] Spawn a overlap sphere whihc will be used as a damage radius and iterate tthrough each overlapping actor. If player apply damage and call AOE event that is bound in Enemy one
  (bind _outactors (Collision|SphereOverlapActors (Transformation|GetActorLocation) (Variables|Default|GetSphere%20Radius) (Utilities|Array|MakeArray "ObjectTypeQuery4") 0 (Utilities|Array|MakeArray (Variables|Actor|GetInstigator))))
  (for _array_element _outactors
    (if (== _array_element (Game|GetPlayerCharacter 0))
      (Default|CallOnOverlapAOEAttack) ; Call to bind in enemy 4 to apply damage
      (else
        (Development|PrintString "Could not find player in aoe overlap" true true "(R=0.000000,G=0.660000,B=1.000000,A=1.000000)" 5.0)))
    (if (< (Variables|Default|GetScale) 0.1)
      ;[1 0.6378 0.2622] Spawn in emitter or set visible for niagara component
      (Rendering|SetVisibility (Variables|Default|GetNiagaraComponent) true false)
      (else
        (bind _emitter (Variables|Default|GetEmitter)
          (:then
            (bind _returnvalue (Effects|SpawnEmitterAttached _emitter (Variables|Default|GetDefaultSceneRoot) "None" "0, 0, 0" "0, 0, 0" (Math|Vector|MakeVector _scale _scale 1.0)))
            (EventDispatchers|AssignOnSystemFinished _returnvalue (delegate Custom|on%20emitter%20finished))
            (Utilities|FlowControl|Delay 5.0)
            (Actor|DestroyActor))
          (:else
            (Utilities|FlowControl|Delay 1.0)
            (Actor|DestroyActor))))))
  (if (< (Variables|Default|GetScale) 0.1)
    (Rendering|SetVisibility (Variables|Default|GetNiagaraComponent) true false)
    (else
      (bind _emitter_2 (Variables|Default|GetEmitter)
        (:then
          (bind _returnvalue_2 (Effects|SpawnEmitterAttached _emitter_2 (Variables|Default|GetDefaultSceneRoot) "None" "0, 0, 0" "0, 0, 0" (Math|Vector|MakeVector _scale _scale 1.0)))
          (EventDispatchers|AssignOnSystemFinished _returnvalue_2 (delegate Custom|on%20emitter%20finished))
          (Utilities|FlowControl|Delay 5.0)
          (Actor|DestroyActor))
        (:else
          (Utilities|FlowControl|Delay 1.0)
          (Actor|DestroyActor))))))

(event Custom|TriggerAoe
  (params (particleSystem :type Particle%20System%20Object%20Reference) (Radius :type Float%20%28double-precision%29) (Scale :type Float%20%28double-precision%29))
  ;[1 1 1] init size of radius as well as particle effect and is triggere after spawn in call bind process. not large? not small? just right :)
  (Variables|Default|SetEmitter particleSystem)
  (Variables|Default|SetSphere%20Radius Radius)
  (Variables|Default|SetScale Scale)
  (CallFunction|SpawnAOESphere))

(event Custom|on%20emitter%20finished
  (params (PSystem :type Particle%20System%20Component%20Object%20Reference))
  ;[1 0.6378 0.2622] Spawn in emitter or set visible for niagara component
  (Actor|DestroyActor))

(event Custom|CustomEvent
  (params (LargeRadius :type Boolean) (Small%20Radius :type Boolean) (particleSystem :type Particle%20System%20Object%20Reference) (radiusMultiplier :type Float%20%28double-precision%29))
  ;[1 0 0.02871] OLDDDDDDDDD, dont use! init size of radius as well as particle effect and is triggere after spawn in call bind process. not large? not small? just right :)
  (bind _output_get (Variables|Default|SetSmall%20Radius Small%20Radius))
  (if _output_get
    (CallFunction|SpawnAOESphere)
    (else
      (Variables|Default|SetEmitter particleSystem)
      (bind _output_get_2 (Variables|Default|SetLarge%20Radius LargeRadius))
      (if _output_get_2
        (Variables|Default|SetSphere%20Radius 8e+02)
        (Variables|Default|SetSphere%20Radius 0.0)
        (else
          (bind _output_get_3 (Variables|Default|SetSphere%20Radius 4e+02))))
      (CallFunction|SpawnAOESphere))))

(event EventBeginPlay)

(event EventRestart
  (Actor|DestroyActor))

(fn ConstructionScript)