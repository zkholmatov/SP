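; BP_EnemyThree is a child enemy Blueprint that configures a shared AI enemy base with this type's combat setup.
; BeginPlay equips three weapons on right-hand, left-hand and head sockets, sets stagger, trace radius and fracture class, then runs parent logic.
; Overrides supply BP_NoWeapon as the weapon class, attack and defend ranges, and directional hit-reaction montages.
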(event EventBeginPlay
  (Variables|Default|SetEnemyMaxHealth (Variables|Default|GetEnemyMaxHealth))
  (Variables|Default|SetWeaponDamage (Variables|Default|GetWeaponDamage))
  (Variables|Default|SetTraceColliderRadius 5e+01)
  (Variables|Default|SetStaggerTimer 2.5)
  (bind _weapon (CallFunction|WeaponEquip (Variables|Default|GetprimaryWeaponSocket))) ; calls interface function
  (Variables|Default|SetBP_PrimaryWeapon _weapon)
  (bind _weapon_2 (CallFunction|WeaponEquip (Variables|Default|GetSecondaryWeaponSocket)))
  (Variables|Default|SetBP_SecondaryWeapon _weapon_2)
  (bind _weapon_3 (CallFunction|WeaponEquip (Variables|Default|GetThirdWeaponSocket)))
  (Variables|Default|SetBP_ThirdWeapon _weapon_3)
  (Variables|Default|SetFractureClass "/Game/Zak/Fracture/BP_FractureEnemy3.BP_FractureEnemy3_C")
  (|CallParentFunction))

(event Collision|EventActorBeginOverlap
  (params (OtherActor :type Actor%20Object%20Reference)))

(fn ConstructionScript
  (|CallParentFunction)
  (Variables|Default|SetExecutionWidget (Variables|Default|GetExecutionWidget)))

(fn SetWeaponSetSocket
  (Variables|Default|SetprimaryWeaponSocket "R_Weapon")
  (Variables|Default|SetSecondaryWeaponSocket "L_Weapon")
  (Variables|Default|SetThirdWeaponSocket "Head_Weapon")
  (bind _output_get (Variables|Default|SetWeaponClass "/Game/Zak/Weapons/BP_NoWeapon.BP_NoWeapon_C"))
  (return _output_get))

(fn GetIdealRange
  (return 1.2e+02 5e+02 4e+02 6e+02 0.0))

(fn SetHitReactionMontage
  (params (NewParam :type E_DamageDirection%20Enum :default "NewEnumerator0"))
  (LocalVariables|SetLocalDamageDirection NewParam)
  (if (Utilities|Enum|Equal(Enum) (LocalVariables|GetLocalDamageDirection) "NewEnumerator0")
    (return "/Game/Mason/AI_SystemTwo/Enemy3/Enemy3_HitReaction_1.Enemy3_HitReaction_1")
    (elif (Utilities|Enum|Equal(Enum) (LocalVariables|GetLocalDamageDirection) "NewEnumerator1")
      (return "/Game/Mason/AI_SystemTwo/Enemy3/Enemy3_HitReaction_2.Enemy3_HitReaction_2")
      (elif (Utilities|Enum|Equal(Enum) (LocalVariables|GetLocalDamageDirection) "NewEnumerator2")
        (return "/Game/Mason/AI_SystemTwo/Enemy3/Enemy3_HitReaction_3.Enemy3_HitReaction_3")
        (elif (Utilities|Enum|Equal(Enum) (LocalVariables|GetLocalDamageDirection) "NewEnumerator3")
          (return "/Game/Mason/AI_SystemTwo/Enemy3/Enemy3_HitReaction_4.Enemy3_HitReaction_4"))))))