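; BP_EnemyTwo is a child enemy Blueprint that wields a Buster Blade and configures the parent's AI and combat setup.
; It overrides the weapon class, socket and ideal combat ranges, and sets trace radius and stagger timer on BeginPlay before calling the parent.
; The C++ projectile event is empty; a skull projectile spawn from the blade's trail socket is left unconnected.
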(event EventBeginPlay
  (Variables|Default|SetEnemyMaxHealth (Variables|Default|GetEnemyMaxHealth))
  (Variables|Default|SetWeaponDamage (Variables|Default|GetWeaponDamage))
  (Variables|Default|SetTraceColliderRadius 4e+01)
  (Variables|Default|SetStaggerTimer 2.5)
  (|CallParentFunction))

(event EventMyFireProjectileEvent
  ;[1 0.07926 0.7768] Range Attack
)

(fn ConstructionScript
  (|CallParentFunction)
  (Variables|Default|SetExecutionWidget (Variables|Default|GetExecutionWidget)))

(fn GetIdealRange
  (return 3.5e+02 0.0 1.3e+03 6e+02 0.0))

(fn SetWeaponSetSocket
  (Variables|Default|SetprimaryWeaponSocket "BusterBladeSocket")
  (bind _output_get (Variables|Default|SetWeaponClass "/Game/Zak/Weapons/BusterBlade/BP_BusterBlade.BP_BusterBlade_C"))
  (return _output_get))