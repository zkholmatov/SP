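; BP_EnemyFive is a staff-wielding boss enemy with a health bar, death screen and respawn reset.
; Launch events drive a backward leap and a jump that hovers with gravity switched off.
; Staff socket sphere traces deal parriable damage; a parry or every third hit sets the stagger Blackboard key around a hit-reaction montage.
; Summon notifies spawn mages, EnemyTwo minions set to chase the player, or AOE projectiles at the player's location.
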(event Custom|SpawnEnemyTwo
  (bind _returnvalue (Game|GetPlayerCharacter 0))
  ;[1 0.1379 0.7634] Spawn enemy two based off of summon that is called in animation notify
  (bind _returnvalue_2 (Game|SpawnActorfromClass "/Game/Mason/AI_SystemTwo/Enemy2/BP_EnemyTwo.BP_EnemyTwo_C" (Math|Transform|MakeTransform (+ (AI|Components|Blackboard|GetValueasVector (AI|GetBlackboard 0) (Variables|Default|GetPointOfInterest)) "") "0, 0, 0" "1.000000,1.000000,1.000000") "AdjustIfPossibleButAlwaysSpawn" "MultiplyWithRoot" 0 0))
  (bind _weapon (Default|WeaponEquip _returnvalue_2 (Variables|/Game/Mason/AI_SystemTwo/BP_EnemyOne.BP_EnemyOne_C|GetprimaryWeaponSocket _returnvalue_2))) ; calls interface function
  (Variables|Default|SetBP_PrimaryWeapon _weapon)
  (bind _output_get (Variables|/Game/Mason/AI_SystemTwo/BP_EnemyOne.BP_EnemyOne_C|SetBehaviorTree _returnvalue_2 "/Game/Mason/AI_SystemTwo/BT_BB/BT_EnemyTwo.BT_EnemyTwo"))
  (AI|RunBehaviorTree (Variables|/Game/Mason/AI_SystemTwo/BP_EnemyOne.BP_EnemyOne_C|GetAIC_CPP_Obj _returnvalue_2) _output_get)
  (Utilities|IsValid _returnvalue
    (:Is%20Valid
      (Variables|/Game/Mason/AI_SystemTwo/AI_Controllers/EnemyOne/AIC_CPP_EnemyBase.AIC_CPP_EnemyBase_C|SetAttack%20Target (Variables|/Game/Mason/AI_SystemTwo/BP_EnemyOne.BP_EnemyOne_C|GetAIC_CPP_Obj _returnvalue_2) _returnvalue)
      (Default|CallRandomWalkSpeed _returnvalue_2)
      (Default|DisplayHealthBar _returnvalue_2)
      (Class|AIControllerCPP|SetStateasChase (Variables|/Game/Mason/AI_SystemTwo/BP_EnemyOne.BP_EnemyOne_C|GetAIC_CPP_Obj _returnvalue_2))
      (Pawn|SpawnDefaultController _returnvalue_2)
      (Rendering|SetVisibility (Variables|/Game/Mason/AI_SystemTwo/BP_EnemyOne.BP_EnemyOne_C|GetPointLight _returnvalue_2) true false))
    (:Is%20Not%20Valid
      (Development|PrintString "Get player is NOT valid in E5 summon e3" true true "(R=1.000000,G=0.000000,B=0.139431,A=1.000000)" 5.0))))

(event Custom|SummonProjectiles
  ;[1 0.07926 0.7768] Call Summons
  (Game|SpawnActorfromClass "/Game/Mason/AI_SystemTwo/projectiles/BP_EnemyAOE_Summon.BP_EnemyAOE_Summon_C" (Math|Conversions|ToTransform(Vector) (Transformation|GetActorLocation (Game|GetPlayerCharacter 0))) "Undefined" "MultiplyWithRoot" 0 2.0 3.0 false (Variables|EnemyStats|GetMax%20Summoned%20Projectile%20Speed) (Variables|EnemyStats|GetInitial%20Summoned%20Projectile%20Speed) (Variables|EnemyStats|GetProjectile%20Damage) 0) ; Damage Set in Class Construction
)

(event Custom|TracingEvent
  (params (Start :type Vector) (End :type Vector))
  ;[1 0.4849 0.4351 1 30] Trace + apply damage
  (bind _outactors (Actor|GetAllActorsOfClass "/Game/Mason/AI_SystemTwo/BP_EnemyOne.BP_EnemyOne_C"))
  (bind (_outhit _returnvalue) (Collision|SphereTraceForObjects Start End (Variables|Default|GetTraceColliderRadius) (Utilities|Array|MakeArray "ObjectTypeQuery4") false _outactors "ForDuration" true "(R=1.000000,G=0.045752,B=0.620198,A=1.000000)" "(R=0.000000,G=1.000000,B=0.000000,A=1.000000)" 2.0))
  (if _returnvalue
    (Utilities|FlowControl|DoOnce false :!label _label
      (:Completed
        (if (== (Game|GetPlayerCharacter 0) (.HitActor (Collision|BreakHitResult _outhit)))
          (bind _wasparried_ (Class|BPIDamageable|TakeDamage(Message) (.HitActor (Collision|BreakHitResult _outhit)) (Utilities|Struct|MakeS_DamageInfo (Variables|Default|GetWeaponDamage) "NewEnumerator1" "NewEnumerator3" (not (Variables|Default|GetbNotParriable)) false (CallFunction|CalculateDamageDirection self (.HitActor (Collision|BreakHitResult _outhit))) self)))
          (Class|BPIDamageable|GetCurrentHealth(Message) (.HitActor (Collision|BreakHitResult _outhit)))
          (if _wasparried_
            (AI|Components|Blackboard|SetValueasBool (AI|GetBlackboard (AI|GetAIController self)) (Variables|Default|GetBB_bIsStaggered) true)
            (Class|MyEnemy|MySwordTraceStopEvent)
            (bind _hitreactionmontage (CallFunction|SetHitReactionMontage "NewEnumerator0"))
            (Animation|Montage|PlayMontage (Variables|Character|GetMesh) _hitreactionmontage
              (:OnCompleted
                _)
              (:OnInterrupted
                _))
            (AI|Components|Blackboard|SetValueasBool (AI|GetBlackboard (AI|GetAIController self)) (Variables|Default|GetBB_bIsStaggered) false)
            (else
              (Class|MyEnemy|MySwordTraceStopEvent)))
          (else
            (Development|PrintString "Hello")))))
    (else
      (goto _label Reset))))

(event Custom|OnPlayerDeath_Event
  ;[0.07785 0.2591 1] Begin Play - Init enemy and stats
  ;;[1 0.03035 0.07016] if Player is dead turn off boss health bar visibility
  (Widget|SetVisibility (Variables|Default|GetBoss%20Health%20Bar) "Hidden"))

(event Custom|JumpLaunch
  (bind _charactermovement (Variables|Character|GetCharacterMovement))
  ;[0.07785 0.2591 1] Begin Play - Init enemy and stats
  ;;[0.2699 0.8292 1] Jump Attack - is a event that launches enemy in the air after the notify is played inside an animation montage. This is called inside of the BTTtask_JumpAttack
  (Character|LaunchCharacter "0.000000,0.000000,550.000000" true false)
  (Utilities|FlowControl|Delay 0.55) ; I may need to be increased so i dont go on top of the player without consent
  (if (AI|Components|NavMovement|IsFalling (Variables|Character|GetCharacterMovement))
    (Variables|/Script/Engine.CharacterMovementComponent|SetGravityScale _charactermovement 0.0)
    (Utilities|FlowControl|Delay 7.15)
    (Variables|/Script/Engine.CharacterMovementComponent|SetGravityScale _charactermovement 1.0)))

(event Custom|LungeAttack_Event
  ;[0.07785 0.2591 1] Begin Play - Init enemy and stats
  (Character|LaunchCharacter (* (Transformation|GetActorForwardVector) -3.5e+03) false false))

(event Custom|SpawnEnemyMage
  (bind _returnvalue (Game|GetPlayerCharacter 0))
  ;[1 0.1373 0.7647] Spawn enemy mage based off of summon that is called in animation notify
  (bind _returnvalue_2 (Game|SpawnActorfromClass "/Game/Mason/AI_SystemTwo/BP_EnemyMage.BP_EnemyMage_C" (Math|Transform|MakeTransform (+ (AI|Components|Blackboard|GetValueasVector (AI|GetBlackboard 0) (Variables|Default|GetPointOfInterest)) "") "0, 0, 0" "1.000000,1.000000,1.000000") "AdjustIfPossibleButAlwaysSpawn" "MultiplyWithRoot" 0 false 0))
  (bind _weapon (Default|WeaponEquip _returnvalue_2 (Variables|/Game/Mason/AI_SystemTwo/BP_EnemyOne.BP_EnemyOne_C|GetprimaryWeaponSocket _returnvalue_2))) ; calls interface function
  (Variables|Default|SetBP_PrimaryWeapon _weapon)
  (bind _output_get (Variables|/Game/Mason/AI_SystemTwo/BP_EnemyOne.BP_EnemyOne_C|SetBehaviorTree _returnvalue_2 "/Game/Mason/AI_SystemTwo/BT_BB/BT_Mage.BT_Mage"))
  (AI|RunBehaviorTree (Variables|/Game/Mason/AI_SystemTwo/BP_EnemyOne.BP_EnemyOne_C|GetAIC_CPP_Obj _returnvalue_2) _output_get)
  (Utilities|IsValid _returnvalue
    (:Is%20Valid
      (Variables|/Game/Mason/AI_SystemTwo/AI_Controllers/EnemyOne/AIC_CPP_EnemyBase.AIC_CPP_EnemyBase_C|SetAttack%20Target (Variables|/Game/Mason/AI_SystemTwo/BP_EnemyOne.BP_EnemyOne_C|GetAIC_CPP_Obj _returnvalue_2) _returnvalue)
      (Default|CallRandomWalkSpeed _returnvalue_2)
      (Default|DisplayHealthBar _returnvalue_2)
      (Class|AIControllerCPP|SetStateasChase (Variables|/Game/Mason/AI_SystemTwo/BP_EnemyOne.BP_EnemyOne_C|GetAIC_CPP_Obj _returnvalue_2))
      (Pawn|SpawnDefaultController _returnvalue_2)
      (Rendering|SetVisibility (Variables|/Game/Mason/AI_SystemTwo/BP_EnemyOne.BP_EnemyOne_C|GetPointLight _returnvalue_2) true false))
    (:Is%20Not%20Valid
      (Development|PrintString "Get player is NOT valid in E5 summon e3" true true "(R=1.000000,G=0.000000,B=0.139431,A=1.000000)" 5.0))))

(event EventBeginPlay
  (bind _self self)
  ;[0.07785 0.2591 1] Begin Play - Init enemy and stats
  (Variables|Default|SetbIsBoss true)
  (Variables|Default|SetEnemyMaxHealth (Variables|Default|GetEnemyMaxHealth))
  (Variables|Default|SetWeaponDamage (Variables|Default|GetWeaponDamage))
  (Variables|Default|SetTraceColliderRadius 4e+01)
  (Variables|Default|SetStaggerTimer 7.0)
  (Variables|Default|SetAOE%20Damage%20Amount (Variables|Default|GetAOE%20Damage%20Amount))
  (bind _weapon (CallFunction|WeaponEquip (Variables|Default|GetSecondaryWeaponSocket)))
  (Variables|Default|SetBP_SecondaryWeapon _weapon)
  (bind _returnvalue (UserInterface|CreateWidget "/Game/Zak/UI/Wigets/W_BossHealthbar.W_BossHealthbar_C" 0 _self _self (Variables|Default|GetBossName)))
  (Variables|Default|SetBoss%20Health%20Bar _returnvalue)
  (|CallParentFunction)
  (EventDispatchers|BindEventtoJumpAttackLaunch (delegate Custom|JumpLaunch))
  (EventDispatchers|BindEventtoLungeAttack (delegate Custom|LungeAttack_Event)) ; this is used for jump backwards
  ;;[1 0.03035 0.07016] if Player is dead turn off boss health bar visibility
  (bind _as_bp_player (Variables|Default|GetAs%20BP%20Player)
    (:then
      (EventDispatchers|AssignOnPlayerDeath _as_bp_player (delegate Custom|OnPlayerDeath_Event)))
    (:else
      (Development|PrintString "not getting player ref" true true "(R=0.000000,G=0.660000,B=1.000000,A=1.000000)" 2e+01))))

(event EventOnDead
  ;[0.3012 1 0.2163] Self on death
  (Variables|Default|SetWeaponDamage 0.0)
  (Variables|Default|SetAOE%20Damage%20Amount 0.0)
  (Variables|Default|SetDeathDelay 1e+01)
  (Widget|SetVisibility (Variables|Default|GetBoss%20Health%20Bar) "Hidden")
  (|CallParentFunction))

(event EventRestart
  ;[1 1 1] Respawn System for enemies - Zak
  (Transformation|SetActorTransform (Variables|Default|GetSpawnTransform) false true)
  (Default|SetMaxHealth (Variables|Default|GetBPC_DamageSystem) (Variables|Default|GetEnemyMaxHealth) true)
  (Components|Movement|StopMovementImmediately (Variables|Character|GetCharacterMovement))
  (bind _asaic_cpp_enemy_five (Utilities|Casting|CastToAIC_CPP_EnemyFive (AI|GetAIController self))
    (:then
      (Class|AIControllerCPP|SetStateasIdle _asaic_cpp_enemy_five)
      (bind _boss_health_bar (Variables|Default|GetBoss%20Health%20Bar)
        (:then
          (Widget|SetVisibility _boss_health_bar "Hidden"))
        (:else)))
    (:CastFailed
      (Development|PrintString "Cast in E5 respawn logic failed"))))

(event EventDamageResponse
  (params (DamageResponse :type E_DamageResponse%20Enum :default "NewEnumerator0") (DamageDirection :type E_DamageDirection%20Enum :default "NewEnumerator0") (DamageCauser :type Actor%20Object%20Reference))
  ;[0.3843 0.4745 1] DamageResponse / stunned
  (bind _output_get (Variables|Default|SetWasHitCount (+ (Variables|Default|GetWasHitCount) 1)))
  (if (> _output_get 2)
    (Development|PrintString "Staggered")
    (AI|Components|Blackboard|SetValueasBool (AI|GetBlackboard (AI|GetAIController self)) (Variables|Default|GetBB_bIsStaggered) true) ; set black baord decorator bIsStaggered to true for BT to adjust behavior path
    (Variables|Default|SetLastDamageTime (Utilities|Time|GetGameTimeinSeconds)) ; reset time since last damage stimuli
    (Components|Movement|StopMovementImmediately (Variables|Character|GetCharacterMovement)) ; Stop movement of enemy before queuing animation for stagger
    (bind _hitreactionmontage (CallFunction|SetHitReactionMontage DamageDirection))
    (Animation|Montage|PlayMontage (Variables|Character|GetMesh) _hitreactionmontage 0.9
      (:OnCompleted
        _)
      (:OnBlendOut
        _)
      (:OnInterrupted
        _))
    (AI|Components|Blackboard|SetValueasBool (AI|GetBlackboard (AI|GetAIController self)) (Variables|Default|GetBB_bIsStaggered) false) ; reset value of is staggered to false
    (Class|AISenseDamage|ReportDamageEvent self (Game|GetPlayerCharacter 0) 0.0 (Transformation|GetActorLocation) "0, 0, 0" "None") ; Report damage event to AI controller assocaited with enemy
    (Variables|Default|SetWasHitCount 0)))

(event EventSummon
  (params (SummonE1 :type Boolean) (SummonMage :type Boolean) (SummonE2 :type Boolean) (SummonProjectiles :type Boolean))
  ;[1 0.07926 0.7768] Call Summons
  (if SummonMage
    (CallFunction|SpawnEnemyMage)
    (elif SummonE2
      (CallFunction|SpawnEnemyTwo)
      (elif SummonProjectiles
        (CallFunction|SummonProjectiles)))))

(event EventSwordTraceLoop
  (bind _bp_primaryweapon (Variables|Default|GetBP_PrimaryWeapon))
  (bind _bp_secondaryweapon (Variables|Default|GetBP_SecondaryWeapon))
  (bind _weapon (Variables|/Game/Zak/Weapons/BP_Weapon.BP_Weapon_C|GetWeapon _bp_secondaryweapon))
  (bind _weapon_2 (Variables|/Game/Zak/Weapons/BP_Weapon.BP_Weapon_C|GetWeapon _bp_primaryweapon))
  ;[1 0.4849 0.4351 1 30] Trace + apply damage
  ;;[1 1 1] Overriding enemy one base
  ;;[1 1 1] Set socket for each weapon being used for enemy five
  (if (Variables|Default|GetPrimary)
    (CallFunction|TracingEvent (Transformation|GetSocketLocation _weapon_2 "TrailStart") (Transformation|GetSocketLocation _weapon_2 "TrailEnd")))
  (if (Variables|Default|GetSecondary)
    (CallFunction|TracingEvent (Transformation|GetSocketLocation _weapon "TrailStart") (Transformation|GetSocketLocation _weapon "TrailEnd"))))

(fn ConstructionScript
  (|CallParentFunction)
  (Variables|Default|SetExecutionWidget (Variables|Default|GetExecutionWidget)))

(fn GetIdealRange
  (return 2e+02 5.5e+02 3.5e+02 4e+03 4.5e+02))

(fn SetWeaponSetSocket
  (Variables|Default|SetprimaryWeaponSocket "R_FB_Staff")
  (Variables|Default|SetSecondaryWeaponSocket "L_FB_Staff")
  (bind _output_get (Variables|Default|SetWeaponClass "/Game/Mason/AI_SystemTwo/weapon_BluePrints/BP_FBStaff.BP_FBStaff_C"))
  (return _output_get))

(fn DeathExtend
  (|CallParentFunction)
  (bind _returnvalue (UserInterface|CreateWidget "/Game/Zak/UI/Wigets/W_BossDeath.W_BossDeath_C" 0 (Variables|Default|GetBossName)))
  (UserInterface|Viewport|AddtoViewport _returnvalue 0)
  (Audio|PlaySound2D "/Game/Zak/Audio/SFX/dark-impact-232945.dark-impact-232945" 1.0 1.0 0.0 0 0))

(fn HideExecutionWidget
  (Rendering|SetVisibility (Variables|Default|GetExecWidget) false false))

(fn DisplayExecutionWidget
  (Rendering|SetVisibility (Variables|Default|GetExecWidget) true false))