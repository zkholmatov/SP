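; AOE attack actor for Enemy4 that, when triggered, runs a debug-drawn sphere overlap for physics bodies around itself, ignoring its instigator.
; Each hit fires the OnOverlapAOEAttack dispatcher and attaches the Emitter effect, or destroys the actor after a short delay if no emitter is valid.
; Niagara spawning and the effect-finished bindings are disconnected, and an empty overlap result never reaches the destroy step.
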(event Custom|SpawnAOE_Sphere
  (bind _returnvalue (Transformation|GetActorLocation))
  (bind _sphere_radius (Variables|Default|GetSphere%20Radius))
  (Rendering|Debug|DrawDebugSphere _returnvalue _sphere_radius 12 "(R=1.000000,G=0.137930,B=0.763379,A=1.000000)" 2.0 5.0)
  (bind (_outactors _returnvalue_2) (Collision|SphereOverlapActors _returnvalue _sphere_radius (Utilities|Array|MakeArray "ObjectTypeQuery4") 0 (Utilities|Array|MakeArray (Variables|Actor|GetInstigator) 0)))
  (for _array_element _outactors
    (if _returnvalue_2
      (Development|PrintString "true")
      (Default|CallOnOverlapAOEAttack)
      (Development|PrintString "overlapped")
      (bind _emitter (Variables|Default|GetEmitter)
        (:then
          (Effects|SpawnEmitterAttached _emitter (Variables|Default|GetDefaultSceneRoot) "None"))
        (:else
          (Utilities|FlowControl|Delay 1.0 :!label _label)
          (Actor|DestroyActor)))
      (else
        (Development|PrintString "not working ")
        (goto _label)))))

(event Custom|On%20niagara%20finished
  (params (PSystem :type Niagara%20Component%20Object%20Reference))
  (Actor|DestroyActor))

(event Custom|on%20emitter%20finished
  (params (PSystem :type Particle%20System%20Component%20Object%20Reference))
  (Actor|DestroyActor))

(event Custom|TriggerAoe
  (CallFunction|SpawnAOESphere))

(event EventBeginPlay)

(fn ConstructionScript)