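; BP_EnemyFour is an enemy variant in the AI_SystemTwo set, configuring a parent enemy class through overrides.
; BeginPlay sets the trace collider radius and stagger timer before calling the parent BeginPlay, while its max health and weapon damage assignments write each variable back to itself.
; GetIdealRange returns fixed distance bands for attack, defend, second attack and ranged attack.
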(event EventBeginPlay
  (Variables|Default|SetEnemyMaxHealth (Variables|Default|GetEnemyMaxHealth))
  (Variables|Default|SetWeaponDamage (Variables|Default|GetWeaponDamage))
  (Variables|Default|SetTraceColliderRadius 2e+01)
  (Variables|Default|SetStaggerTimer 7.0)
  (|CallParentFunction))

(fn ConstructionScript
  (|CallParentFunction))

(fn GetIdealRange
  (return 3e+02 8e+02 2.8e+03 3.05e+03))