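; BP_EnemyTwo is an enemy Blueprint that configures a parent enemy class with its own health, weapon damage and trace radius.
; On BeginPlay it sets those stats, runs the parent logic, then assigns Weapon1 as the trace location.
; A C++-origin event fires a BP_ProjectileBase ranged attack from ProjectileSpawnLocation through the EnemyProjectile component.
; An unconnected chain for spawning and socketing a BP_BusterBlade sword never runs.
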(event EventBeginPlay
  (Variables|Default|SetEnemyMaxHealth 5e+02)
  (Variables|Default|SetWeaponDamage 2.5e+02)
  (Variables|Default|SetTraceColliderRadius 4e+01)
  (|CallParentFunction)
  (Variables|Default|SetTraceLocation (Variables|Default|Getweapon1)))

(event Collision|EventActorBeginOverlap
  (params (OtherActor :type Actor%20Object%20Reference)))

(event EventTick
  (params (DeltaSeconds :type Float%20%28single-precision%29)))

(event EventMyFireProjectileEvent
  ;[1 0.07926 0.7768] Range Attack
  (Class|EnemyProjectileComponent|SpawnProjectile (Variables|Default|GetEnemyProjectile) "ProjectileSpawnLocation" "/Game/Mason/BluePrints/BP_ProjectileBase.BP_ProjectileBase_C"))

(fn ConstructionScript
  (|CallParentFunction))