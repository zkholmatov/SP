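; Actor that spawns a ring of BP_Column actors around itself one at a time, then destroys itself.
; BeginPlay uses sine and cosine to precompute evenly spaced circle offsets from MaxSpawn and Radius into Locations.
; A looping timer fires Spawner to place each column at the next offset, then stops and destroys the spawner after a delay.
; Older hard-coded and degree-based placement attempts remain in the graph, disconnected.
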(event Custom|Spawner
  (bind _returnvalue (Transformation|GetActorTransform))
  ;[0.2023 0.3454 1 1 40] spawn mesh at location at incremented time
  (bind _result (Math|Integer|IncrementInt (Variables|Default|Getactors_Spawned)) ; increment actors spawned
    (:%20%20
      (Variables|Default|Setactors_Spawned _result)
      (if (not (> (Variables|Default|Getactors_Spawned) (Variables|Default|GetmaxSpawn#))) ; only spawn actors for number of max spawned var
        (Game|SpawnActorfromClass "/Game/Mason/BP_Column.BP_Column_C" (Math|Transform|MakeTransform (+ (Utilities|Array|Get(acopy) (Variables|Default|GetLocations) (Variables|Default|Getactors_Spawned)) (.location _returnvalue)) "0, 0, 0" (.scale _returnvalue)) "Undefined" "MultiplyWithRoot" 0 0)
        (else
          (Utilities|Time|ClearTimerbyFunctionName 0 "Spawner") ; Clearn timer so it stops looping after it cant pass branch
          (Utilities|FlowControl|Delay 5.0)
          (Actor|DestroyActor))))))

(event EventBeginPlay
  (bind _maxspawn_ (Variables|Default|GetmaxSpawn#))
  ;[0 1 0.5043 1 40] Is in radians- Set intial angle whihc is determined by #spawned
  (Variables|Default|Setangle (* (/ (Math|Trig|GetPI) _maxspawn_) 2.0)) ; Set intial angle whihc is determined by #spawned
  ;[1 0.8614 0.2768 1 40] init locations for circle spawn
  (for _index (range 0 _maxspawn_)
    (Variables|Default|Settheta (+ (Variables|Default|Gettheta) (Variables|Default|Getangle)))
    (bind _output_get (Variables|NotUsed|SetY (* (Math|Trig|Sin(Radians) (Variables|Default|Gettheta)) (Variables|Default|Getradius))))
    (bind _output_get_2 (Variables|NotUsed|SetX (* (Math|Trig|Cos(Radians) (Variables|Default|Gettheta)) (Variables|Default|Getradius))))
    (bind _output_get_3 (Variables|Default|SetOffsettingVector (Math|Vector|MakeVector _output_get_2 _output_get 0.0)))
    ;[1 0.1914 0.3927 1 40] Load Vectors in array
    (Utilities|Array|Add (Variables|Default|GetLocations) (* _output_get_3 "1.500000,1.500000,0.000000")))
  ;[0.2023 0.3454 1 1 40] spawn mesh at location at incremented time
  (Utilities|Time|SetTimerbyEvent (delegate Custom|Spawner) (Variables|Default|GetTime) true))

(fn ConstructionScript)