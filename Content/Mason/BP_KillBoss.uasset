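; BP_KillBoss is a trigger that kills a level boss when the player character overlaps its Box, apparently as a dev shortcut.
; The overlap optionally fires CallDevPortal to reveal a bound teleport portal, then checks flags for Myre, Warden or the final boss.
; It finds the selected boss with GetActorOfClass and passes it to DamageBoss, which sends huge damage through TakeDamageMessage and prints the result.
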(event OnComponentBeginOverlap(Box)
  (params (OverlappedComponent :type Primitive%20Component%20Object%20Reference) (OtherActor :type Actor%20Object%20Reference) (OtherComp :type Primitive%20Component%20Object%20Reference) (OtherBodyIndex :type Integer) (bFromSweep :type Boolean) (SweepResult :type Hit%20Result%20Structure%20%28by%20ref%29))
  ;[0.2314 1 0.1848 1 40] ensure overlap is character,
  (if (== OtherActor (Game|GetPlayerCharacter 0))
    ;[1 0.2532 0.6284 1 40] if call portal is true, call event that is bound inside teleportal, visibility of portal is then enabled and no longer hidden in game
    (if (Variables|Default|GetbCallPortal)
      (Default|CallDevPortal))
    ;[1 0.2599 0.2499 1 40] based off of set bool choose whihc boss in level to damage ie kill in game
    (if (Variables|Default|Getmyre)
      (bind _returnvalue (Actor|GetActorOfClass "/Game/Mason/AI_SystemTwo/Enemy4/BP_EnemyFour.BP_EnemyFour_C"))
      (Variables|Default|SetMyreBoss _returnvalue)
      (bind _myreboss (Variables|Default|GetMyreBoss)
        (:then
          (CallFunction|DamageBoss _myreboss))
        (:else))
      (elif (Variables|Default|Getwarden)
        (bind _returnvalue_2 (Actor|GetActorOfClass "/Game/Zak/AbyssalWarden/BP_AbyssalWarden.BP_AbyssalWarden_C"))
        (Variables|Default|SetWardenBoss _returnvalue_2)
        (bind _wardenboss (Variables|Default|GetWardenBoss)
          (:then
            (CallFunction|DamageBoss _wardenboss))
          (:else))
        (elif (Variables|Default|GetbFinalBoss)
          (bind _returnvalue_3 (Actor|GetActorOfClass "/Game/Mason/AI_SystemTwo/Enemy5/BP_EnemyFive.BP_EnemyFive_C"))
          (Variables|Default|SetFinalBoss _returnvalue_3)
          (bind _finalboss (Variables|Default|GetFinalBoss)
            (:then
              (CallFunction|DamageBoss _finalboss))
            (:else)))))))

(event EventBeginPlay)

(fn ConstructionScript)

(fn DamageBoss
  (params (Boss%20Ref :type Object%20Object%20Reference))
  (bind _wasdamaged_ (Class|BPIDamageable|TakeDamage(Message) Boss%20Ref (Utilities|Struct|MakeS_DamageInfo 1e+04 "NewEnumerator1" "NewEnumerator3" true false "NewEnumerator0" self)))
  (if _wasdamaged_
    (Development|PrintString "damaged")
    (else
      (Development|PrintString "Not damaged in kill boss"))))