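; BP_Lift is a lift that automatically shuttles between its placed location and a target point, pausing at each turnaround.
; On BeginPlay it stores the start location and converts TargetLocation from a relative offset to a world position.
; The UppyThenDowny timeline lerps the actor between both points without sweeping.
; When the timeline finishes, it flips Direction and, after a delay, replays forward or in reverse.
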(event Custom|PlatformMovement
  (bind _trackone (Timeline|Uppy%20then%20downy Play)
    (:Update
      (Transformation|SetActorLocation (Math|Vector|Lerp(Vector) (Variables|Default|GetStartLocation) (Variables|Default|GetTargetLocation) _trackone) false false))
    (:Finished
      (Variables|Default|SetbDirection (not (Variables|Default|GetbDirection)))
      (Utilities|FlowControl|Delay 2.0)
      (if (Variables|Default|GetbDirection)
        (Timeline|Uppy%20then%20downy PlayFromStart)
        (else
          (Timeline|Uppy%20then%20downy ReverseFromEnd))))))

(event EventBeginPlay
  (Variables|Default|SetStartLocation (Transformation|GetActorLocation))
  (Variables|Default|SetTargetLocation (+ (Variables|Default|GetStartLocation) (Variables|Default|GetTargetLocation)))
  (CallFunction|PlatformMovement))

(fn ConstructionScript)