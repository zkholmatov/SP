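; Inventory actor component that handles looking at, interacting with and opening the inventory for the local player.
; BeginPlay adds the default input mapping and creates the inventory widget, which IA_Inventory shows with UI-only input.
; A per-tick camera sphere trace caches LookAtActor and prints its look-at message; IA_PickUp calls InteractWith on that actor's ItemDataComponent.
; AddToInventory, RemoveFromInventory and FindSlot are empty stubs.
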(event EventBeginPlay
  (Input|AddMappingContext (PlayerController|LocalPlayerSubsystems|GetEnhancedInputLocalPlayerSubsystem (Game|GetPlayerController 0)) "/Game/ThirdPerson/Input/IMC_Default.IMC_Default" 0 "(bIgnoreAllPressedKeysUntilRelease=True,bForceImmediately=False,bNotifyUserSettings=False)")
  (bind _returnvalue (UserInterface|CreateWidget "/Game/Omar/UI/WB_Inventory.WB_Inventory_C"))
  (Variables|Widget|SetInventoryWidget _returnvalue))

(event EventTick
  (params (DeltaSeconds :type Float%20%28single-precision%29))
  (CallFunction|InteractionTrace))

(event Input|EnhancedActionEvents|EnhancedInputActionIA_PickUp
  (params (ActionValue :type Boolean) (ElapsedSeconds :type Float%20%28double-precision%29) (TriggeredSeconds :type Float%20%28double-precision%29) (InputAction :type Input%20Action%20Object%20Reference :default "/Game/ThirdPerson/Input/Actions/IA_PickUp.IA_PickUp"))
  ;[1 1 1] Pickup items
  (:Started
    (bind _lookatactor (Variables|Default|GetLookAtActor)
      (:then
        (Utilities|IsValid (Actor|GetComponentbyClass _lookatactor "/Game/Omar/Inventory/ItemDataComponent.ItemDataComponent_C")
          (:Is%20Valid
            (Class|IInteractInterface|Interactwith(Message) (Actor|GetComponentbyClass _lookatactor "/Game/Omar/Inventory/ItemDataComponent.ItemDataComponent_C")))))
      (:else))))

(event Input|EnhancedActionEvents|EnhancedInputActionIA_Inventory
  (params (ActionValue :type Boolean) (ElapsedSeconds :type Float%20%28double-precision%29) (TriggeredSeconds :type Float%20%28double-precision%29) (InputAction :type Input%20Action%20Object%20Reference :default "/Game/ThirdPerson/Input/Actions/IA_Inventory.IA_Inventory"))
  (bind _returnvalue (Game|GetPlayerController 0))
  ;[1 1 1] open inventory
  (:Started
    (UserInterface|Viewport|AddtoViewport (Variables|Widget|GetInventoryWidget) 0)
    (Variables|/Script/Engine.PlayerController|SetbShowMouseCursor _returnvalue true)
    (Input|SetInputModeUIOnly _returnvalue (Variables|Widget|GetInventoryWidget) "DoNotLock" false)))

(fn AddtoInventory
  (params (ItemID :type Name)))

(fn RemovefromInventory)

(fn InteractionTrace
  (bind _returnvalue (Game|GetPlayerCameraManager 0))
  (bind _returnvalue_2 (Transformation|GetActorLocation _returnvalue))
  (bind (_outhit _returnvalue_3) (Collision|SphereTraceByChannel _returnvalue_2 (+ _returnvalue_2 (* (Transformation|GetActorForwardVector _returnvalue) (Variables|Default|GetInteractionRange))) 15.0 "TraceTypeQuery3" false (Utilities|Array|MakeArray (Components|GetOwner)) "None"))
  (if _returnvalue_3
    (if (!= (.HitActor (Collision|BreakHitResult _outhit)) (Variables|Default|GetLookAtActor))
      (bind _output_get (Variables|Default|SetLookAtActor (.HitActor (Collision|BreakHitResult _outhit))))
      (bind _message (Class|IInteractInterface|Lookat(Message) _output_get))
      (Development|PrintString (Utilities|String|ToString(Text) _message)))
    (else
      (Variables|Default|SetLookAtActor 0))))

(fn FindSlot
  (params (ItemID :type Name)))