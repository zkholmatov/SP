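; BP_Item is an inventory item actor that shows its mesh as a spinning object in the world.
; The construction script looks up the item ID in DT_Items and assigns that row's mesh to both Mesh and Overlay.
; It also passes the item's Color to the Overlay materials' Color parameter.
; Tick yaws Mesh by a fixed step each frame, independent of delta time.
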(event EventTick
  (params (DeltaSeconds :type Float%20%28single-precision%29))
  (Transformation|AddRelativeRotation (Variables|Default|GetMesh) (Math|Rotator|MakeRotator 0.0 0.0 1.0) false false))

(fn ConstructionScript
  (bind _returnvalue (Utilities|GetDataTableRow "/Game/Omar/Inventory/DataTables/DT_Items.DT_Items" (.RowName (Utilities|Struct|BreakDataTableRowHandle (.ItemID (Utilities|Struct|BreakS_Slot (Variables|Default|GetItem))))))
    (:then
      (Components|StaticMesh|SetStaticMesh (Variables|Default|GetMesh) (.mesh _returnvalue))
      (Components|StaticMesh|SetStaticMesh (Variables|Default|GetOverlay) (.mesh _returnvalue))
      (Rendering|Material|SetVectorParameterValueonMaterials (Variables|Default|GetOverlay) "Color" (Math|Conversions|ToVector(LinearColor) (Variables|Default|GetColor))))))