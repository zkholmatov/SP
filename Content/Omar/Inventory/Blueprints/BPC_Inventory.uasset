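; Player inventory component that stores items in fixed-size category arrays for swords, three armor types and gemstones, and saves and loads them.
; A forward sphere trace each tick shows the interact prompt for BP_Item actors.
; Interact stacks the item up to its DT_Items stack size or fills an empty slot, then destroys the pickup.
; It also creates and opens the inventory and pause menus, capturing the player's SceneCapture when inventory opens.
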(event EventBeginPlay
  (bind _allitem (Variables|Default|GetAllitem))
  (bind (_swords _helmets _chest_armors _leg_armors _gemstones) (Utilities|Struct|BreakS_Allitem _allitem))
  ;[1 1 1] Create Widgets(currently: interact, pause, inventory)
  (bind _asbp_game_instance (Utilities|Casting|CastToBP_GameInstance (Game|GetGameInstance)))
  (Variables|Default|SetAs%20BP%20Game%20Instance _asbp_game_instance)
  (Class|BPIPersistence|RequestLoad(Message) (Game|GetGameInstance) self)
  (Input|AddMappingContext (PlayerController|LocalPlayerSubsystems|GetEnhancedInputLocalPlayerSubsystem (Game|GetPlayerController 0)) "/Game/ThirdPerson/Input/IMC_Default.IMC_Default" 0 "(bIgnoreAllPressedKeysUntilRelease=True,bForceImmediately=False,bNotifyUserSettings=False)")
  (bind _returnvalue (UserInterface|CreateWidget "/Game/Omar/UI/WidgetBlueprints/WBP_Inventory.WBP_Inventory_C"))
  (Variables|Widget|SetWBP_Inventory _returnvalue)
  (bind _returnvalue_2 (UserInterface|CreateWidget "/Game/Omar/UI/WidgetBlueprints/WBP_Interact.WBP_Interact_C"))
  (Variables|Widget|SetWBP_Interact _returnvalue_2)
  (bind _returnvalue_3 (UserInterface|CreateWidget "/Game/Omar/UI/WidgetBlueprints/WB_PauseMenu.WB_PauseMenu_C"))
  (Variables|Widget|SetPauseWidget _returnvalue_3)
  (Utilities|Array|Resize _swords 12)
  (Utilities|Array|Resize _helmets 12)
  (Utilities|Array|Resize _chest_armors 12)
  (Utilities|Array|Resize _leg_armors 12)
  (Utilities|Array|Resize _gemstones 12)
  (Default|UpdateItemsinInventoryUI (Variables|Widget|GetWBP_Inventory) (Variables|Default|GetAllitem)))

(event EventLoadData
  (params (SaveGameRef :type BP%20Save%20Game%20Object%20Reference))
  ;[1 1 1] Load Inventory
  (Variables|Default|SetAllitem (Variables|/Game/Zak/SaveGame/BP_SaveGame.BP_SaveGame_C|GetInventorySave SaveGameRef)))

(event EventTick
  (params (DeltaSeconds :type Float%20%28single-precision%29))
  (bind _wbp_interact (Variables|Widget|GetWBP_Interact))
  ;[1 1 1] Show pick up widget
  (bind (_item _founditem) (Inventory|TraceItemtoPickUp))
  (Variables|/Game/Omar/UI/WidgetBlueprints/WBP_ItemInfo.WBP_ItemInfo_C|SetItem (Variables|/Game/Omar/UI/WidgetBlueprints/WBP_Interact.WBP_Interact_C|GetWBP_ItemInfo (Variables|Widget|GetWBP_Interact)) _item)
  (if _founditem
    (UserInterface|Viewport|AddtoViewport _wbp_interact 0)
    (else
      (Widget|RemovefromParent _wbp_interact))))

(event EventSaveData
  (params (SaveGameRef :type BP%20Save%20Game%20Object%20Reference))
  ;[1 1 1] Save inventory
  (Variables|/Game/Zak/SaveGame/BP_SaveGame.BP_SaveGame_C|SetInventorySave SaveGameRef (Variables|Default|GetAllitem)))

(event Input|EnhancedActionEvents|EnhancedInputActionIA_Interact
  (params (ActionValue :type Boolean) (ElapsedSeconds :type Float%20%28double-precision%29) (TriggeredSeconds :type Float%20%28double-precision%29) (InputAction :type Input%20Action%20Object%20Reference :default "/Game/ThirdPerson/Input/Actions/IA_Interact.IA_Interact"))
  ;[1 1 1] Pick up item(destroy item)
  (bind (_item _founditem _itemactor) (Inventory|TraceItemtoPickUp))
  (if _founditem
    (bind _sucess (Inventory|AddtoInventory _item))
    (if _sucess
      (Actor|DestroyActor _itemactor)
      (Default|UpdateItemsinInventoryUI (Variables|Widget|GetWBP_Inventory) (Variables|Default|GetAllitem)))))

(event Input|EnhancedActionEvents|EnhancedInputActionIA_Pause
  (params (ActionValue :type Boolean) (ElapsedSeconds :type Float%20%28double-precision%29) (TriggeredSeconds :type Float%20%28double-precision%29) (InputAction :type Input%20Action%20Object%20Reference :default "/Game/ThirdPerson/Input/Actions/IA_Pause.IA_Pause"))
  (bind _returnvalue (Game|GetPlayerController 0))
  (bind _returnvalue_2 (Game|GetPlayerController 0))
  ;[1 1 1] Pause
  (:Started
    (if (Game|IsGamePaused)
      (Widget|RemovefromParent (Variables|Widget|GetPauseWidget))
      (Game|SetGamePaused false)
      (Variables|/Script/Engine.PlayerController|SetbShowMouseCursor _returnvalue_2 false)
      (Input|SetInputModeGameOnly _returnvalue_2 false)
      (else
        (UserInterface|Viewport|AddtoViewport (Variables|Widget|GetPauseWidget) 0)
        (Variables|/Script/Engine.PlayerController|SetbShowMouseCursor _returnvalue true)
        (Game|SetGamePaused true)
        (Input|SetInputModeGameandUI _returnvalue (Variables|Widget|GetPauseWidget) "DoNotLock" true false)))))

(event Input|EnhancedActionEvents|EnhancedInputActionIA_Inventory
  (params (ActionValue :type Boolean) (ElapsedSeconds :type Float%20%28double-precision%29) (TriggeredSeconds :type Float%20%28double-precision%29) (InputAction :type Input%20Action%20Object%20Reference :default "/Game/ThirdPerson/Input/Actions/IA_Inventory.IA_Inventory"))
  (bind _returnvalue (Game|GetPlayerController 0))
  ;[1 1 1] open inventory
  (:Started
    (bind _returnvalue_2 (Actor|GetActorOfClass "/Game/Zak/BP_Player.BP_Player_C"))
    (bind _asbp_player (Utilities|Casting|CastToBP_Player _returnvalue_2))
    (Rendering|SceneCapture|CaptureScene (Variables|/Game/Zak/BP_Player.BP_Player_C|GetSceneCaptureComponent2D _asbp_player) :!class /Script/Engine.SceneCaptureComponent2D)
    (UserInterface|Viewport|AddtoViewport (Variables|Widget|GetWBP_Inventory) 0)
    (Variables|/Script/Engine.PlayerController|SetbShowMouseCursor _returnvalue true)
    (Input|SetInputModeUIOnly _returnvalue (Variables|Widget|GetWBP_Inventory) "DoNotLock" false)))

(fn TraceItemtoPickUp
  (bind _returnvalue (Game|GetPlayerCharacter 0))
  (bind _returnvalue_2 (Transformation|GetActorLocation _returnvalue))
  (bind _returnvalue_3 (- _returnvalue_2 "0.000000,0.000000,60.000000"))
  ;[1 1 1] Trace item
  (Utilities|IsValid _returnvalue
    (:Is%20Valid
      (bind _outhit (Collision|SphereTraceForObjects _returnvalue_3 (+ _returnvalue_3 (* (Transformation|GetActorForwardVector _returnvalue) 1.5e+02)) 6e+01 (Utilities|Array|MakeArray "ObjectTypeQuery4") false 0 "None"))
      (bind _asbp_item (Utilities|Casting|CastToBP_Item (.hitactor _outhit))
        (:then
          (return (Variables|/Game/Omar/Inventory/Blueprints/BP_Item.BP_Item_C|GetItem _asbp_item) true (.hitactor _outhit)))
        (:CastFailed
          (return "" false 0))))))

(fn AddtoInventory
  (params (Item :type S%20Slot%20Structure))
  (bind (_itemid _quantity _itemtype) (Utilities|Struct|BreakS_Slot Item))
  (bind (_itemid_2 _quantity_2 _itemtype_2) (Utilities|Struct|BreakS_Slot Item))
  (bind (_itemid_3 _quantity_3 _itemtype_3) (Utilities|Struct|BreakS_Slot Item))
  (bind (_itemid_4 _quantity_4 _itemtype_4) (Utilities|Struct|BreakS_Slot Item))
  (bind (_itemid_5 _quantity_5 _itemtype_5) (Utilities|Struct|BreakS_Slot Item))
  (switch Utilities|FlowControl|Switch|SwitchonE_ItemTypes (.ItemType (Utilities|Struct|BreakS_Slot Item))
    (:NewEnumerator0
      ;[1 1 1] swords
      ;;[1 1 1] Add to quantity(swords)
      (for (_array_element _array_index) (.Swords (Utilities|Struct|BreakS_Allitem (Variables|Default|GetAllitem)))
        (if (== (.RowName (Utilities|Struct|BreakDataTableRowHandle (.ItemID (Utilities|Struct|BreakS_Slot _array_element)))) (.RowName (Utilities|Struct|BreakDataTableRowHandle (.ItemID (Utilities|Struct|BreakS_Slot Item)))))
          (bind _returnvalue (Utilities|GetDataTableRow "/Game/Omar/Inventory/DataTables/DT_Items.DT_Items" (.RowName (Utilities|Struct|BreakDataTableRowHandle (.ItemID (Utilities|Struct|BreakS_Slot Item)))))
            (:then
              (if (>= (.StackSize (Utilities|Struct|BreakS_Item _returnvalue)) (+ (.Quantity (Utilities|Struct|BreakS_Slot Item)) (.Quantity (Utilities|Struct|BreakS_Slot _array_element))))
                (Utilities|Array|SetArrayElem (.Swords (Utilities|Struct|BreakS_Allitem (Variables|Default|GetAllitem))) _array_index (Utilities|Struct|MakeS_Slot _itemid_3 (+ (.Quantity (Utilities|Struct|BreakS_Slot Item)) (.Quantity (Utilities|Struct|BreakS_Slot _array_element))) _itemtype_3))
                (return true))))))
      ;;[1 1 1] Add to next inventory slot if stack size is full(swords)
      (for (_array_element_2 _array_index_2) (.Swords (Utilities|Struct|BreakS_Allitem (Variables|Default|GetAllitem)))
        (if (== (.Quantity (Utilities|Struct|BreakS_Slot _array_element_2)) 0)
          (Utilities|Array|SetArrayElem (.Swords (Utilities|Struct|BreakS_Allitem (Variables|Default|GetAllitem))) _array_index_2 Item)
          (return true)))
      (return false))
    (:NewEnumerator1
      ;[1 1 1] Helmets
      ;;[1 1 1] Add to quantity(helmets)
      (for (_array_element_3 _array_index_3) (.Helmets (Utilities|Struct|BreakS_Allitem (Variables|Default|GetAllitem)))
        (if (== (.RowName (Utilities|Struct|BreakDataTableRowHandle (.ItemID (Utilities|Struct|BreakS_Slot _array_element_3)))) (.RowName (Utilities|Struct|BreakDataTableRowHandle (.ItemID (Utilities|Struct|BreakS_Slot Item)))))
          (bind _returnvalue_2 (Utilities|GetDataTableRow "/Game/Omar/Inventory/DataTables/DT_Items.DT_Items" (.RowName (Utilities|Struct|BreakDataTableRowHandle (.ItemID (Utilities|Struct|BreakS_Slot Item)))))
            (:then
              (if (>= (.StackSize (Utilities|Struct|BreakS_Item _returnvalue_2)) (+ (.Quantity (Utilities|Struct|BreakS_Slot Item)) (.Quantity (Utilities|Struct|BreakS_Slot _array_element_3))))
                (Utilities|Array|SetArrayElem (.Helmets (Utilities|Struct|BreakS_Allitem (Variables|Default|GetAllitem))) _array_index_3 (Utilities|Struct|MakeS_Slot _itemid_4 (+ (.Quantity (Utilities|Struct|BreakS_Slot Item)) (.Quantity (Utilities|Struct|BreakS_Slot _array_element_3))) _itemtype_4))
                (return true))))))
      ;;[1 1 1] Add to next inventory slot if stack size is full(helmets)
      (for (_array_element_4 _array_index_4) (.Helmets (Utilities|Struct|BreakS_Allitem (Variables|Default|GetAllitem)))
        (if (== (.Quantity (Utilities|Struct|BreakS_Slot _array_element_4)) 0)
          (Utilities|Array|SetArrayElem (.Helmets (Utilities|Struct|BreakS_Allitem (Variables|Default|GetAllitem))) _array_index_4 Item)
          (return true)))
      (return false))
    (:NewEnumerator2
      ;[1 1 1] chest armors
      ;;[1 1 1] Add to quantity(chest armor)
      (for (_array_element_5 _array_index_5) (.Chest_Armors (Utilities|Struct|BreakS_Allitem (Variables|Default|GetAllitem)))
        (if (== (.RowName (Utilities|Struct|BreakDataTableRowHandle (.ItemID (Utilities|Struct|BreakS_Slot _array_element_5)))) (.RowName (Utilities|Struct|BreakDataTableRowHandle (.ItemID (Utilities|Struct|BreakS_Slot Item)))))
          (bind _returnvalue_3 (Utilities|GetDataTableRow "/Game/Omar/Inventory/DataTables/DT_Items.DT_Items" (.RowName (Utilities|Struct|BreakDataTableRowHandle (.ItemID (Utilities|Struct|BreakS_Slot Item)))))
            (:then
              (if (>= (.StackSize (Utilities|Struct|BreakS_Item _returnvalue_3)) (+ (.Quantity (Utilities|Struct|BreakS_Slot Item)) (.Quantity (Utilities|Struct|BreakS_Slot _array_element_5))))
                (Utilities|Array|SetArrayElem (.Chest_Armors (Utilities|Struct|BreakS_Allitem (Variables|Default|GetAllitem))) _array_index_5 (Utilities|Struct|MakeS_Slot _itemid_5 (+ (.Quantity (Utilities|Struct|BreakS_Slot Item)) (.Quantity (Utilities|Struct|BreakS_Slot _array_element_5))) _itemtype_5))
                (return true))))))
      ;;[1 1 1] Add to next inventory slot if stack size is full(chest armors)
      (for (_array_element_6 _array_index_6) (.Chest_Armors (Utilities|Struct|BreakS_Allitem (Variables|Default|GetAllitem)))
        (if (== (.Quantity (Utilities|Struct|BreakS_Slot _array_element_6)) 0)
          (Utilities|Array|SetArrayElem (.Chest_Armors (Utilities|Struct|BreakS_Allitem (Variables|Default|GetAllitem))) _array_index_6 Item)
          (return true)))
      (return false))
    (:NewEnumerator3
      ;[1 1 1] Leg armors
      ;;[1 1 1] Add to quantity(leg armors)
      (for (_array_element_7 _array_index_7) (.Leg_Armors (Utilities|Struct|BreakS_Allitem (Variables|Default|GetAllitem)))
        (if (== (.RowName (Utilities|Struct|BreakDataTableRowHandle (.ItemID (Utilities|Struct|BreakS_Slot _array_element_7)))) (.RowName (Utilities|Struct|BreakDataTableRowHandle (.ItemID (Utilities|Struct|BreakS_Slot Item)))))
          (bind _returnvalue_4 (Utilities|GetDataTableRow "/Game/Omar/Inventory/DataTables/DT_Items.DT_Items" (.RowName (Utilities|Struct|BreakDataTableRowHandle (.ItemID (Utilities|Struct|BreakS_Slot Item)))))
            (:then
              (if (>= (.StackSize (Utilities|Struct|BreakS_Item _returnvalue_4)) (+ (.Quantity (Utilities|Struct|BreakS_Slot Item)) (.Quantity (Utilities|Struct|BreakS_Slot _array_element_7))))
                (Utilities|Array|SetArrayElem (.Leg_Armors (Utilities|Struct|BreakS_Allitem (Variables|Default|GetAllitem))) _array_index_7 (Utilities|Struct|MakeS_Slot _itemid_2 (+ (.Quantity (Utilities|Struct|BreakS_Slot Item)) (.Quantity (Utilities|Struct|BreakS_Slot _array_element_7))) _itemtype_2))
                (return true))))))
      ;;[1 1 1] Add to next inventory slot if stack size is full(leg armors)
      (for (_array_element_8 _array_index_8) (.Leg_Armors (Utilities|Struct|BreakS_Allitem (Variables|Default|GetAllitem)))
        (if (== (.Quantity (Utilities|Struct|BreakS_Slot _array_element_8)) 0)
          (Utilities|Array|SetArrayElem (.Leg_Armors (Utilities|Struct|BreakS_Allitem (Variables|Default|GetAllitem))) _array_index_8 Item)
          (return true)))
      (return false))
    (:NewEnumerator4
      ;[1 1 1] gemstones
      ;;[1 1 1] Add to quantity(gemstones)
      (for (_array_element_9 _array_index_9) (.Gemstones (Utilities|Struct|BreakS_Allitem (Variables|Default|GetAllitem)))
        (if (== (.RowName (Utilities|Struct|BreakDataTableRowHandle (.ItemID (Utilities|Struct|BreakS_Slot _array_element_9)))) (.RowName (Utilities|Struct|BreakDataTableRowHandle (.ItemID (Utilities|Struct|BreakS_Slot Item)))))
          (bind _returnvalue_5 (Utilities|GetDataTableRow "/Game/Omar/Inventory/DataTables/DT_Items.DT_Items" (.RowName (Utilities|Struct|BreakDataTableRowHandle (.ItemID (Utilities|Struct|BreakS_Slot Item)))))
            (:then
              (if (>= (.StackSize (Utilities|Struct|BreakS_Item _returnvalue_5)) (+ (.Quantity (Utilities|Struct|BreakS_Slot Item)) (.Quantity (Utilities|Struct|BreakS_Slot _array_element_9))))
                (Utilities|Array|SetArrayElem (.Gemstones (Utilities|Struct|BreakS_Allitem (Variables|Default|GetAllitem))) _array_index_9 (Utilities|Struct|MakeS_Slot _itemid (+ (.Quantity (Utilities|Struct|BreakS_Slot Item)) (.Quantity (Utilities|Struct|BreakS_Slot _array_element_9))) _itemtype))
                (return true))))))
      ;;[1 1 1] Add to next inventory slot if stack size is full(leg armors)
      (for (_array_element_10 _array_index_10) (.Gemstones (Utilities|Struct|BreakS_Allitem (Variables|Default|GetAllitem)))
        (if (== (.Quantity (Utilities|Struct|BreakS_Slot _array_element_10)) 0)
          (Utilities|Array|SetArrayElem (.Gemstones (Utilities|Struct|BreakS_Allitem (Variables|Default|GetAllitem))) _array_index_10 Item)
          (return true)))
      (return false))))