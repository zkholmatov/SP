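; Player controller Blueprint that sets up gamepad left-stick control of the mouse cursor.
; Left X checks for nonzero input and a visible cursor, while Left Y skips that check, and both offset the current position by scaled axis input.
; The result goes to SetMousePosition, whose body is empty: its viewport-clamped set call is disconnected, so the cursor never moves through it.
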(event EventBeginPlay)

(event EventTick
  (params (DeltaSeconds :type Float%20%28single-precision%29)))

(event Input|GamepadEvents|GamepadLeftX
  (params (AxisValue :type Float%20%28single-precision%29))
  (bind _returnvalue (Game|GetPlayerController 0))
  (bind (_locationx _locationy) (Game|Player|GetMousePosition _returnvalue))
  (if (and (!= AxisValue 0.0) (Variables|/Script/Engine.PlayerController|GetbShowMouseCursor (Game|GetPlayerController 0)))
    (bind _asbp_player_controller (Utilities|Casting|CastToBP_PlayerController (Game|GetPlayerController 0)))
    (CallFunction|SetMousePosition _asbp_player_controller (Math|Float|Round (+ (* (Class|Actor|GetInputAxisKeyValue) 5.0) _locationx)) (Math|Float|Round (+ _locationy (* (Class|Actor|GetInputAxisKeyValue) 5.0))))))

(event Input|GamepadEvents|GamepadLeftY
  (params (AxisValue :type Float%20%28single-precision%29))
  (bind _returnvalue (Game|GetPlayerController 0))
  (bind (_locationx _locationy) (Game|Player|GetMousePosition _returnvalue))
  (if true
    (bind _asbp_player_controller (Utilities|Casting|CastToBP_PlayerController (Game|GetPlayerController 0)))
    (CallFunction|SetMousePosition _asbp_player_controller (Math|Float|Round (+ (* (Class|Actor|GetInputAxisKeyValue) 5.0) _locationx)) (Math|Float|Round (+ _locationy (* (Class|Actor|GetInputAxisKeyValue) 5.0))))))

(fn ConstructionScript)

(fn SetMousePosition
  (params (X :type Integer) (Y :type Integer))
  (return))