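; BP_MusicTrigger is a trigger actor that plays the tutorial area music in the intro map.
; The first overlap of its box starts the TutorialAreaAudio component, and a PlayMusic flag blocks replays.
; On BeginPlay it binds StopMusic to the TriggerStopTutorialMusic event to silence the track.
; The dungeon music start is unfinished, with an empty StartMusic event and disconnected bind and play nodes.
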(event OnComponentBeginOverlap(OverlapTriggerBox)
  (params (OverlappedComponent :type Primitive%20Component%20Object%20Reference) (OtherActor :type Actor%20Object%20Reference) (OtherComp :type Primitive%20Component%20Object%20Reference) (OtherBodyIndex :type Integer) (bFromSweep :type Boolean) (SweepResult :type Hit%20Result%20Structure%20%28by%20ref%29))
  (if (Variables|Default|GetbPlayMusic)
    (Variables|Default|SetbPlayMusic false)
    (Audio|Components|Audio|Play (Variables|Default|Gettutorial%20area%20audio) 0.0)
    (Development|PrintString "playing ")))

(event Custom|StopMusic
  (Audio|Components|Audio|Stop (Variables|Default|Gettutorial%20area%20audio))
  (Development|PrintString "stopped"))

(event Custom|StartMusic)

(event EventBeginPlay
  (Variables|Default|SetbPlayMusic true)
  (EventDispatchers|BindEventtoTriggerStopTutorialMusic (delegate Custom|StopMusic)))

(fn ConstructionScript)