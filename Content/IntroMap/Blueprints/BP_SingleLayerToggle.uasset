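; BP_SingleLayerToggle is a trigger actor in the IntroMap folder that sets a World Partition data layer's runtime state, commented as serving the intro dungeon area.
; Any overlap on LayerTriggerBox applies StateOfLayer to ModDataLayerAsset through the Data Layer Manager, non-recursively and without filtering the overlapping actor.
; If the manager is invalid, it prints debug strings and sets a separate DataLayer variable through DataLayerSubsystem.
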(event OnComponentBeginOverlap(LayerTriggerBox)
  (params (OverlappedComponent :type Primitive%20Component%20Object%20Reference) (OtherActor :type Actor%20Object%20Reference) (OtherComp :type Primitive%20Component%20Object%20Reference) (OtherBodyIndex :type Integer) (bFromSweep :type Boolean) (SweepResult :type Hit%20Result%20Structure%20%28by%20ref%29))
  ;[0.1872 0.1985 1] On Collision Toggle data layers and music events for intro dungeon area
  (bind _returnvalue (WorldPartition|GetDataLayerManager)) ; get data layer manager for world level partition as reference to set data layer in runtime
  (Utilities|IsValid _returnvalue
    (:Is%20Valid
      (DataLayers|SetDataLayerRuntimeState _returnvalue (Variables|Default|GetModDataLayerAsset) (Variables|Default|GetStateOfLayer) false :!class /Script/Engine.DataLayerManager) ; Function to toggle data layers
    )
    (:Is%20Not%20Valid
      (Development|PrintString "Data layer manager is null")
      (DataLayers|SetDataLayerRuntimeState (WorldSubsystems|GetDataLayerSubsystem) (Variables|Default|GetData%20Layer) (Variables|Default|GetStateOfLayer) false :!class /Script/Engine.DataLayerSubsystem)
      (Development|PrintString "Hello"))))

(event EventBeginPlay
  ;[1 1 1] On Begin Play
)

(fn ConstructionScript)