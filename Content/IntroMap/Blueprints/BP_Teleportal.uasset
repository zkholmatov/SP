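; BP_Teleportal is a portal actor that teleports the player to other portals with matching gameplay tags.
; It can start hidden until a boss death, dev-portal event or boss-state interface call enables it and shows InvisBody.
; Player overlap scans all teleportals for tag matches, then plays a sound, shows a widget and moves the player with an offset.
; With SaveLocation set, it also updates the player's spawn transform and requests a game save.
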(event OnComponentBeginOverlap(OverlapBox)
  (params (OverlappedComponent :type Primitive%20Component%20Object%20Reference) (OtherActor :type Actor%20Object%20Reference) (OtherComp :type Primitive%20Component%20Object%20Reference) (OtherBodyIndex :type Integer) (bFromSweep :type Boolean) (SweepResult :type Hit%20Result%20Structure%20%28by%20ref%29))
  (bind _portaltag (Variables|Portal|GetPortalTag))
  (if (Variables|Default|GetEnabled?)
    (if (and (!= OtherActor self) (== OtherActor (Game|GetPlayerCharacter 0)))
      (bind _outactors (Actor|GetAllActorsOfClass "BP_Teleportal_C"))
      (for _array_element _outactors
        (if (!= _array_element self)
          (Development|PrintString "Is not self " (!= _array_element self))
          (if (or (GameplayTags|HasAnyTags (Variables|BP_Teleportal_C|GetPortalTag _array_element) _portaltag true) (GameplayTags|HasAllTags (Variables|BP_Teleportal_C|GetPortalTag _array_element) _portaltag true))
            (Development|PrintString (GameplayTags|GetDebugStringfromGameplayTagContainer (Variables|BP_Teleportal_C|GetPortalTag _array_element)) true true "(R=0.000000,G=0.660000,B=1.000000,A=1.000000)" 1e+01)
            (Audio|PlaySound2D "/Engine/EditorSounds/GamePreview/EjectFromPlayer_Cue.EjectFromPlayer_Cue" 1.0 1.0 0.0 0 0)
            (bind _returnvalue (UserInterface|CreateWidget (Variables|Default|GetClass)))
            (UserInterface|Viewport|AddtoViewport _returnvalue -1)
            (Transformation|SetActorLocationAndRotation OtherActor (- (Transformation|GetActorLocation _array_element) (* (Transformation|GetActorForwardVector _array_element) (Variables|Default|GetOffsetFloat))) (* (Transformation|GetActorRotation _array_element) -1.5))
            (if (Variables|Default|GetbSaveLocation)
              (bind _asbp_player (Utilities|Casting|CastToBP_Player OtherActor))
              (Variables|/Game/Zak/BP_Player.BP_Player_C|SetSpawnTransform _asbp_player (Math|Transform|MakeTransform (- (Transformation|GetActorLocation _array_element) (* (Transformation|GetActorForwardVector _array_element) (Variables|Default|GetOffsetFloat))) "0, 0, 0" "1.000000,1.000000,1.000000"))
              (Default|RequestSave (Variables|Default|GetAs%20BP%20Game%20Instance) true))))))))

(event Custom|EnablePortal1
  (CallFunction|PortalVisible))

(event Custom|EnablePortal2
  (CallFunction|PortalVisible))

(event Custom|PortalVisible
  (bind _output_get (Variables|Default|SetEnabled? true))
  (Rendering|SetVisibility (Variables|Default|GetInvisBody) _output_get true))

(event Custom|EnablePortal3
  (CallFunction|PortalVisible))

(event Custom|EnablePortal4
  (CallFunction|PortalVisible))

(event EventBPIBossIsDead
  (params (myre :type Boolean) (warden :type Boolean) (finalBoss :type Boolean))
  (Utilities|FlowControl|Sequence
    (:then_0
      (if (and myre (Variables|Default|GetforMyre))
        (CallFunction|PortalVisible :!label _label)))
    (:then_1
      (if (and warden (Variables|Default|GetforWarden))
        (goto _label)))
    (:then_2
      (if (and finalBoss (Variables|Default|GetforFinalBoss))
        (goto _label)))))

(event EventLoadData
  (params (SaveGameRef :type BP%20Save%20Game%20Object%20Reference)))

(event EventSaveData
  (params (SaveGameRef :type BP%20Save%20Game%20Object%20Reference)))

(event EventBeginPlay
  (bind _asbp_game_instance (Utilities|Casting|CastToBP_GameInstance (Game|GetGameInstance)))
  (bind _output_get (Variables|Default|SetAs%20BP%20Game%20Instance _asbp_game_instance))
  (Class|BPIPersistence|RequestLoad(Message) _output_get self)
  (bind _output_get_2 (Variables|Default|SetEnabled? (Variables|Default|GetEnabled?)))
  (Rendering|SetVisibility (Variables|Default|GetInvisBody) _output_get_2 true)
  (bind _myreboss (Variables|Default|GetMyreBoss)
    (:then
      (EventDispatchers|BindEventtoOnBossDeath _myreboss (delegate Custom|EnablePortal1)))
    (:else
      _))
  (bind _wardenboss (Variables|Default|GetWardenBoss)
    (:then
      (EventDispatchers|BindEventtoOnBossDeath _wardenboss (delegate Custom|EnablePortal2)))
    (:else
      _))
  (bind _finalboss (Variables|Default|GetFinalBoss)
    (:then
      (EventDispatchers|BindEventtoOnBossDeath _finalboss (delegate Custom|EnablePortal3)))
    (:else
      _))
  (if (Variables|Default|GetbDevPortal)
    (for _array_element (Variables|Default|GetKillBossAlt)
      (EventDispatchers|BindEventtoDevPortal _array_element (delegate Custom|EnablePortal4)))))

(fn ConstructionScript)