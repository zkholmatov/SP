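; BP_LayerToggle is a trigger actor that swaps World Partition data layers and music for the intro dungeon area.
; Overlapping LayerTriggerBox sets the outgoing layer to Loaded, hiding it, on every overlap.
; The PlayFallingStone flag limits the rest to once: a quake sound, activating the incoming layer, and telling BP_MusicTrigger actors to switch from tutorial to dungeon music.
; Deprecated DataLayerSubsystem calls remain unconnected.
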(event OnComponentBeginOverlap(LayerTriggerBox)
  (params (OverlappedComponent :type Primitive%20Component%20Object%20Reference) (OtherActor :type Actor%20Object%20Reference) (OtherComp :type Primitive%20Component%20Object%20Reference) (OtherBodyIndex :type Integer) (bFromSweep :type Boolean) (SweepResult :type Hit%20Result%20Structure%20%28by%20ref%29))
  ;[0.1872 0.1985 1] On Collision Toggle data layers and music events for intro dungeon area
  (bind _returnvalue (WorldPartition|GetDataLayerManager)) ; get data layer manager for world level partition as reference to set data layer in runtime
  (DataLayers|SetDataLayerRuntimeState _returnvalue (Variables|Default|GetOutDataLayerAsset) "Loaded" false :!class /Script/Engine.DataLayerManager) ; Function to toggle data layers
  (if (Variables|Default|GetbPlayFallingStone)
    (Variables|Default|SetbPlayFallingStone false) ; set falling stone boolean to false after single use so it cant be used again to determine functionality that follows
    (Audio|PlaySound2D "/Game/IntroMap/quake-and-break-99034.quake-and-break-99034" 1.0 1.0 0.0 0 0) ; Play sound of old data layer ie tower being moved
    (bind _returnvalue_2 (WorldPartition|GetDataLayerManager)) ; get data layer manager for world level partition as reference to set data layer in runtime
    (DataLayers|SetDataLayerRuntimeState _returnvalue_2 (Variables|Default|GetInDataLayerAsset) "Activated" false :!class /Script/Engine.DataLayerManager) ; Function to toggle data layers
    (bind _outactors (Actor|GetAllActorsOfClass "/Game/IntroMap/Blueprints/BP_MusicTrigger.BP_MusicTrigger_C")) ; get reference to actor of class BP Music toggle to call event s
    (Default|CallTriggerStopTutorialMusic _outactors) ; call event to stop current intro music
    (Default|CallTriggerStartDungeonMusic _outactors) ; call event to start new dungeon music
  ))

(event EventBeginPlay
  ;[1 1 1] On Begin Play
  (Variables|Default|SetbPlayFallingStone true) ; set falling stone bollean to true
)

(event Collision|EventActorBeginOverlap
  (params (OtherActor :type Actor%20Object%20Reference)))

(fn ConstructionScript)