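; BP_SimpleLayerToggle is a trigger volume that switches World Partition data layers when the player enters it, intended to activate the elevator layer and set the starter area to loaded.
; On overlap of LayerTriggerBox with player character 0, it sets configurable Out and In data layer assets to their runtime states through the Data Layer Manager, non-recursively.
; Older DataLayerSubsystem calls and an EndGame-tag widget branch remain in the graph but are unconnected.
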(event OnComponentBeginOverlap(LayerTriggerBox)
  (params (OverlappedComponent :type Primitive%20Component%20Object%20Reference) (OtherActor :type Actor%20Object%20Reference) (OtherComp :type Primitive%20Component%20Object%20Reference) (OtherBodyIndex :type Integer) (bFromSweep :type Boolean) (SweepResult :type Hit%20Result%20Structure%20%28by%20ref%29))
  (bind _returnvalue (Game|GetPlayerCharacter 0))
  ;[1 1 1] On Collision Toggle data layers. This is designed to activate the elevator layer and set starter area to loaded
  (Utilities|IsValid _returnvalue
    (:Is%20Valid
      (if (== OtherActor _returnvalue)
        (bind _returnvalue_2 (WorldPartition|GetDataLayerManager)) ; get data layer manager for world level partition as reference to set data layer in runtime
        (DataLayers|SetDataLayerRuntimeState _returnvalue_2 (Variables|Default|GetOutDataLayerAsset) (Variables|Default|GetOutState) false :!class /Script/Engine.DataLayerManager) ; Function to toggle data layers
        (bind _returnvalue_3 (WorldPartition|GetDataLayerManager)) ; get data layer manager for world level partition as reference to set data layer in runtime
        (DataLayers|SetDataLayerRuntimeState _returnvalue_3 (Variables|Default|GetInDataLayerAsset) (Variables|Default|GetIn%20State) false :!class /Script/Engine.DataLayerManager) ; Function to toggle data layers
      ))
    (:Is%20Not%20Valid
      (Development|PrintString "Not valid get player in toggle "))))

(event EventBeginPlay)

(event Collision|EventActorBeginOverlap
  (params (OtherActor :type Actor%20Object%20Reference)))

(fn ConstructionScript)